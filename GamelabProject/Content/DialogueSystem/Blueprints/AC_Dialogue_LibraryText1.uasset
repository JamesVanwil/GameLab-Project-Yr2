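; Dialogue component for a library bookcase interaction, where Roland notices a strange book and can leave it or take it.
; Dialogue disables player movement and branches on the chosen option; both paths close the conversation and restore walking.
; Leave clears dialogue progress, while Take adds the book weapon to the JRPG controller's inventory and destroys the NPC_Base_Library1 actor found by class.
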(fn `Dialogue`
  (`parent.Dialogue`)
  (`CharacterMovementComponent.SetMovementMode` (`Character.CharacterMovement` (`GameplayStatics.GetPlayerCharacter` 0)) "MOVE_None" 0)
  (bind (_state _optionindex) (`self.AddDialogue` "Roland" "The bookcase is full of uninteresting books, but one of them catches your attention, a book with a deformed face drawn on the cover." (`|MakeArray` "(Leave)" "(Take)" :!type "Text")))
  (switch `/Game/DialogueSystem/Blueprints/Enum_DialogueState` _state
    (:`NewEnumerator0`
      (switch `int` _optionindex
        (:`0`
          (`self.ClearDialogueProgress`))
        (:`1`
          (bind _asbp_jrpgplayer_controller (cast `/Game/TurnBasedJRPGTemplate/Blueprints/Controllers/BP_JRPGPlayerController` (`GameplayStatics.GetPlayerController` 0)))
          (`/Game/TurnBasedJRPGTemplate/Blueprints/Controllers/BP_JRPGPlayerController.AddEquipmentToInventory` _asbp_jrpgplayer_controller "/Game/TurnBasedJRPGTemplate/Blueprints/Items/Equipment/Weapons/BP_BookWeapon.BP_BookWeapon_C" 1)
          (bind _returnvalue (`GameplayStatics.GetActorOfClass` "/Game/DialogueSystem/Blueprints/NPC_Base_Library1.NPC_Base_Library1_C"))
          (`Actor.K2_DestroyActor` _returnvalue)))
      (`self.CloseConversation`)
      (`CharacterMovementComponent.SetMovementMode` (`Character.CharacterMovement` (`GameplayStatics.GetPlayerCharacter` 0)) "MOVE_Walking" 0))))