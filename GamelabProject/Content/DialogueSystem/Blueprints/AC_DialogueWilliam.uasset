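; Dialogue component for the NPC William, who tries to talk Roland out of leaving to follow Preston into danger.
; Its Dialogue function calls the parent, disables player movement, then branches through AddDialogue calls on the chosen option index.
; All branches converge on clearing dialogue progress, closing the conversation and restoring walking.
; A disconnected snippet that would destroy the William NPC never runs.
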(fn `Dialogue`
  (`parent.Dialogue`)
  (`CharacterMovementComponent.SetMovementMode` (`Character.CharacterMovement` (`GameplayStatics.GetPlayerCharacter` 0)) "MOVE_None" 0)
  (bind (_state _optionindex) (`self.AddDialogue` "William" "What do you think you are doing Roland?" (`|MakeArray` "We have to escape this place." "Step aside, I don't have time for this." :!type "Text")))
  (switch `/Game/DialogueSystem/Blueprints/Enum_DialogueState` _state
    (:`NewEnumerator0`
      (switch `int` _optionindex
        (:`0`
          (bind (_state_2 _optionindex_2) (`self.AddDialogue` "William" "Preston came out because he knows the villa and probably knows a way to stop those creatures... don't risk your life unnecessarily, stay safe here!" (`|MakeArray` "Ok fine, I'll wait a little longer" "Step aside" :!type "Text")))
          (switch `/Game/DialogueSystem/Blueprints/Enum_DialogueState` _state_2
            (:`NewEnumerator0`
              (switch `int` _optionindex_2
                (:`0`
                  _)
                (:`1`
                  (bind _state_3 (`self.AddDialogue` "William" "OK... all right \nBut know that when those creatures see you, they will kill you like they did to so many of us." (`|MakeArray` "I don't care, I have nothing left to lose but Preston" :!type "Text")))
                  (switch `/Game/DialogueSystem/Blueprints/Enum_DialogueState` _state_3
                    (:`NewEnumerator0`
                      _)))))))
        (:`1`
          (bind _state_4 (`self.AddDialogue` "William" "Don't worry Roland, Preston is safe and sound and will come to save us shortly" (`|MakeArray` "Mmh" :!type "Text")))
          (switch `/Game/DialogueSystem/Blueprints/Enum_DialogueState` _state_4
            (:`NewEnumerator0`
              _))))
      (`self.ClearDialogueProgress`)
      (`self.CloseConversation`)
      (`CharacterMovementComponent.SetMovementMode` (`Character.CharacterMovement` (`GameplayStatics.GetPlayerCharacter` 0)) "MOVE_Walking" 0))))