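; NPC base Blueprint that lets the player start a dialogue with this character through an interaction detector.
; On BeginPlay it casts its interaction child actor to BP_InteractionDetector and binds the detector's interacted event to open the Winchester Wall dialogue component's conversation.
; When the conversation closes, it re-enables the detector and refreshes the JRPG player controller's interactions so the NPC can be talked to again.
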(event `self.ReceiveBeginPlay`
  (bind _asbp_interaction_detector (cast `/Game/TurnBasedJRPGTemplate/Blueprints/Interactables/BP_InteractionDetector` (`ChildActorComponent.ChildActor` (`self.InteractionActor`))))
  (bind _output_get (set `self.As BP Interaction Detector` _asbp_interaction_detector))
  (add `/Game/TurnBasedJRPGTemplate/Blueprints/Interactables/BP_InteractionDetector.OnInteracted` _output_get (delegate `StartConversation`))
  (add `/Game/DialogueSystem/Blueprints/AC_Dialogue_Base.Close Conversation` (`self.AC_Dialogue_Base_WinchesterWall`) (delegate `ResetDialogueInteraction`)))

(event `StartConversation`
  (`/Game/DialogueSystem/Blueprints/AC_Dialogue_Base.OpenConversation` (`self.AC_Dialogue_Base_WinchesterWall`)))

(event `ResetDialogueInteraction`
  (bind _as_bp_interaction_detector (`self.As BP Interaction Detector`))
  (`/Game/TurnBasedJRPGTemplate/Blueprints/Interactables/BP_InteractionDetector.EnableInteraction` _as_bp_interaction_detector)
  (`/Game/TurnBasedJRPGTemplate/Blueprints/Controllers/BP_JRPGPlayerController.RefreshInteractions` (`/Game/TurnBasedJRPGTemplate/Blueprints/Interactables/BP_InteractionDetector.jRPGPlayerController` _as_bp_interaction_detector)))

(fn `UserConstructionScript`
  (`parent.UserConstructionScript`))