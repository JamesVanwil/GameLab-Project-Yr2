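; Dialogue component for the secret book interaction, where Roland finds a hidden trigger among the library books.
; It overrides Dialogue, freezing player movement and chaining AddDialogue calls that branch on the chosen option.
; Pressing, then leaving, calls OpenLibraryDoor on the NPC_BaseSecretBook found by class and destroys that actor.
; Both finished branches remove dialogue progress, close the conversation and restore walking.
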(fn `Dialogue`
  (`parent.Dialogue`)
  (`CharacterMovementComponent.SetMovementMode` (`Character.CharacterMovement` (`GameplayStatics.GetPlayerCharacter` 0)) "MOVE_None" 0)
  (bind (_state _optionindex) (`self.AddDialogue` "Roland" "(there is a trigger hidden among the books)" (`|MakeArray` "Press" "Don't press" :!type "Text")))
  (switch `/Game/DialogueSystem/Blueprints/Enum_DialogueState` _state
    (:`NewEnumerator0`
      (switch `int` _optionindex
        (:`0`
          (bind _state_2 (`self.AddDialogue` "Roland" "(you hear a metallic sound at a distance)" (`|MakeArray` "Leave" :!type "Text")))
          (switch `/Game/DialogueSystem/Blueprints/Enum_DialogueState` _state_2
            (:`NewEnumerator0`
              (bind _returnvalue (`GameplayStatics.GetActorOfClass` "/Game/DialogueSystem/Blueprints/NPC_BaseSecretBook.NPC_BaseSecretBook_C"))
              (`/Game/DialogueSystem/Blueprints/NPC_BaseSecretBook.OpenLibraryDoor` _returnvalue)
              (`self.RemoveDialogueProgress` 1)
              (`self.CloseConversation`)
              (bind _returnvalue_2 (`GameplayStatics.GetActorOfClass` "/Game/DialogueSystem/Blueprints/NPC_BaseSecretBook.NPC_BaseSecretBook_C"))
              (`Actor.K2_DestroyActor` _returnvalue_2)
              (`CharacterMovementComponent.SetMovementMode` (`Character.CharacterMovement` (`GameplayStatics.GetPlayerCharacter` 0)) "MOVE_Walking" 0))))
        (:`1`
          (`self.RemoveDialogueProgress` 1)
          (`self.CloseConversation`)
          (`CharacterMovementComponent.SetMovementMode` (`Character.CharacterMovement` (`GameplayStatics.GetPlayerCharacter` 0)) "MOVE_Walking" 0))))))