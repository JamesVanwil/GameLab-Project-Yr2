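; NPC_BeforeWallleaper is a one-shot trigger that stages a dialogue cutscene introducing the wall leaper enemy.
; When the mage overlaps its box, it freezes movement and input, saves the camera transform to the dialogue component, and moves the camera to a hardcoded shot.
; It spawns a scaled-up BP_WallEnemy at a fixed spot and opens the conversation.
; The actor destroys itself when the conversation closes; this graph does not restore camera or controls.
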(event `self.Box.OnComponentBeginOverlap`
  (params (OverlappedComponent :type "PrimitiveComponent Object Reference") (OtherActor :type "Actor Object Reference") (OtherComp :type "PrimitiveComponent Object Reference") (OtherBodyIndex :type Integer) (bFromSweep :type Boolean) (SweepResult :type "HitResult Structure (by ref)"))
  (bind _ac_dialoguebeforemeetwallleaper (`self.AC_DialogueBeforeMeetWallLeaper`))
  (cast `/Game/TurnBasedJRPGTemplate/Blueprints/PlayerPawns/BP_MageCharacter` OtherActor)
  (bind _asbp_mage_character (cast `/Game/TurnBasedJRPGTemplate/Blueprints/PlayerPawns/BP_MageCharacter` (`GameplayStatics.GetPlayerCharacter` 0)))
  (`CharacterMovementComponent.SetMovementMode` (`Character.CharacterMovement` _asbp_mage_character) "MOVE_None" 0)
  (bind _camera (`/Game/TurnBasedJRPGTemplate/Blueprints/PlayerPawns/BP_JRPGCharacterBase.Camera` _asbp_mage_character))
  (bind _returnvalue (`SceneComponent.K2_GetComponentRotation` _camera))
  (`KismetSystemLibrary.PrintString` (`KismetStringLibrary.Conv_RotatorToString` _returnvalue))
  (set `/Game/DialogueSystem/Blueprints/AC_DialogueBeforeMeetWallLeaper.Camera World Rotation` _returnvalue _ac_dialoguebeforemeetwallleaper)
  (bind _returnvalue_2 (`SceneComponent.K2_GetComponentLocation` _camera))
  (`KismetSystemLibrary.PrintString` (`KismetStringLibrary.Conv_VectorToString` _returnvalue_2))
  (set `/Game/DialogueSystem/Blueprints/AC_DialogueBeforeMeetWallLeaper.Camera World Location` _returnvalue_2 _ac_dialoguebeforemeetwallleaper)
  (`SceneComponent.K2_SetWorldLocationAndRotation` _camera (-959.758572 6318.037186 260.0) (struct :`Yaw` 140.0) false false)
  (`self.DisableInput` (`GameplayStatics.GetPlayerController` 0))
  (`|SpawnActorFromClass` "/Game/BP_WallEnemy.BP_WallEnemy_C" (`KismetMathLibrary.MakeTransform` (-1325.0 6600.0 200.0) (struct :`Yaw` -130.0) (2.0 2.0 2.0)) "Undefined" "MultiplyWithRoot" null null)
  (`/Game/DialogueSystem/Blueprints/AC_Dialogue_Base.OpenConversation` (`self.AC_DialogueBeforeMeetWallLeaper`)))

(event `/Game/DialogueSystem/Blueprints/BPI_Interactable.ConversationClosed`
  (`self.K2_DestroyActor`))

(fn `UserConstructionScript`
  (`parent.UserConstructionScript`))