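; Dialogue component for the encounter before meeting the Wall Leaper, in which an unseen "???" speaker lures the cowboy player toward a crack in the wall.
; Overrides Dialogue, calls the parent, then runs a short branching conversation whose two replies converge on one ending.
; That ending closes the conversation, debug-prints and reapplies the CameraWorld location and rotation to the BP_MageCharacter camera, then re-enables input and walking movement.
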(fn `Dialogue`
  (bind _camera_world_rotation (`self.Camera World Rotation`))
  (bind _camera_world_location (`self.Camera World Location`))
  (`parent.Dialogue`)
  (bind (_state _optionindex) (`self.AddDialogue` "???" "pssss...hey you cowboy! Come here!" (`|MakeArray` "Where are you?" "..." :!type "Text")))
  (switch `/Game/DialogueSystem/Blueprints/Enum_DialogueState` _state
    (:`NewEnumerator0`
      (switch `int` _optionindex
        (:`0`
          (bind _state_2 (`self.AddDialogue` "???" "Come on! Don't be a shy cowboy! Come here. I'm on the wall inside the crack!" (`|MakeArray` "..." :!type "Text")))
          (switch `/Game/DialogueSystem/Blueprints/Enum_DialogueState` _state_2
            (:`NewEnumerator0`
              _)))
        (:`1`
          (bind _state_3 (`self.AddDialogue` "???" "I am here, on the wall, inside the crack...come closer cowboy" (`|MakeArray` "..." :!type "Text")))
          (switch `/Game/DialogueSystem/Blueprints/Enum_DialogueState` _state_3
            (:`NewEnumerator0`
              _))))
      (`self.CloseConversation`)
      (bind _asbp_mage_character (cast `/Game/TurnBasedJRPGTemplate/Blueprints/PlayerPawns/BP_MageCharacter` (`GameplayStatics.GetPlayerCharacter` 0)))
      (`KismetSystemLibrary.PrintString` (`KismetStringLibrary.Conv_RotatorToString` _camera_world_rotation))
      (`KismetSystemLibrary.PrintString` (`KismetStringLibrary.Conv_VectorToString` _camera_world_location))
      (`SceneComponent.K2_SetWorldLocationAndRotation` (`/Game/TurnBasedJRPGTemplate/Blueprints/PlayerPawns/BP_JRPGCharacterBase.Camera` _asbp_mage_character) _camera_world_location _camera_world_rotation true true)
      (`Actor.EnableInput` _asbp_mage_character (`GameplayStatics.GetPlayerController` 0))
      (`CharacterMovementComponent.SetMovementMode` (`Character.CharacterMovement` _asbp_mage_character) "MOVE_Walking" 0))))