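; NPC_Base_Placida is the dialogue-system Blueprint for the Placida NPC, which starts a conversation when interacted with.
; On BeginPlay it casts its InteractionActor child actor to BP_InteractionDetector, caches it and binds StartConversation to its interaction event.
; StartConversation opens the conversation through ACDialoguePlacida.
; A ConversationClosed event destroys the NPC, so the actor does not persist after that event fires.
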(event `self.ReceiveBeginPlay`
  (bind _asbp_interaction_detector (cast `/Game/TurnBasedJRPGTemplate/Blueprints/Interactables/BP_InteractionDetector` (`ChildActorComponent.ChildActor` (`self.InteractionActor`))))
  (bind _output_get (set `self.As BP Interaction Detector` _asbp_interaction_detector))
  (add `/Game/TurnBasedJRPGTemplate/Blueprints/Interactables/BP_InteractionDetector.OnInteracted` _output_get (delegate `StartConversation`)))

(event `StartConversation`
  (`/Game/DialogueSystem/Blueprints/AC_Dialogue_Base.OpenConversation` (`self.AC_Dialogue_Placida`)))

(event `/Game/DialogueSystem/Blueprints/BPI_Interactable.ConversationClosed`
  (`self.K2_DestroyActor`))

(fn `UserConstructionScript`
  (`parent.UserConstructionScript`))