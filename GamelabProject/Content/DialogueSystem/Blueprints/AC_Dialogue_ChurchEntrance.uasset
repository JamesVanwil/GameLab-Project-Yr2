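; AC_Dialogue_ChurchEntrance is a dialogue component that plays Placida's remark about the villa chapel's intact Virgin Mary statue.
; Its Dialogue override calls the parent, then uses GetActorOfClass on BP_PriestCharacter to check that Placida is present.
; If found, it disables player movement, shows one line with a single continue option, then closes the conversation and restores walking.
; Otherwise it prints a not-in-team message and closes the conversation.
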(fn `Dialogue`
  (`parent.Dialogue`)
  (bind _returnvalue (`GameplayStatics.GetActorOfClass` "/Game/TurnBasedJRPGTemplate/Blueprints/PlayerPawns/BP_PriestCharacter.BP_PriestCharacter_C"))
  (`/Engine/EditorBlueprintResources/StandardMacros.IsValid` _returnvalue
    (:`Is Valid`
      (`CharacterMovementComponent.SetMovementMode` (`Character.CharacterMovement` (`GameplayStatics.GetPlayerCharacter` 0)) "MOVE_None" 0)
      (bind _state (`self.AddDialogue` "Placida" "At least those abominations did not manage to touch the villa's small chapel.... The statue of the Virgin Mary is still intact" (`|MakeArray` "..." :!type "Text")))
      (switch `/Game/DialogueSystem/Blueprints/Enum_DialogueState` _state
        (:`NewEnumerator0`
          (`self.CloseConversation`)
          (`CharacterMovementComponent.SetMovementMode` (`Character.CharacterMovement` (`GameplayStatics.GetPlayerCharacter` 0)) "MOVE_Walking" 0))))
    (:`Is Not Valid`
      (`KismetSystemLibrary.PrintString` "Placida not in team")
      (`self.CloseConversation`))))