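; James is a human NPC Blueprint in the dialogue system that the player can talk to.
; Interacting stores the instigator and opens a conversation through the ACDialogueJames component.
; Capsule overlap begin and end events show and hide the TalkToNPC prompt, found by searching for the WBP_InteractionsUI widget at runtime.
; The overlap handlers do not filter the overlapping actor, and the construction script only calls its parent.
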(event `/Game/DialogueSystem/Blueprints/BPI_Interactable.Interact`
  (params (Instigator :type "Actor Object Reference"))
  (set `self.InteractInstigator` Instigator)
  (`/Game/DialogueSystem/Blueprints/AC_Dialogue_Base.OpenConversation` (`self.AC_DialogueJames`)))

(event `self.CapsuleComponent.OnComponentBeginOverlap`
  (params (OverlappedComponent :type "PrimitiveComponent Object Reference") (OtherActor :type "Actor Object Reference") (OtherComp :type "PrimitiveComponent Object Reference") (OtherBodyIndex :type Integer) (bFromSweep :type Boolean) (SweepResult :type "HitResult Structure (by ref)"))
  (bind _foundwidgets (`WidgetBlueprintLibrary.GetAllWidgetsOfClass` "/Game/WBP_InteractionsUI.WBP_InteractionsUI_C"))
  (`Widget.SetVisibility` (`/Game/WBP_InteractionsUI.TalkToNPC` (`|GetArrayItem` _foundwidgets)) "Visible"))

(event `self.CapsuleComponent.OnComponentEndOverlap`
  (params (OverlappedComponent :type "PrimitiveComponent Object Reference") (OtherActor :type "Actor Object Reference") (OtherComp :type "PrimitiveComponent Object Reference") (OtherBodyIndex :type Integer))
  (bind _foundwidgets (`WidgetBlueprintLibrary.GetAllWidgetsOfClass` "/Game/WBP_InteractionsUI.WBP_InteractionsUI_C"))
  (`Widget.SetVisibility` (`/Game/WBP_InteractionsUI.TalkToNPC` (`|GetArrayItem` _foundwidgets)) "Hidden"))

(fn `UserConstructionScript`
  (`parent.UserConstructionScript`))