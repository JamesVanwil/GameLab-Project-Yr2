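; Church statue NPC Blueprint that opens a dialogue when interacted with.
; On BeginPlay it casts its InteractionActor1 child actor to BP_InteractionDetector and binds StartConversation to the detector's OnInteracted event.
; StartConversation opens the conversation on the ACDialogueChurchStatue component.
; The separate Interact event only stores its instigator, and an unused OpenConversation call on ACDialogueJames never runs.
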(event `self.ReceiveBeginPlay`
  ;[1 1 1] Setup Interaction
  (bind _asbp_interaction_detector (cast `/Game/TurnBasedJRPGTemplate/Blueprints/Interactables/BP_InteractionDetector` (`ChildActorComponent.ChildActor` (`self.InteractionActor1`))))
  (bind _output_get (set `self.As BP Interaction Detector` _asbp_interaction_detector))
  (add `/Game/TurnBasedJRPGTemplate/Blueprints/Interactables/BP_InteractionDetector.OnInteracted` _output_get (delegate `StartConversation`)))

(event `StartConversation`
  ;[1 1 1] Setup Interaction
  (`/Game/DialogueSystem/Blueprints/AC_Dialogue_Base.OpenConversation` (`self.AC_Dialogue_ChurchStatue`)))

(event `/Game/DialogueSystem/Blueprints/BPI_Interactable.Interact`
  (params (Instigator :type "Actor Object Reference"))
  (set `self.InteractInstigator` Instigator))

(fn `UserConstructionScript`
  (`parent.UserConstructionScript`))