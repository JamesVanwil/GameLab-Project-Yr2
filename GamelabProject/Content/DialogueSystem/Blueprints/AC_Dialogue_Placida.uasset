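; Dialogue component for Placida, scripting the branching conversation in which Roland asks about Preston and learns of a flesh wall beyond the door.
; Dialogue runs the parent, disables player movement, then chains AddDialogue calls, branching on option index with shared paths rejoining.
; Inviting Placida along adds BP_PriestPlayerUnit to the player's units and party through BP_JRPGPlayerController.
; Both final choices restore walking and close the conversation.
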(fn `Dialogue`
  (`parent.Dialogue`)
  (`CharacterMovementComponent.SetMovementMode` (`Character.CharacterMovement` (`GameplayStatics.GetPlayerCharacter` 0)) "MOVE_None" 0)
  (bind _state (`self.AddDialogue` "Placida" " What are you doing here Roland? And where are the others?" (`|MakeArray` "how to summarise it..." :!type "Text")))
  (switch `/Game/DialogueSystem/Blueprints/Enum_DialogueState` _state
    (:`NewEnumerator0`
      (bind (_state_2 _optionindex) (`self.AddDialogue` "Roland" "Most of them died when the creatures attacked the villa, me and a handful of survivors locked ourselves inside a saferoom, but I went out to find a way to escape from this hell" (`|MakeArray` "Have you seen Preston?" "What are you doing here?" :!type "Text")))
      (switch `/Game/DialogueSystem/Blueprints/Enum_DialogueState` _state_2
        (:`NewEnumerator0`
          (switch `int` _optionindex
            (:`0`
              (bind _state_3 (`self.AddDialogue` "Placida" "Preston? Eh... Preston was here with me!" (`|MakeArray` "And where is he now? He'll surely know how to escape from here." :!type "Text")))
              (switch `/Game/DialogueSystem/Blueprints/Enum_DialogueState` _state_3
                (:`NewEnumerator0`
                  _)))
            (:`1`
              (bind _state_4 (`self.AddDialogue` "Harper" " I'm waiting for Preston, but he's taking too long to come back and I can't kill another one of those beasts anymore" (`|MakeArray` "And where is he now? He'll surely know how to escape from here." :!type "Text")))
              (switch `/Game/DialogueSystem/Blueprints/Enum_DialogueState` _state_4
                (:`NewEnumerator0`
                  _))))
          (bind (_state_5 _optionindex_2) (`self.AddDialogue` "Placida" "I don't know if he is safe right know when the monsters attacked he took me by the arm and brought me here and told me to stand guard and make sure no one followed him" (`|MakeArray` "Stand guard on what?" "Where is he now?" :!type "Text")))
          (switch `/Game/DialogueSystem/Blueprints/Enum_DialogueState` _state_5
            (:`NewEnumerator0`
              (switch `int` _optionindex_2
                (:`0`
                  (bind (_state_6 _optionindex_3) (`self.AddDialogue` "Placida" " Beyond that door, the problem is that a sort of wall of flesh has formed there, it is not aggressive, but it keeps releasing strange fumes and I struggle to get rid of it myself" (`|MakeArray` " You can join me, together we could do it" "Step aside I'll take care of it" :!type "Text")))
                  (switch `/Game/DialogueSystem/Blueprints/Enum_DialogueState` _state_6
                    (:`NewEnumerator0`
                      (switch `int` _optionindex_3
                        (:`0`
                          (bind _asbp_jrpgplayer_controller (cast `/Game/TurnBasedJRPGTemplate/Blueprints/Controllers/BP_JRPGPlayerController` (`GameplayStatics.GetPlayerController` 0) :!label _label))
                          (`/Game/TurnBasedJRPGTemplate/Blueprints/Controllers/BP_JRPGPlayerController.AddPlayerUnit` _asbp_jrpgplayer_controller "/Game/TurnBasedJRPGTemplate/Blueprints/Units/PlayerUnits/BP_PriestPlayerUnit.BP_PriestPlayerUnit_C" 0)
                          (`/Game/TurnBasedJRPGTemplate/Blueprints/Controllers/BP_JRPGPlayerController.AddToParty` _asbp_jrpgplayer_controller "/Game/TurnBasedJRPGTemplate/Blueprints/Units/PlayerUnits/BP_PriestPlayerUnit.BP_PriestPlayerUnit_C"))
                        (:`1`
                          _)))))
                (:`1`
                  (bind (_state_7 _optionindex_4) (`self.AddDialogue` "Placida" "I don't know exactly, he ran in that door and shouted at me to stay here, the problem is that a kind of wall of flesh has formed there, it's not aggressive, but it keeps releasing strange exhalations and I struggle to get rid of it." (`|MakeArray` "Step aside I'll take care of it" " You can join me, together we could do it" :!type "Text")))
                  (switch `/Game/DialogueSystem/Blueprints/Enum_DialogueState` _state_7
                    (:`NewEnumerator0`
                      (switch `int` _optionindex_4
                        (:`0`
                          _)
                        (:`1`
                          (goto _label)))))))
              (`CharacterMovementComponent.SetMovementMode` (`Character.CharacterMovement` (`GameplayStatics.GetPlayerCharacter` 0)) "MOVE_Walking" 0)
              (`self.CloseConversation`))))))))