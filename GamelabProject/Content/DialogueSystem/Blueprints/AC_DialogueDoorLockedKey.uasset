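; Dialogue component that runs the conversation for a key-locked door.
; Its Dialogue override checks the JRPG player controller's MiscItems for BP_Key, then offers to use it or shows a missing-key hint.
; Accepting removes one key and calls DoorOpening on the BP_DoorLockedKey found via GetActorOfClass, rather than a direct reference.
; Each ending rolls back dialogue progress by one and closes the conversation.
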(fn `Dialogue`
  (`parent.Dialogue`)
  (bind _state (`self.AddDialogue` "Door" "This door needs a key to open" (`|MakeArray` "Let me check" :!type "Text")))
  (switch `/Game/DialogueSystem/Blueprints/Enum_DialogueState` _state
    (:`NewEnumerator0`
      (bind _asbp_jrpgplayer_controller (cast `/Game/TurnBasedJRPGTemplate/Blueprints/Controllers/BP_JRPGPlayerController` (`GameplayStatics.GetPlayerController` 0)))
      (if (`.ReturnValue` (`BlueprintMapLibrary.Map_Find` (`/Game/TurnBasedJRPGTemplate/Blueprints/Controllers/BP_JRPGPlayerController.miscItems` _asbp_jrpgplayer_controller) "/Game/TurnBasedJRPGTemplate/Blueprints/Items/MiscItems/BP_Key.BP_Key_C"))
        (bind (_state_2 _optionindex) (`self.AddDialogue` "Archer" "Use key" (`|MakeArray` "Yes" "No" :!type "Text")))
        (switch `/Game/DialogueSystem/Blueprints/Enum_DialogueState` _state_2
          (:`NewEnumerator0`
            (switch `int` _optionindex
              (:`0`
                (`self.RemoveDialogueProgress` 1)
                (`self.CloseConversation`)
                (bind _asbp_jrpgplayer_controller_2 (cast `/Game/TurnBasedJRPGTemplate/Blueprints/Controllers/BP_JRPGPlayerController` (`GameplayStatics.GetPlayerController` 0)))
                (`/Game/TurnBasedJRPGTemplate/Blueprints/Controllers/BP_JRPGPlayerController.RemoveItemFromInventory` _asbp_jrpgplayer_controller_2 "/Game/TurnBasedJRPGTemplate/Blueprints/Items/MiscItems/BP_Key.BP_Key_C" 1)
                (bind _returnvalue (`GameplayStatics.GetActorOfClass` "/Game/Blueprints/01_DoorBP/BP_DoorLockedKey.BP_DoorLockedKey_C"))
                (`/Game/Blueprints/01_DoorBP/BP_DoorLockedKey.DoorOpening` _returnvalue))
              (:`1`
                (bind _state_3 (`self.AddDialogue` "Door" "Rip" (`|MakeArray` "Leave" :!type "Text")))
                (switch `/Game/DialogueSystem/Blueprints/Enum_DialogueState` _state_3
                  (:`NewEnumerator0`
                    (`self.RemoveDialogueProgress` 1)
                    (`self.CloseConversation`)))))))
        (else
          (bind _state_4 (`self.AddDialogue` "Archer" "I don't have the key, come back when you do. I think I left it in a chest somewhere around here." (`|MakeArray` "Leave" :!type "Text")))
          (switch `/Game/DialogueSystem/Blueprints/Enum_DialogueState` _state_4
            (:`NewEnumerator0`
              (`self.RemoveDialogueProgress` 1)
              (`self.CloseConversation`))))))))