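; Dialogue component for the Archer NPC, who joins the player's party in exchange for a stone.
; Overrides Dialogue as a branching tree of AddDialogue nodes that continue on Pass Through and branch on option index.
; Checks the JRPG player controller's MiscItems for BP_Stone; accepting removes one, adds the archer unit and destroys the owning actor.
; Other endings close the conversation, stepping back or clearing dialogue progress.
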(fn `Dialogue`
  (`parent.Dialogue`)
  (bind (_state _optionindex) (`self.AddDialogue` "Archer" "I will join your party, if you bring me stone." (`|MakeArray` "Cool" "I don't need your help" :!type "Text")))
  (switch `/Game/DialogueSystem/Blueprints/Enum_DialogueState` _state
    (:`NewEnumerator0`
      (switch `int` _optionindex
        (:`0`
          (bind _state_2 (`self.AddDialogue` "Archer" "Do you have a stone?" (`|MakeArray` "Let me check" :!type "Text")))
          (switch `/Game/DialogueSystem/Blueprints/Enum_DialogueState` _state_2
            (:`NewEnumerator0`
              (bind _asbp_jrpgplayer_controller (cast `/Game/TurnBasedJRPGTemplate/Blueprints/Controllers/BP_JRPGPlayerController` (`GameplayStatics.GetPlayerController` 0)))
              (if (`.ReturnValue` (`BlueprintMapLibrary.Map_Find` (`/Game/TurnBasedJRPGTemplate/Blueprints/Controllers/BP_JRPGPlayerController.miscItems` _asbp_jrpgplayer_controller) "/Game/TurnBasedJRPGTemplate/Blueprints/Items/MiscItems/BP_Stone.BP_Stone_C"))
                (bind (_state_3 _optionindex_2) (`self.AddDialogue` "Archer" "Ahh, I see you have stone! Give it to me and I'll join your party." (`|MakeArray` "Sure" "No" :!type "Text")))
                (switch `/Game/DialogueSystem/Blueprints/Enum_DialogueState` _state_3
                  (:`NewEnumerator0`
                    (switch `int` _optionindex_2
                      (:`0`
                        (bind _state_4 (`self.AddDialogue` "Archer" "Good job, let's go now." (`|MakeArray` "Goodbye" :!type "Text")))
                        (switch `/Game/DialogueSystem/Blueprints/Enum_DialogueState` _state_4
                          (:`NewEnumerator0`
                            (`self.RemoveDialogueProgress` 1)
                            (`self.CloseConversation`)
                            (bind _asbp_jrpgplayer_controller_2 (cast `/Game/TurnBasedJRPGTemplate/Blueprints/Controllers/BP_JRPGPlayerController` (`GameplayStatics.GetPlayerController` 0)))
                            (`/Game/TurnBasedJRPGTemplate/Blueprints/Controllers/BP_JRPGPlayerController.RemoveItemFromInventory` _asbp_jrpgplayer_controller_2 "/Game/TurnBasedJRPGTemplate/Blueprints/Items/MiscItems/BP_Stone.BP_Stone_C" 1)
                            (`/Game/TurnBasedJRPGTemplate/Blueprints/Controllers/BP_JRPGPlayerController.AddPlayerUnit` _asbp_jrpgplayer_controller_2 "/Game/TurnBasedJRPGTemplate/Blueprints/Units/PlayerUnits/BP_ArcherPlayerUnit.BP_ArcherPlayerUnit_C" 0)
                            (`Actor.K2_DestroyActor` (`self.GetOwner`)))))
                      (:`1`
                        (bind _state_5 (`self.AddDialogue` "Archer" "Whatever, come back if you change your mind." (`|MakeArray` "(Leave)" :!type "Text")))
                        (switch `/Game/DialogueSystem/Blueprints/Enum_DialogueState` _state_5
                          (:`NewEnumerator0`
                            (`self.RemoveDialogueProgress` 1)
                            (`self.CloseConversation`)))))))
                (else
                  (bind _state_6 (`self.AddDialogue` "Archer" "You don't have any, come back when you do." (`|MakeArray` "(Leave)" :!type "Text")))
                  (switch `/Game/DialogueSystem/Blueprints/Enum_DialogueState` _state_6
                    (:`NewEnumerator0`
                      (`self.RemoveDialogueProgress` 1)
                      (`self.CloseConversation`))))))))
        (:`1`
          (bind _state_7 (`self.AddDialogue` "Archer" "Whatever, come back if you change your mind." (`|MakeArray` "(Leave)" :!type "Text")))
          (switch `/Game/DialogueSystem/Blueprints/Enum_DialogueState` _state_7
            (:`NewEnumerator0`
              (`self.ClearDialogueProgress`)
              (`self.CloseConversation`))))))))