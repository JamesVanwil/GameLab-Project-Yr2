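; Dialogue component for the NPC Jerome, giving his line about guarding the last crate of alcohol.
; Overrides Dialogue to call the parent, disable the player character's movement, then add the line with two player reply options.
; On the Pass Through state, it clears dialogue progress, closes the conversation and restores walking movement, with no separate branch per reply.
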(fn `Dialogue`
  (`parent.Dialogue`)
  (`CharacterMovementComponent.SetMovementMode` (`Character.CharacterMovement` (`GameplayStatics.GetPlayerCharacter` 0)) "MOVE_None" 0)
  (bind _state (`self.AddDialogue` "Jerome" "Inside that crate are the last supplies of alcohol. Monsters from other dimensions may kill me but they will never have me sober." (`|MakeArray` "Cheers!" "Strange philosophy of life man." :!type "Text")))
  (switch `/Game/DialogueSystem/Blueprints/Enum_DialogueState` _state
    (:`NewEnumerator0`
      (`self.ClearDialogueProgress`)
      (`self.CloseConversation`)
      (`CharacterMovementComponent.SetMovementMode` (`Character.CharacterMovement` (`GameplayStatics.GetPlayerCharacter` 0)) "MOVE_Walking" 0))))