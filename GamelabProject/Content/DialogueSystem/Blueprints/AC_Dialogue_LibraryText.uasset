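; AC_Dialogue_LibraryText is a dialogue component that shows Roland's remark about the library's books on American history, duck hunting and finance.
; Its Dialogue function calls the parent, freezes the player by setting movement mode to None, and adds one line with a single Leave option.
; On pass-through it clears dialogue progress, closes the conversation and restores walking.
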(fn `Dialogue`
  (`parent.Dialogue`)
  (`CharacterMovementComponent.SetMovementMode` (`Character.CharacterMovement` (`GameplayStatics.GetPlayerCharacter` 0)) "MOVE_None" 0)
  (bind _state (`self.AddDialogue` "Roland" "The library is full of books on the history of America, duck hunting and finance." (`|MakeArray` "(Leave)" :!type "Text")))
  (switch `/Game/DialogueSystem/Blueprints/Enum_DialogueState` _state
    (:`NewEnumerator0`
      (`self.ClearDialogueProgress`)
      (`self.CloseConversation`)
      (`CharacterMovementComponent.SetMovementMode` (`Character.CharacterMovement` (`GameplayStatics.GetPlayerCharacter` 0)) "MOVE_Walking" 0))))