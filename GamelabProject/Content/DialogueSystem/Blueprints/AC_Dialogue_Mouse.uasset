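; Dialogue component for the Mouse NPC, which begs the player for cheese and remembers whether it received any.
; Overrides Dialogue, switching on the active branch and chaining AddDialogue nodes whose option index picks the next line.
; Giving cheese saves the GivenCheese branch, so later talks show one of two random happy lines.
; Other endings clear dialogue progress and close the conversation.
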(fn `Dialogue`
  (`parent.Dialogue`)
  (switch `name` (`self.ActiveDialogueBranch`)
    (:`Default`
      (bind (_state _optionindex) (`self.AddDialogue` "Mouse" "Hi, do you have any cheese?" (`|MakeArray` "Yes" "No" :!type "Text")))
      (switch `/Game/DialogueSystem/Blueprints/Enum_DialogueState` _state
        (:`NewEnumerator0`
          (switch `int` _optionindex
            (:`0`
              (bind (_state_2 _optionindex_2) (`self.AddDialogue` "Mouse" "Wow, really? That's amazing :) Can I have some?" (`|MakeArray` "Give Cheese" "Keep Cheese" :!type "Text")))
              (switch `/Game/DialogueSystem/Blueprints/Enum_DialogueState` _state_2
                (:`NewEnumerator0`
                  (switch `int` _optionindex_2
                    (:`0`
                      (bind _state_3 (`self.AddDialogue` "Mouse" "Thank you, THANK YOU!!!" (`|MakeArray` "Continue" :!type "Text")))
                      (switch `/Game/DialogueSystem/Blueprints/Enum_DialogueState` _state_3
                        (:`NewEnumerator0`
                          (`self.SetDialogueBranch` "GivenCheese")
                          (`self.CloseConversation`))))
                    (:`1`
                      (bind _state_4 (`self.AddDialogue` "Mouse" "Fuck you, bitch." (`|MakeArray` "Continue" :!type "Text")))
                      (switch `/Game/DialogueSystem/Blueprints/Enum_DialogueState` _state_4
                        (:`NewEnumerator0`
                          (`self.ClearDialogueProgress`)
                          (`self.CloseConversation`))))))))
            (:`1`
              (bind _state_5 (`self.AddDialogue` "Mouse" "Awww, that's too bad. I really want some cheese!" (`|MakeArray` "Continue" :!type "Text")))
              (switch `/Game/DialogueSystem/Blueprints/Enum_DialogueState` _state_5
                (:`NewEnumerator0`
                  (`self.ClearDialogueProgress`)
                  (`self.CloseConversation`))))))))
    (:`GivenCheese`
      (bind _state_6 (`self.AddDialogue` "Mouse" (select `int` (`KismetMathLibrary.RandomIntegerInRange` 0 1) :`0` "You're such a nice person!" :`1` "Nom Nom Nom" :!type "Text") (`|MakeArray` "Continue" :!type "Text")))
      (switch `/Game/DialogueSystem/Blueprints/Enum_DialogueState` _state_6
        (:`NewEnumerator0`
          (`self.ClearDialogueProgress`)
          (`self.CloseConversation`))))))