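; Dialogue component for James, who tells Roland that the trapped Henry may know a safe way out.
; The overridden Dialogue function calls its parent, then builds a branching conversation from nested AddDialogue calls, switching on state and chosen option.
; Agreeing to help rewards bandages, added to the JRPG player controller's inventory as a red potion.
; Both branches remove dialogue progress, close the conversation and destroy the James NPC found by class.
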(fn `Dialogue`
  (`parent.Dialogue`)
  (bind (_state _optionindex) (`self.AddDialogue` "James" "Henry is trapped in the room next to ours, he probably knows how to escape safely from here" (`|MakeArray` "I'll try to do my best" "We don't need him" :!type "Text")))
  (switch `/Game/DialogueSystem/Blueprints/Enum_DialogueState` _state
    (:`NewEnumerator0`
      (switch `int` _optionindex
        (:`0`
          (bind _state_2 (`self.AddDialogue` "James" "Thank you Roland, take this, it may be useful to you" (`|MakeArray` "Take bandages" :!type "Text")))
          (switch `/Game/DialogueSystem/Blueprints/Enum_DialogueState` _state_2
            (:`NewEnumerator0`
              (bind _asbp_jrpgplayer_controller (cast `/Game/TurnBasedJRPGTemplate/Blueprints/Controllers/BP_JRPGPlayerController` (`GameplayStatics.GetPlayerController` 0)))
              (`/Game/TurnBasedJRPGTemplate/Blueprints/Controllers/BP_JRPGPlayerController.AddUsableItemToInventory` _asbp_jrpgplayer_controller "/Game/TurnBasedJRPGTemplate/Blueprints/Items/UsableItems/BP_RedPotion.BP_RedPotion_C" 1)
              (`self.RemoveDialogueProgress` 1)
              (`self.CloseConversation`)
              (bind _returnvalue (`GameplayStatics.GetActorOfClass` "/Game/DialogueSystem/Blueprints/NPC_Base_Human_James.NPC_Base_Human_James_C"))
              (`Actor.K2_DestroyActor` _returnvalue))))
        (:`1`
          (bind _state_3 (`self.AddDialogue` "James" "I look forward to seeing your plan in action then" (`|MakeArray` "Leave" :!type "Text")))
          (switch `/Game/DialogueSystem/Blueprints/Enum_DialogueState` _state_3
            (:`NewEnumerator0`
              (`self.RemoveDialogueProgress` 1)
              (`self.CloseConversation`)
              (bind _returnvalue_2 (`GameplayStatics.GetActorOfClass` "/Game/DialogueSystem/Blueprints/NPC_Base_Human_James.NPC_Base_Human_James_C"))
              (`Actor.K2_DestroyActor` _returnvalue_2))))))))