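; Dialogue component for Plàcida's "before" conversation, in which she threatens a supposed monster, then recognises Roland.
; The Dialogue override calls its parent, then chains two AddDialogue exchanges, each with a single reply option and advancing on the Pass Through state.
; After the second exchange it closes the conversation and sets the player's BP_MageCharacter movement mode back to Walking.
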(fn `Dialogue`
  (`parent.Dialogue`)
  (bind _state (`self.AddDialogue` "Placida" "Stop there monster! Si das un paso más, te mato!" (`|MakeArray` "Plàcida stop! It's me! Roland!" :!type "Text")))
  (switch `/Game/DialogueSystem/Blueprints/Enum_DialogueState` _state
    (:`NewEnumerator0`
      (bind _state_2 (`self.AddDialogue` "Placida" "Roland! I don't believe it! You scared me! But I'm so happy to know it's you and that you're safe and sound! \nThe same can't be said for me." (`|MakeArray` "..." :!type "Text")))
      (switch `/Game/DialogueSystem/Blueprints/Enum_DialogueState` _state_2
        (:`NewEnumerator0`
          (`self.CloseConversation`)
          (bind _asbp_mage_character (cast `/Game/TurnBasedJRPGTemplate/Blueprints/PlayerPawns/BP_MageCharacter` (`GameplayStatics.GetPlayerCharacter` 0)))
          (`CharacterMovementComponent.SetMovementMode` (`Character.CharacterMovement` _asbp_mage_character) "MOVE_Walking" 0))))))