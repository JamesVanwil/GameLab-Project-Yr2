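; Dialogue component for a medkit pickup that lets the player take two Gauze or leave it.
; The Dialogue override calls its parent, freezes player movement and shows a Take/Leave prompt through AddDialogue, branching on the returned option.
; Take adds the Gauze through BP_JRPGPlayerController, destroys the owning actor and plays a sound, while Leave clears dialogue progress.
; Both choices close the conversation and restore walking.
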(fn `Dialogue`
  (`parent.Dialogue`)
  (`CharacterMovementComponent.SetMovementMode` (`Character.CharacterMovement` (`GameplayStatics.GetPlayerCharacter` 0)) "MOVE_None" 0)
  (bind (_state _optionindex) (`self.AddDialogue` "" "A closed Medkit, there are 2 Gauze inside." (`|MakeArray` "(Take)" "(Leave)" :!type "Text")))
  (switch `/Game/DialogueSystem/Blueprints/Enum_DialogueState` _state
    (:`NewEnumerator0`
      (switch `int` _optionindex
        (:`0`
          (bind _asbp_jrpgplayer_controller (cast `/Game/TurnBasedJRPGTemplate/Blueprints/Controllers/BP_JRPGPlayerController` (`GameplayStatics.GetPlayerController` 0)))
          (`/Game/TurnBasedJRPGTemplate/Blueprints/Controllers/BP_JRPGPlayerController.AddUsableItemToInventory` _asbp_jrpgplayer_controller "/Game/TurnBasedJRPGTemplate/Blueprints/Items/UsableItems/BP_Gauze.BP_Gauze_C" 2)
          (`Actor.K2_DestroyActor` (`self.GetOwner`))
          (`self.CloseConversation`)
          (`GameplayStatics.PlaySound2D` "/Game/Audio/equipmaxingShort.equipmaxingShort" 1.0 1.0 0.0 null null)
          (`CharacterMovementComponent.SetMovementMode` (`Character.CharacterMovement` (`GameplayStatics.GetPlayerCharacter` 0)) "MOVE_Walking" 0))
        (:`1`
          (`self.ClearDialogueProgress`)
          (`self.CloseConversation`)
          (`CharacterMovementComponent.SetMovementMode` (`Character.CharacterMovement` (`GameplayStatics.GetPlayerCharacter` 0)) "MOVE_Walking" 0))))))