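; Dialogue Blueprint for the WallLeaper, a "???" speaker who offers to trade a party member's ability.
; It freezes player movement and runs branching AddDialogue prompts.
; Only Harper's "Power of knowledge" trade is implemented, swapping BP_MagePlayerUnit's equipment for BP_BookWeapon through the JRPG player controller; Roland's branch is a stub.
; A completed trade sets IsSkillChanged, restores walking and closes the conversation, so later talks show only a brief taunt.
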(fn `Dialogue`
  (`parent.Dialogue`)
  (`CharacterMovementComponent.SetMovementMode` (`Character.CharacterMovement` (`GameplayStatics.GetPlayerCharacter` 0)) "MOVE_None" 0)
  (if (`self.IsSkillChanged?`)
    (bind _state (`self.AddDialogue` "???" "This is not very sigma of you" (`|MakeArray` "I always knew you were a beta" :!type "Text")))
    (switch `/Game/DialogueSystem/Blueprints/Enum_DialogueState` _state
      (:`NewEnumerator0`
        (`CharacterMovementComponent.SetMovementMode` (`Character.CharacterMovement` (`GameplayStatics.GetPlayerCharacter` 0)) "MOVE_Walking" 0)
        (`self.CloseConversation`)))
    (else
      (bind _state_2 (`self.AddDialogue` "???" "Well hello Cowboy, you finally decided to come closer :) how are you in this beautiful snowy evening?" (`|MakeArray` "W-what are you? Are you a monster too?" "How can you say that? Hundreds of people died because of you and your friends!" "..." :!type "Text")))
      (switch `/Game/DialogueSystem/Blueprints/Enum_DialogueState` _state_2
        (:`NewEnumerator0`
          (bind _state_3 (`self.AddDialogue` "???" "Lets talk about business" (`|MakeArray` "Ok" :!type "Text")))
          (switch `/Game/DialogueSystem/Blueprints/Enum_DialogueState` _state_3
            (:`NewEnumerator0`
              (bind (_state_4 _optionindex) (`self.AddDialogue` "???" "Who do you want to acquire the new ability?" (`|MakeArray` "Harper" "Roland" :!type "Text")))
              (switch `/Game/DialogueSystem/Blueprints/Enum_DialogueState` _state_4
                (:`NewEnumerator0`
                  (switch `int` _optionindex
                    (:`0`
                      (bind (_state_5 _optionindex_2) (`self.AddDialogue` "???" "Which ability do you want to trade?" (`|MakeArray` "Power of knowledge" "High Understanding" "First aid" :!type "Text")))
                      (switch `/Game/DialogueSystem/Blueprints/Enum_DialogueState` _state_5
                        (:`NewEnumerator0`
                          (switch `int` _optionindex_2
                            (:`0`
                              (`KismetSystemLibrary.PrintString` "Remove power of knowledge")
                              (bind _asbp_jrpgplayer_controller (cast `/Game/TurnBasedJRPGTemplate/Blueprints/Controllers/BP_JRPGPlayerController` (`GameplayStatics.GetPlayerController` 0)))
                              (bind _keys (`BlueprintMapLibrary.Map_Keys` (`/Game/TurnBasedJRPGTemplate/Blueprints/Controllers/BP_JRPGPlayerController.playerUnits` _asbp_jrpgplayer_controller)))
                              (for _array_element _keys
                                (if (== _array_element "/Game/TurnBasedJRPGTemplate/Blueprints/Units/PlayerUnits/BP_MagePlayerUnit.BP_MagePlayerUnit_C")
                                  (`/Game/TurnBasedJRPGTemplate/Blueprints/Controllers/BP_JRPGPlayerController.RemoveEquipmentOnUnit` _asbp_jrpgplayer_controller _array_element "NewEnumerator0")
                                  (`/Game/TurnBasedJRPGTemplate/Blueprints/Controllers/BP_JRPGPlayerController.WearEquipmentOnUnit` _asbp_jrpgplayer_controller "/Game/TurnBasedJRPGTemplate/Blueprints/Units/PlayerUnits/BP_MagePlayerUnit.BP_MagePlayerUnit_C" "/Game/TurnBasedJRPGTemplate/Blueprints/Items/Equipment/Weapons/BP_BookWeapon.BP_BookWeapon_C")
                                  (set `self.IsSkillChanged?` true)
                                  (`CharacterMovementComponent.SetMovementMode` (`Character.CharacterMovement` (`GameplayStatics.GetPlayerCharacter` 0)) "MOVE_Walking" 0)
                                  (`self.ClearDialogueProgress`)
                                  (`self.CloseConversation`))))))))
                    (:`1`
                      (`self.AddDialogue` "???" "Who do you want to acquire the new ability?"))))))))))))