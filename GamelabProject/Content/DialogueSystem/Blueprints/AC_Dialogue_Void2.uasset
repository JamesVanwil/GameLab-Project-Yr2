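; Dialogue component for a mysterious sphere encounter, where an unnamed speaker offers a choice to look inside or ignore it.
; The Dialogue override calls its parent, disables player movement, then branches on AddDialogue's state and chosen option.
; Looking inside shows a vision of women burning a bound person.
; Both paths end by restoring walking, closing the conversation and clearing dialogue progress.
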(fn `Dialogue`
  (`parent.Dialogue`)
  (`CharacterMovementComponent.SetMovementMode` (`Character.CharacterMovement` (`GameplayStatics.GetPlayerCharacter` 0)) "MOVE_None" 0)
  (bind (_state _optionindex) (`self.AddDialogue` "???" "The sphere seems to release a familiar light" (`|MakeArray` "[looks inside]" "[ignores]" :!type "Text")))
  (switch `/Game/DialogueSystem/Blueprints/Enum_DialogueState` _state
    (:`NewEnumerator0`
      (switch `int` _optionindex
        (:`0`
          (bind _state_2 (`self.AddDialogue` "???" "You see women surrounding, binding and setting fire to a living person" (`|MakeArray` "Leave" :!type "Text")))
          (switch `/Game/DialogueSystem/Blueprints/Enum_DialogueState` _state_2
            (:`NewEnumerator0`
              _)))
        (:`1`
          _))
      (`CharacterMovementComponent.SetMovementMode` (`Character.CharacterMovement` (`GameplayStatics.GetPlayerCharacter` 0)) "MOVE_Walking" 0)
      (`self.CloseConversation`)
      (`self.ClearDialogueProgress`))))