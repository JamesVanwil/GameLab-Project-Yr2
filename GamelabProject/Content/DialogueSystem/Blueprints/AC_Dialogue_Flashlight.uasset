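; Dialogue component for the flashlight pickup, letting the player take the flashlight or leave it in place.
; The overridden Dialogue function disables player movement and presents both options, restoring walking once the conversation closes.
; Taking it adds flashlight equipment through the JRPG player controller and destroys the NPC_Base_Flashlight actor found by class lookup.
; Leaving it clears dialogue progress.
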(fn `Dialogue`
  (`parent.Dialogue`)
  (`CharacterMovementComponent.SetMovementMode` (`Character.CharacterMovement` (`GameplayStatics.GetPlayerCharacter` 0)) "MOVE_None" 0)
  (bind (_state _optionindex) (`self.AddDialogue` "" "A flashlgiht, might come in handy" (`|MakeArray` "Take it" "Leave in place" :!type "Text")))
  (switch `/Game/DialogueSystem/Blueprints/Enum_DialogueState` _state
    (:`NewEnumerator0`
      (switch `int` _optionindex
        (:`0`
          (bind _asbp_jrpgplayer_controller (cast `/Game/TurnBasedJRPGTemplate/Blueprints/Controllers/BP_JRPGPlayerController` (`GameplayStatics.GetPlayerController` 0)))
          (`/Game/TurnBasedJRPGTemplate/Blueprints/Controllers/BP_JRPGPlayerController.AddEquipmentToInventory` _asbp_jrpgplayer_controller "/Game/TurnBasedJRPGTemplate/Blueprints/Items/Equipment/Shields/BP_FlashlightEquipment.BP_FlashlightEquipment_C" 1)
          (bind _returnvalue (`GameplayStatics.GetActorOfClass` "/Game/DialogueSystem/Blueprints/NPC_Base_Flashlight.NPC_Base_Flashlight_C"))
          (`Actor.K2_DestroyActor` _returnvalue)
          (`self.CloseConversation`)
          (`CharacterMovementComponent.SetMovementMode` (`Character.CharacterMovement` (`GameplayStatics.GetPlayerCharacter` 0)) "MOVE_Walking" 0))
        (:`1`
          (`self.ClearDialogueProgress`)
          (`self.CloseConversation`)
          (`CharacterMovementComponent.SetMovementMode` (`Character.CharacterMovement` (`GameplayStatics.GetPlayerCharacter` 0)) "MOVE_Walking" 0))))))