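; Interactable secret book NPC that runs a dialogue and can open the library's secret bookshelf door.
; On BeginPlay it binds its child BP_InteractionDetector to open the ACDialogueSecretBook conversation, and re-enables and refreshes interaction when the conversation closes.
; OpenLibraryDoor finds BP_SecretDoorBookShelf by class and snaps its root to a fixed rotation.
; Timeline and interaction-widget visibility logic is disconnected, and the capsule overlap events are empty.
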(event `self.ReceiveBeginPlay`
  ;[1 1 1] Setup Interaction
  (bind _asbp_interaction_detector (cast `/Game/TurnBasedJRPGTemplate/Blueprints/Interactables/BP_InteractionDetector` (`ChildActorComponent.ChildActor` (`self.InteractionActor`))))
  (bind _output_get (set `self.As BP Interaction Detector` _asbp_interaction_detector))
  (add `/Game/TurnBasedJRPGTemplate/Blueprints/Interactables/BP_InteractionDetector.OnInteracted` _output_get (delegate `StartConversation`))
  (add `/Game/DialogueSystem/Blueprints/AC_Dialogue_Base.Close Conversation` (`self.AC_DialogueSecretBook`) (delegate `ResetDialogueInteraction`)))

(event `StartConversation`
  ;[1 1 1] Setup Interaction
  (`/Game/DialogueSystem/Blueprints/AC_Dialogue_Base.OpenConversation` (`self.AC_DialogueSecretBook`)))

(event `ResetDialogueInteraction`
  (bind _as_bp_interaction_detector (`self.As BP Interaction Detector`))
  ;[1 1 1] Setup Interaction
  (`/Game/TurnBasedJRPGTemplate/Blueprints/Interactables/BP_InteractionDetector.EnableInteraction` _as_bp_interaction_detector)
  (`/Game/TurnBasedJRPGTemplate/Blueprints/Controllers/BP_JRPGPlayerController.RefreshInteractions` (`/Game/TurnBasedJRPGTemplate/Blueprints/Interactables/BP_InteractionDetector.jRPGPlayerController` _as_bp_interaction_detector)))

(event `/Game/DialogueSystem/Blueprints/BPI_Interactable.Interact`
  (params (Instigator :type "Actor Object Reference"))
  (set `self.InteractInstigator` Instigator))

(event `OpenLibraryDoor`
  (bind _returnvalue (`GameplayStatics.GetActorOfClass` "/Game/BP_SecretDoorBookShelf.BP_SecretDoorBookShelf_C"))
  (`SceneComponent.K2_SetWorldRotation` (`Actor.RootComponent` _returnvalue) (struct :`Yaw` 135.0) false false))

(event `self.CapsuleComponent.OnComponentBeginOverlap`
  (params (OverlappedComponent :type "PrimitiveComponent Object Reference") (OtherActor :type "Actor Object Reference") (OtherComp :type "PrimitiveComponent Object Reference") (OtherBodyIndex :type Integer) (bFromSweep :type Boolean) (SweepResult :type "HitResult Structure (by ref)")))

(event `self.CapsuleComponent.OnComponentEndOverlap`
  (params (OverlappedComponent :type "PrimitiveComponent Object Reference") (OtherActor :type "Actor Object Reference") (OtherComp :type "PrimitiveComponent Object Reference") (OtherBodyIndex :type Integer)))

(fn `UserConstructionScript`
  (`parent.UserConstructionScript`))