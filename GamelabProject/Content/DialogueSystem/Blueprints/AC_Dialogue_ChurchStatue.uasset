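; Dialogue component for the church statue, with branching conversations that depend on whether a BP_PriestCharacter exists in the level.
; With the priest present Placida speaks, otherwise Roland does, while player movement is disabled.
; Choosing prayer shows a speaker-specific WBP_VoidText message.
; Endings close the conversation and restore walking, except Roland's prayer, which stops at an empty loop over party units.
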(fn `Dialogue`
  (`parent.Dialogue`)
  (bind _returnvalue (`GameplayStatics.GetActorOfClass` "/Game/TurnBasedJRPGTemplate/Blueprints/PlayerPawns/BP_PriestCharacter.BP_PriestCharacter_C"))
  (`/Engine/EditorBlueprintResources/StandardMacros.IsValid` _returnvalue
    (:`Is Valid`
      (`CharacterMovementComponent.SetMovementMode` (`Character.CharacterMovement` (`GameplayStatics.GetPlayerCharacter` 0)) "MOVE_None" 0)
      (bind (_state _optionindex) (`self.AddDialogue` "Placida" "Whenever I see the statue of the Virgin Mary, I always think how lucky we are to be observed and protected from above by such a sweet, kind and beautiful woman. " (`|MakeArray` "I don't think Mary is helping us at all right now" "Could you say a prayer for us? " :!type "Text")))
      (switch `/Game/DialogueSystem/Blueprints/Enum_DialogueState` _state
        (:`NewEnumerator0`
          (switch `int` _optionindex
            (:`0`
              (bind _state_2 (`self.AddDialogue` "Placida" "HOW CAN YOU SAY SUCH THINGS! Mary is always watching us from above and wants only the best for us, it is we who do not understand her painting! Don't ever say such a thing again or I'll slaughter you like those beasts! I DON'T CARE IF YOU ARE A MAN!" (`|MakeArray` "..." :!type "Text")))
              (switch `/Game/DialogueSystem/Blueprints/Enum_DialogueState` _state_2
                (:`NewEnumerator0`
                  _)))
            (:`1`
              (bind _state_3 (`self.AddDialogue` "Placida" "“Hail Mary, \nfull of Grace, \nthe Lord is with thee. \nblessed art thou among women, \nand blessed is the fruit of thy womb, Jesus. \nHoly Mary, Mother of God, \npray for us sinners \nnow, and at the hour of death.\"" (`|MakeArray` "Amen" :!type "Text")))
              (switch `/Game/DialogueSystem/Blueprints/Enum_DialogueState` _state_3
                (:`NewEnumerator0`
                  (bind _returnvalue_2 (`|CreateWidget` "/Game/TheVoid/WBP_VoidText.WBP_VoidText_C"))
                  (`/Game/TheVoid/WBP_VoidText.ShowPlacidaStatueText` _returnvalue_2)))))
          (`self.CloseConversation`)
          (`CharacterMovementComponent.SetMovementMode` (`Character.CharacterMovement` (`GameplayStatics.GetPlayerCharacter` 0)) "MOVE_Walking" 0))))
    (:`Is Not Valid`
      (`CharacterMovementComponent.SetMovementMode` (`Character.CharacterMovement` (`GameplayStatics.GetPlayerCharacter` 0)) "MOVE_None" 0)
      (bind (_state_4 _optionindex_2) (`self.AddDialogue` "Roland" "I have never been a great believer....  \nBut in this situation this place makes me feel safe even for a little while" (`|MakeArray` "..." "Pray" :!type "Text")))
      (switch `/Game/DialogueSystem/Blueprints/Enum_DialogueState` _state_4
        (:`NewEnumerator0`
          (switch `int` _optionindex_2
            (:`0`
              (`self.CloseConversation`)
              (`CharacterMovementComponent.SetMovementMode` (`Character.CharacterMovement` (`GameplayStatics.GetPlayerCharacter` 0)) "MOVE_Walking" 0))
            (:`1`
              (bind _state_5 (`self.AddDialogue` "Roland" "Praying calmed your spirit" (`|MakeArray` "..." :!type "Text")))
              (switch `/Game/DialogueSystem/Blueprints/Enum_DialogueState` _state_5
                (:`NewEnumerator0`
                  (bind _returnvalue_3 (`|CreateWidget` "/Game/TheVoid/WBP_VoidText.WBP_VoidText_C"))
                  (`/Game/TheVoid/WBP_VoidText.ShowRolandSatuteText` _returnvalue_3)
                  (bind _asbp_jrpgplayer_controller (cast `/Game/TurnBasedJRPGTemplate/Blueprints/Controllers/BP_JRPGPlayerController` (`GameplayStatics.GetPlayerController` 0)))
                  (bind _keys (`BlueprintMapLibrary.Map_Keys` (`/Game/TurnBasedJRPGTemplate/Blueprints/Controllers/BP_JRPGPlayerController.playerUnits` _asbp_jrpgplayer_controller)))
                  (for _ _keys
                    _))))))))))