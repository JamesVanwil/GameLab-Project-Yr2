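; Dialogue component for a battery pickup that explains the item, which refills half the flashlight's charge, and offers Take or Leave.
; The overridden Dialogue function freezes player movement, then branches on the chosen option.
; Take plays a sound, adds the battery to the JRPG controller's inventory and destroys the first NPC_Battery found by class.
; Leave clears dialogue progress; both choices close the conversation and restore walking.
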(fn `Dialogue`
  (`parent.Dialogue`)
  (`CharacterMovementComponent.SetMovementMode` (`Character.CharacterMovement` (`GameplayStatics.GetPlayerCharacter` 0)) "MOVE_None" 0)
  (bind (_state _optionindex) (`self.AddDialogue` "" "A battery. Use it from the inventory to refill half of the flashlight's charge." (`|MakeArray` "Take" "Leave" :!type "Text")))
  (switch `/Game/DialogueSystem/Blueprints/Enum_DialogueState` _state
    (:`NewEnumerator0`
      (switch `int` _optionindex
        (:`0`
          (`GameplayStatics.PlaySound2D` "/Game/Audio/equipmaxingShort.equipmaxingShort" 1.0 1.0 0.0 null null)
          (bind _asbp_jrpgplayer_controller (cast `/Game/TurnBasedJRPGTemplate/Blueprints/Controllers/BP_JRPGPlayerController` (`GameplayStatics.GetPlayerController` 0)))
          (`/Game/TurnBasedJRPGTemplate/Blueprints/Controllers/BP_JRPGPlayerController.AddUsableItemToInventory` _asbp_jrpgplayer_controller "/Game/Blueprints/PickUps/BP_BatteryPickUp.BP_BatteryPickUp_C" 1)
          (bind _returnvalue (`GameplayStatics.GetActorOfClass` "/Game/DialogueSystem/Blueprints/NPC_Battery.NPC_Battery_C"))
          (`Actor.K2_DestroyActor` _returnvalue)
          (`self.CloseConversation`)
          (`CharacterMovementComponent.SetMovementMode` (`Character.CharacterMovement` (`GameplayStatics.GetPlayerCharacter` 0)) "MOVE_Walking" 0))
        (:`1`
          (`self.ClearDialogueProgress`)
          (`self.CloseConversation`)
          (`CharacterMovementComponent.SetMovementMode` (`Character.CharacterMovement` (`GameplayStatics.GetPlayerCharacter` 0)) "MOVE_Walking" 0))))))