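; Piano NPC in the dialogue system that opens a conversation through its dialogue component when the player interacts with it.
; On BeginPlay it binds to the child interaction detector's interact event and the component's close-conversation event.
; Closing the conversation re-enables the detector and refreshes the player controller's interactions.
; A counter tracks interactions and plays a Pirates of the Caribbean piano track as an easter egg on exactly the tenth.
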(event `self.ReceiveBeginPlay`
  (bind _asbp_interaction_detector (cast `/Game/TurnBasedJRPGTemplate/Blueprints/Interactables/BP_InteractionDetector` (`ChildActorComponent.ChildActor` (`self.InteractionActor`))))
  (bind _output_get (set `self.As BP Interaction Detector` _asbp_interaction_detector))
  (add `/Game/TurnBasedJRPGTemplate/Blueprints/Interactables/BP_InteractionDetector.OnInteracted` _output_get (delegate `StartConversation`))
  (add `/Game/DialogueSystem/Blueprints/AC_Dialogue_Base.Close Conversation` (`self.AC_Dialogue_Piano`) (delegate `ResetDialogueInteraction`)))

(event `StartConversation`
  (`/Game/DialogueSystem/Blueprints/AC_Dialogue_Base.OpenConversation` (`self.AC_Dialogue_Piano`))
  (bind _result (`/Engine/EditorBlueprintResources/StandardMacros.IncrementInt` (`self.PianoCounter`))
    (:`  `
      (set `self.PianoCounter` _result)
      (if (== (`self.PianoCounter`) 10)
        (`GameplayStatics.PlaySound2D` "/Game/Audio/Pirates_Of_The_Caribbean__Easy_Piano_Tutorial___Synthesia-Sheet_Music_.Pirates_Of_The_Caribbean__Easy_Piano_Tutorial___Synthesia-Sheet_Music_" 1.0 1.0 0.0 null null)))))

(event `ResetDialogueInteraction`
  (bind _as_bp_interaction_detector (`self.As BP Interaction Detector`))
  (`/Game/TurnBasedJRPGTemplate/Blueprints/Interactables/BP_InteractionDetector.EnableInteraction` _as_bp_interaction_detector)
  (`/Game/TurnBasedJRPGTemplate/Blueprints/Controllers/BP_JRPGPlayerController.RefreshInteractions` (`/Game/TurnBasedJRPGTemplate/Blueprints/Interactables/BP_InteractionDetector.jRPGPlayerController` _as_bp_interaction_detector)))

(fn `UserConstructionScript`
  (`parent.UserConstructionScript`))