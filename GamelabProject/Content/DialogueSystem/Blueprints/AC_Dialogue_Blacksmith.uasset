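; Blacksmith NPC dialogue component that varies conversation by time of day and runs a small bread request.
; OpenConversation reads the instigating top-down test character's hour and selects the Morning, Afternoon or Night branch before calling the parent.
; Dialogue nests AddDialogue calls by state and chosen option, with afternoon lines gated by HasBread and HasGivenBread.
; Endings clear or step back progress before closing, and accepting the bread handover sets HasGivenBread.
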(fn `Dialogue`
  (`parent.Dialogue`)
  (switch `name` (`self.ActiveDialogueBranch`)
    (:`Morning`
      (bind _state (`self.AddDialogue` "Blacksmith" "Good morning!" (`|MakeArray` "Bye Bye!" :!type "Text")))
      (switch `/Game/DialogueSystem/Blueprints/Enum_DialogueState` _state
        (:`NewEnumerator0`
          (`self.ClearDialogueProgress`)
          (`self.CloseConversation`))))
    (:`Afternoon`
      (if (`self.bHasGivenBread?`)
        (bind _state_2 (`self.AddDialogue` "Blacksmith" "Thank you for the bread, friend!" (`|MakeArray` "No worries" :!type "Text")))
        (switch `/Game/DialogueSystem/Blueprints/Enum_DialogueState` _state_2
          (:`NewEnumerator0`
            (`self.ClearDialogueProgress`)
            (`self.CloseConversation`)))
        (else
          (bind (_state_3 _optionindex) (`self.AddDialogue` "Blacksmith" "Give me bread please, I haven't eaten all day" (`|MakeArray` "Yes" "No" :!type "Text")))
          (switch `/Game/DialogueSystem/Blueprints/Enum_DialogueState` _state_3
            (:`NewEnumerator0`
              (switch `int` _optionindex
                (:`0`
                  (bind _state_4 (`self.AddDialogue` "Blacksmith" "Great, do you have any?" (`|MakeArray` "Sure" :!type "Text")))
                  (switch `/Game/DialogueSystem/Blueprints/Enum_DialogueState` _state_4
                    (:`NewEnumerator0`
                      (if (`self.bHasBread?`)
                        (bind (_state_5 _optionindex_2) (`self.AddDialogue` "Blacksmith" "Ahh, I see you have bread, can I have it please?" (`|MakeArray` "Sure" "No" :!type "Text")))
                        (switch `/Game/DialogueSystem/Blueprints/Enum_DialogueState` _state_5
                          (:`NewEnumerator0`
                            (switch `int` _optionindex_2
                              (:`0`
                                (bind _state_6 (`self.AddDialogue` "Blacksmith" "Thank you! It's very tasty :)" (`|MakeArray` "Goodbye" :!type "Text")))
                                (switch `/Game/DialogueSystem/Blueprints/Enum_DialogueState` _state_6
                                  (:`NewEnumerator0`
                                    (`self.RemoveDialogueProgress` 1)
                                    (`self.CloseConversation`))
                                  (:`NewEnumerator1`
                                    (set `self.bHasGivenBread?` true))))
                              (:`1`
                                (bind _state_7 (`self.AddDialogue` "Blacksmith" "Ah, okay. Tell me if you change your mind please." (`|MakeArray` "Goodbye" :!type "Text")))
                                (switch `/Game/DialogueSystem/Blueprints/Enum_DialogueState` _state_7
                                  (:`NewEnumerator0`
                                    (`self.RemoveDialogueProgress` 1)
                                    (`self.CloseConversation`)))))))
                        (else
                          (bind _state_8 (`self.AddDialogue` "Blacksmith" "Seems like you don't have any bread now. Come talk to me when you do!" (`|MakeArray` "Goodbye" :!type "Text")))
                          (switch `/Game/DialogueSystem/Blueprints/Enum_DialogueState` _state_8
                            (:`NewEnumerator0`
                              (`self.RemoveDialogueProgress` 1)
                              (`self.CloseConversation`))))))))
                (:`1`
                  (bind _state_9 (`self.AddDialogue` "Blacksmith" "Ah, okay. Tell me if you change your mind please." (`|MakeArray` "Goodbye" :!type "Text")))
                  (switch `/Game/DialogueSystem/Blueprints/Enum_DialogueState` _state_9
                    (:`NewEnumerator0`
                      (`self.ClearDialogueProgress`)
                      (`self.CloseConversation`))))))))))
    (:`Night`
      (bind _state_10 (`self.AddDialogue` "Blacksmith" "Let me sleep!" (`|MakeArray` "Sorry" :!type "Text")))
      (switch `/Game/DialogueSystem/Blueprints/Enum_DialogueState` _state_10
        (:`NewEnumerator0`
          (`self.ClearDialogueProgress`)
          (`self.CloseConversation`))))))

(fn `OpenConversation`
  (bind _interactioninstigator (message `/Game/DialogueSystem/Blueprints/BPI_Interactable.GetInteractionInstigator` (`self.GetOwner`)))
  (bind _asbp_top_down_character_dialogue_tests (cast `/Game/DialogueSystem/BP_TopDownCharacterDialogueTests` _interactioninstigator))
  (bind (_timeofday_days _timeofday_hours) (`KismetMathLibrary.BreakTimespan` (`/Game/DialogueSystem/BP_TopDownCharacterDialogueTests.TimeOfDay` _asbp_top_down_character_dialogue_tests)))
  (`self.SetDialogueBranch` (select `int` (+ (`KismetMathLibrary.Conv_BoolToInt` (and (>= _timeofday_hours 5) (< _timeofday_hours 15))) (* (`KismetMathLibrary.Conv_BoolToInt` (and (>= _timeofday_hours 15) (< _timeofday_hours 22))) 2)) :`0` "Night" :`1` "Morning" :`2` "Afternoon" :`3` "Default" :!type "Name"))
  (`parent.OpenConversation`))