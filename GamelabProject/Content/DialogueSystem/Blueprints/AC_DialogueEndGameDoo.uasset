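; Dialogue component for the end-game door, where Roland remarks that this is the wrong way and he should find Preston's secret room.
; The Dialogue override calls the parent, then offers "Open door" or "Leave".
; Opening triggers DoorOpening on the BP_DoorEndGame found by class lookup.
; Both choices roll back dialogue progress and close the conversation, with player movement set to Walking at start and end.
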(fn `Dialogue`
  (`parent.Dialogue`)
  (`CharacterMovementComponent.SetMovementMode` (`Character.CharacterMovement` (`GameplayStatics.GetPlayerCharacter` 0)) "MOVE_Walking" 0)
  (bind (_state _optionindex) (`self.AddDialogue` "Roland" "(this is the wrong way, I need to go find Preston's secret room in his office)" (`|MakeArray` "Open door" "Leave" :!type "Text")))
  (switch `/Game/DialogueSystem/Blueprints/Enum_DialogueState` _state
    (:`NewEnumerator0`
      (switch `int` _optionindex
        (:`0`
          (bind _returnvalue (`GameplayStatics.GetActorOfClass` "/Game/Blueprints/01_DoorBP/BP_DoorEndGame.BP_DoorEndGame_C"))
          (`/Game/Blueprints/01_DoorBP/BP_DoorEndGame.DoorOpening` _returnvalue)
          (`self.RemoveDialogueProgress` 1)
          (`self.CloseConversation`)
          (`CharacterMovementComponent.SetMovementMode` (`Character.CharacterMovement` (`GameplayStatics.GetPlayerCharacter` 0)) "MOVE_Walking" 0))
        (:`1`
          (`self.RemoveDialogueProgress` 1)
          (`self.CloseConversation`)
          (`CharacterMovementComponent.SetMovementMode` (`Character.CharacterMovement` (`GameplayStatics.GetPlayerCharacter` 0)) "MOVE_Walking" 0))))))