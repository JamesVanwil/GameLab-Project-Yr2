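; Dialogue component for a wall-mounted Winchester pickup, presented as Roland's line with take-or-leave options.
; The Dialogue override freezes player movement, shows the prompt and branches on the chosen option.
; Taking it adds the Winchester weapon to the JRPG controller's inventory, destroys the wall actor found by class and plays a sound.
; Leaving clears dialogue progress; both choices then close the conversation and restore walking.
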(fn `Dialogue`
  (`parent.Dialogue`)
  (`CharacterMovementComponent.SetMovementMode` (`Character.CharacterMovement` (`GameplayStatics.GetPlayerCharacter` 0)) "MOVE_None" 0)
  (bind (_state _optionindex) (`self.AddDialogue` "Roland" "An old winchester from Preston's private collection, looks in good condition " (`|MakeArray` "(Take it)" "(Leave it)" :!type "Text")))
  (switch `/Game/DialogueSystem/Blueprints/Enum_DialogueState` _state
    (:`NewEnumerator0`
      (switch `int` _optionindex
        (:`0`
          (bind _asbp_jrpgplayer_controller (cast `/Game/TurnBasedJRPGTemplate/Blueprints/Controllers/BP_JRPGPlayerController` (`GameplayStatics.GetPlayerController` 0)))
          (`/Game/TurnBasedJRPGTemplate/Blueprints/Controllers/BP_JRPGPlayerController.AddEquipmentToInventory` _asbp_jrpgplayer_controller "/Game/TurnBasedJRPGTemplate/Blueprints/Items/Equipment/Weapons/BP_WinchesterWeapon.BP_WinchesterWeapon_C" 1)
          (bind _returnvalue (`GameplayStatics.GetActorOfClass` "/Game/DialogueSystem/Blueprints/NPC_Base_WinchestrWall.NPC_Base_WinchestrWall_C"))
          (`Actor.K2_DestroyActor` _returnvalue)
          (`GameplayStatics.PlaySound2D` "/Game/Audio/equipmaxingShort.equipmaxingShort" 1.0 1.0 0.0 null null))
        (:`1`
          (`self.ClearDialogueProgress`)))
      (`self.CloseConversation`)
      (`CharacterMovementComponent.SetMovementMode` (`Character.CharacterMovement` (`GameplayStatics.GetPlayerCharacter` 0)) "MOVE_Walking" 0))))