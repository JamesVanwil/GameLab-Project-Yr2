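; Dialogue component for the Champagne NPC that turns the conversation into an item pickup.
; Its Dialogue override runs the parent dialogue, then disables player movement and adds one BP_Alchohol usable item to the inventory through BP_JRPGPlayerController.
; It then destroys the first NPC_Champagne actor found in the world, closes the conversation and restores walking.
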(fn `Dialogue`
  (`parent.Dialogue`)
  (`CharacterMovementComponent.SetMovementMode` (`Character.CharacterMovement` (`GameplayStatics.GetPlayerCharacter` 0)) "MOVE_None" 0)
  (bind _asbp_jrpgplayer_controller (cast `/Game/TurnBasedJRPGTemplate/Blueprints/Controllers/BP_JRPGPlayerController` (`GameplayStatics.GetPlayerController` 0)))
  (`/Game/TurnBasedJRPGTemplate/Blueprints/Controllers/BP_JRPGPlayerController.AddUsableItemToInventory` _asbp_jrpgplayer_controller "/Game/TurnBasedJRPGTemplate/Blueprints/Items/UsableItems/BP_Alchohol.BP_Alchohol_C" 1)
  (bind _returnvalue (`GameplayStatics.GetActorOfClass` "/Game/DialogueSystem/Blueprints/NPC_Champagne.NPC_Champagne_C"))
  (`Actor.K2_DestroyActor` _returnvalue)
  (`self.CloseConversation`)
  (`CharacterMovementComponent.SetMovementMode` (`Character.CharacterMovement` (`GameplayStatics.GetPlayerCharacter` 0)) "MOVE_Walking" 0))