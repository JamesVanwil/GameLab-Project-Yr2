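; Dialogue component for a window interaction, in which Roland remarks on the steady snowfall blocking the view.
; The Dialogue override calls its parent, disables player character movement and adds the line with a single Leave option.
; On the Pass Through state it calls RemoveDialogueProgress, closes the conversation and restores walking movement.
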(fn `Dialogue`
  (`parent.Dialogue`)
  (`CharacterMovementComponent.SetMovementMode` (`Character.CharacterMovement` (`GameplayStatics.GetPlayerCharacter` 0)) "MOVE_None" 0)
  (bind _state (`self.AddDialogue` "Roland" "It is continuing to snow steadily,  \nI can't see anything" (`|MakeArray` "Leave" :!type "Text")))
  (switch `/Game/DialogueSystem/Blueprints/Enum_DialogueState` _state
    (:`NewEnumerator0`
      (`self.RemoveDialogueProgress` 1)
      (`self.CloseConversation`)
      (`CharacterMovementComponent.SetMovementMode` (`Character.CharacterMovement` (`GameplayStatics.GetPlayerCharacter` 0)) "MOVE_Walking" 0))))