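; Enemy Jab battle skill for the turn-based JRPG, which plays an attack animation and damages the current target.
; Each skill notify deals multiplied damage through BattleController if the target is alive, applying buffs when DealDamage returns true; a graph note labels this "Attack twice".
; The skill completes when the animation ends.
; Move-to-target and move-back branches are present but disconnected, so the skill triggers no movement.
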(event `/Game/TurnBasedJRPGTemplate/Blueprints/Skills/BP_SkillBase.UseSkill`
  ;[1 1 1] Move to target
  (`self.PlaySkillAnimation` :!label _label))

(event `OnUnitMovedToTargetHandler`
  ;[1 1 1] Move to target
  (goto _label))

(event `self.UseSkillOnNotify`
  (bind _battlecontroller (`self.battleController`))
  ;[1 1 1] Attack twice
  (bind _isunitdead (`/Game/TurnBasedJRPGTemplate/Blueprints/Units/BP_UnitBase.IsUnitDead` (`/Game/TurnBasedJRPGTemplate/Blueprints/Battle/BP_BattleController.currentTargetUnit` _battlecontroller)))
  (if (not _isunitdead)
    (bind _ishit (`/Game/TurnBasedJRPGTemplate/Blueprints/Battle/BP_BattleController.DealDamage` _battlecontroller 0 1.5))
    (if _ishit
      (`self.ApplyBuffs` (`|MakeArray` (`/Game/TurnBasedJRPGTemplate/Blueprints/Battle/BP_BattleController.currentTargetUnit` (`self.battleController`)))))))

(event `self.OnSkillAnimationEnded`
  ;[1 1 1] Attack twice
  (`self.OnSkillUsed` :!label _label_2))

(event `OnUnitMovedBackHandler`
  ;[1 1 1] Attack twice
  (goto _label_2))

(fn `UserConstructionScript`
  (`parent.UserConstructionScript`))