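; Revolver buff Blueprint for the turn-based JRPG template, with events for applying and ending the buff.
; Both events are empty, so the buff currently has no effect of its own.
; Disconnected nodes print a message and raise or lower attack range and action time, using BP_MagePlayerUnit class defaults rather than a unit instance.
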(event `self.ApplyBuff`
  ;[1 1 1] Appply Revolver Buff
)

(event `self.OnBuffEnded`
  ;[1 1 1] End Revolver Buff
)

(fn `UserConstructionScript`
  (`parent.UserConstructionScript`))