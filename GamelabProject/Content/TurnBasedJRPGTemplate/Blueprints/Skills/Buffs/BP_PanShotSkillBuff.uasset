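; BP_PanShotSkillBuff is a skill buff for the turn-based JRPG template that changes the target unit's ActionTime stat while active.
; ApplyBuff adds a fixed amount to ActionTime in the target's FirstLevelStats struct, and OnBuffEnded subtracts the same amount.
; The change is a relative offset, with no cached original value to restore.
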(event `self.ApplyBuff`
  (bind _firstlevelstats (`/Game/TurnBasedJRPGTemplate/Blueprints/Units/BP_UnitBase.firstLevelStats` (`self.targetUnit`)))
  (setmembers `/Game/TurnBasedJRPGTemplate/Blueprints/Structs/S_UnitStats` :`StructRef` _firstlevelstats :`actionTime` (+ (`.actionTime_31_CD6B6FA04FF3CB1C1BA72A93110B7A28` (break `/Game/TurnBasedJRPGTemplate/Blueprints/Structs/S_UnitStats` _firstlevelstats)) 0.3)))

(event `self.OnBuffEnded`
  (bind _firstlevelstats (`/Game/TurnBasedJRPGTemplate/Blueprints/Units/BP_UnitBase.firstLevelStats` (`self.targetUnit`)))
  (setmembers `/Game/TurnBasedJRPGTemplate/Blueprints/Structs/S_UnitStats` :`StructRef` _firstlevelstats :`actionTime` (- (`.actionTime_31_CD6B6FA04FF3CB1C1BA72A93110B7A28` (break `/Game/TurnBasedJRPGTemplate/Blueprints/Structs/S_UnitStats` _firstlevelstats)) 0.3)))

(fn `UserConstructionScript`
  (`parent.UserConstructionScript`))