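; BP_BuffDamage is a skill buff for the turn-based JRPG template, meant to temporarily raise a unit's maximum attack.
; ApplyBuff adds a fixed bonus to MaxAttack, and OnBuffEnded subtracts the same amount, each printing a debug message.
; Both events are hardcoded to the unit stats struct read from BP_MagePlayerUnit's class defaults, with no reference to a unit instance.
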(event `self.ApplyBuff`
  (bind _firstlevelstats (defaults `/Game/TurnBasedJRPGTemplate/Blueprints/Units/PlayerUnits/BP_MagePlayerUnit` "/Game/TurnBasedJRPGTemplate/Blueprints/Units/PlayerUnits/BP_MagePlayerUnit.BP_MagePlayerUnit_C"))
  (`KismetSystemLibrary.PrintString` "Buff applied")
  (setmembers `/Game/TurnBasedJRPGTemplate/Blueprints/Structs/S_UnitStats` :`StructRef` _firstlevelstats :`maxAttack` (+ (`.maxAttack_15_24D8527844E2DFB657716C9F16A4AE21` (break `/Game/TurnBasedJRPGTemplate/Blueprints/Structs/S_UnitStats` _firstlevelstats)) 100)))

(event `self.OnBuffEnded`
  (bind _firstlevelstats (defaults `/Game/TurnBasedJRPGTemplate/Blueprints/Units/PlayerUnits/BP_MagePlayerUnit` "/Game/TurnBasedJRPGTemplate/Blueprints/Units/PlayerUnits/BP_MagePlayerUnit.BP_MagePlayerUnit_C"))
  (`KismetSystemLibrary.PrintString` "Buff Ended")
  (setmembers `/Game/TurnBasedJRPGTemplate/Blueprints/Structs/S_UnitStats` :`StructRef` _firstlevelstats :`maxAttack` (- (`.maxAttack_15_24D8527844E2DFB657716C9F16A4AE21` (break `/Game/TurnBasedJRPGTemplate/Blueprints/Structs/S_UnitStats` _firstlevelstats)) 100)))

(fn `UserConstructionScript`
  (`parent.UserConstructionScript`))