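; High Understanding buff for the turn-based JRPG template, meant to raise the targeted unit's Speed by a fixed amount until it ends.
; ApplyBuff sets an applied flag and gets the current target from BP_BattleController.
; OnBuffEnded clears the flag and subtracts the same amount.
; Both events edit the stats struct read from the target's class defaults, not the unit instance's stats.
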(event `self.ApplyBuff`
  (`KismetSystemLibrary.PrintString` "High buff applied")
  (set `self.HasHighUnderstandingBuffBeenApplied?` true)
  (bind _returnvalue (`GameplayStatics.GetActorOfClass` "/Game/TurnBasedJRPGTemplate/Blueprints/Battle/BP_BattleController.BP_BattleController_C"))
  (bind _output_get (set `self.Current Target Unit` (`/Game/TurnBasedJRPGTemplate/Blueprints/Battle/BP_BattleController.currentTargetUnit` _returnvalue)))
  (bind _firstlevelstats (defaults `Object` (`GameplayStatics.GetObjectClass` _output_get)))
  (setmembers `/Game/TurnBasedJRPGTemplate/Blueprints/Structs/S_UnitStats` :`StructRef` _firstlevelstats :`speed` (+ (`.speed_17_747DDA004CC2DC11462387A6F382E254` (break `/Game/TurnBasedJRPGTemplate/Blueprints/Structs/S_UnitStats` _firstlevelstats)) 15)))

(event `self.OnBuffEnded`
  (bind _firstlevelstats (defaults `Object` (`GameplayStatics.GetObjectClass` (`self.Current Target Unit`))))
  (set `self.HasHighUnderstandingBuffBeenApplied?` false)
  (setmembers `/Game/TurnBasedJRPGTemplate/Blueprints/Structs/S_UnitStats` :`StructRef` _firstlevelstats :`speed` (- (`.speed_17_747DDA004CC2DC11462387A6F382E254` (break `/Game/TurnBasedJRPGTemplate/Blueprints/Structs/S_UnitStats` _firstlevelstats)) 15)))

(fn `UserConstructionScript`
  (`parent.UserConstructionScript`))