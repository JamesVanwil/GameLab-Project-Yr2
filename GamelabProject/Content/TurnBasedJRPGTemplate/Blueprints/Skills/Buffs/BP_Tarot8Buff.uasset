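; BP_Tarot8Buff is a JRPG buff that trades physical attack for magic on player units wearing a Tarot 8 item.
; ApplyBuff scans the controller's PlayerUnits for that tarot in helm, boots or two sockets, then lowers min/max attack and raises max magical attack.
; OnBuffEnded repeats the scan and reverses the offsets.
; Stat edits target unit class defaults, and both events toggle a flag named IsTarot3SwordsActive, despite the Tarot 8 theme.
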(event `self.ApplyBuff`
  (set `self.IsTarot3SwordsActive?` true)
  (bind _asbp_jrpgplayer_controller (cast `/Game/TurnBasedJRPGTemplate/Blueprints/Controllers/BP_JRPGPlayerController` (`GameplayStatics.GetPlayerController` 0)))
  (bind _playerunits (`/Game/TurnBasedJRPGTemplate/Blueprints/Controllers/BP_JRPGPlayerController.playerUnits` _asbp_jrpgplayer_controller))
  (bind _keys (`BlueprintMapLibrary.Map_Keys` _playerunits))
  (for _array_element _keys
    (bind ((`HelmTarot1_31_751FB906466EBEC2597E348A40B77276` _helmtarot1) (`BootsTarot2_34_494ABC0E4604C5FA6716CDB909310B09` _bootstarot2) (`TarotSocket3_45_BED5D59A4998303E41DEC9B4897C5719` _tarotsocket3) (`TarotSocket4_46_D6A172B14760122AE2FE539D76A47580` _tarotsocket4)) (break `/Game/TurnBasedJRPGTemplate/Blueprints/Structs/S_PlayerUnitData` (`BlueprintMapLibrary.Map_Find` _playerunits _array_element)))
    (if (or (== _helmtarot1 "/Game/TurnBasedJRPGTemplate/Blueprints/Items/Equipment/Tarot_8/BP_Tarot8Helm.BP_Tarot8Helm_C") (== _bootstarot2 "/Game/TurnBasedJRPGTemplate/Blueprints/Items/Equipment/Tarot_8/BP_Tarot8Boots.BP_Tarot8Boots_C") (== _tarotsocket3 "/Game/TurnBasedJRPGTemplate/Blueprints/Items/Equipment/Tarot_8/BP_Tarot8-3.BP_Tarot8-3_C") (== _tarotsocket4 "/Game/TurnBasedJRPGTemplate/Blueprints/Items/Equipment/Tarot_8/BP_Tarot8-4.BP_Tarot8-4_C"))
      (`KismetSystemLibrary.PrintString` "Buff applied")
      (bind _firstlevelstats (defaults `Object` _array_element))
      (bind ((`minAttack_14_0D64A0224152A597434ECDAF6DFC9964` _minattack) (`maxAttack_15_24D8527844E2DFB657716C9F16A4AE21` _maxattack) (`maxMagicalAttack_24_C0C7731143A09315B418E7876A1F2F19` _maxmagicalattack)) (break `/Game/TurnBasedJRPGTemplate/Blueprints/Structs/S_UnitStats` _firstlevelstats))
      (setmembers `/Game/TurnBasedJRPGTemplate/Blueprints/Structs/S_UnitStats` :`StructRef` _firstlevelstats :`minAttack` (- _minattack 10) :`maxAttack` (- _maxattack 10) :`maxMagicalAttack` (+ _maxmagicalattack 20)))))

(event `self.OnBuffEnded`
  (set `self.IsTarot3SwordsActive?` false)
  (`KismetSystemLibrary.PrintString` "Buff Ended")
  (bind _asbp_jrpgplayer_controller (cast `/Game/TurnBasedJRPGTemplate/Blueprints/Controllers/BP_JRPGPlayerController` (`GameplayStatics.GetPlayerController` 0)))
  (bind _playerunits (`/Game/TurnBasedJRPGTemplate/Blueprints/Controllers/BP_JRPGPlayerController.playerUnits` _asbp_jrpgplayer_controller))
  (bind _keys (`BlueprintMapLibrary.Map_Keys` _playerunits))
  (for _array_element _keys
    (bind ((`HelmTarot1_31_751FB906466EBEC2597E348A40B77276` _helmtarot1) (`BootsTarot2_34_494ABC0E4604C5FA6716CDB909310B09` _bootstarot2) (`TarotSocket3_45_BED5D59A4998303E41DEC9B4897C5719` _tarotsocket3) (`TarotSocket4_46_D6A172B14760122AE2FE539D76A47580` _tarotsocket4)) (break `/Game/TurnBasedJRPGTemplate/Blueprints/Structs/S_PlayerUnitData` (`BlueprintMapLibrary.Map_Find` _playerunits _array_element)))
    (if (or (== _helmtarot1 "/Game/TurnBasedJRPGTemplate/Blueprints/Items/Equipment/Tarot_8/BP_Tarot8Helm.BP_Tarot8Helm_C") (== _bootstarot2 "/Game/TurnBasedJRPGTemplate/Blueprints/Items/Equipment/Tarot_8/BP_Tarot8Boots.BP_Tarot8Boots_C") (== _tarotsocket3 "/Game/TurnBasedJRPGTemplate/Blueprints/Items/Equipment/Tarot_8/BP_Tarot8-3.BP_Tarot8-3_C") (== _tarotsocket4 "/Game/TurnBasedJRPGTemplate/Blueprints/Items/Equipment/Tarot_8/BP_Tarot8-4.BP_Tarot8-4_C"))
      (bind _firstlevelstats (defaults `Object` _array_element))
      (bind ((`minAttack_14_0D64A0224152A597434ECDAF6DFC9964` _minattack) (`maxAttack_15_24D8527844E2DFB657716C9F16A4AE21` _maxattack) (`maxMagicalAttack_24_C0C7731143A09315B418E7876A1F2F19` _maxmagicalattack)) (break `/Game/TurnBasedJRPGTemplate/Blueprints/Structs/S_UnitStats` _firstlevelstats))
      (setmembers `/Game/TurnBasedJRPGTemplate/Blueprints/Structs/S_UnitStats` :`StructRef` _firstlevelstats :`minAttack` (+ _minattack 10) :`maxAttack` (+ _maxattack 10) :`maxMagicalAttack` (- _maxmagicalattack 20)))))

(fn `UserConstructionScript`
  (`parent.UserConstructionScript`))