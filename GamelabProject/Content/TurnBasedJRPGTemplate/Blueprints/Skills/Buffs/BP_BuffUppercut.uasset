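; Buff for the Uppercut skill in the turn-based JRPG template that temporarily changes the target unit's ActionTime.
; ApplyBuff stores the current ActionTime in a variable and raises the unit's value by a fixed one unit.
; OnBuffEnded subtracts the same amount from the current value instead of restoring the stored one, leaving other changes to ActionTime intact.
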(event `self.ApplyBuff`
  (bind _targetunit (`self.targetUnit`))
  (bind _output_get (set `self.Action Time Defaukt` (`/Game/TurnBasedJRPGTemplate/Blueprints/Units/BP_UnitBase.ActionTime` _targetunit)))
  (set `/Game/TurnBasedJRPGTemplate/Blueprints/Units/BP_UnitBase.ActionTime` (+ _output_get 1.0) _targetunit))

(event `self.OnBuffEnded`
  (bind _targetunit (`self.targetUnit`))
  (set `/Game/TurnBasedJRPGTemplate/Blueprints/Units/BP_UnitBase.ActionTime` (- (`/Game/TurnBasedJRPGTemplate/Blueprints/Units/BP_UnitBase.ActionTime` _targetunit) 1.0) _targetunit))

(fn `UserConstructionScript`
  (`parent.UserConstructionScript`))