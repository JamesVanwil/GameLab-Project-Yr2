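; BP_BuffTest is a test buff for the JRPG template, aimed at the mage player unit's MaxAttack.
; ApplyBuff and OnBuffEnded print messages and set MaxAttack 100 above or below the class default, writing to the struct from GetClassDefaults rather than a unit instance.
; Tick looks up the mage in the player controller's PlayerUnits and calls OnBuffEnded once through DoOnce when CurrentHP drops below 125.
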(event `self.ApplyBuff`
  (bind _firstlevelstats (defaults `/Game/TurnBasedJRPGTemplate/Blueprints/Units/PlayerUnits/BP_MagePlayerUnit` "/Game/TurnBasedJRPGTemplate/Blueprints/Units/PlayerUnits/BP_MagePlayerUnit.BP_MagePlayerUnit_C"))
  (`KismetSystemLibrary.PrintString` "Buff apllied")
  (setmembers `/Game/TurnBasedJRPGTemplate/Blueprints/Structs/S_UnitStats` :`StructRef` _firstlevelstats :`maxAttack` (+ (`.maxAttack_15_24D8527844E2DFB657716C9F16A4AE21` (break `/Game/TurnBasedJRPGTemplate/Blueprints/Structs/S_UnitStats` _firstlevelstats)) 100)))

(event `self.OnBuffEnded`
  (bind _firstlevelstats (defaults `/Game/TurnBasedJRPGTemplate/Blueprints/Units/PlayerUnits/BP_MagePlayerUnit` "/Game/TurnBasedJRPGTemplate/Blueprints/Units/PlayerUnits/BP_MagePlayerUnit.BP_MagePlayerUnit_C"))
  (`KismetSystemLibrary.PrintString` "Buff Ended")
  (setmembers `/Game/TurnBasedJRPGTemplate/Blueprints/Structs/S_UnitStats` :`StructRef` _firstlevelstats :`maxAttack` (- (`.maxAttack_15_24D8527844E2DFB657716C9F16A4AE21` (break `/Game/TurnBasedJRPGTemplate/Blueprints/Structs/S_UnitStats` _firstlevelstats)) 100)))

(event `self.ReceiveTick`
  (params (DeltaSeconds :type "Float (single-precision)"))
  (bind _asbp_jrpgplayer_controller (cast `/Game/TurnBasedJRPGTemplate/Blueprints/Controllers/BP_JRPGPlayerController` (`GameplayStatics.GetPlayerController` 0)))
  (if (< (`.currentHP_4_0B53A15447C685E66E26429EA6694AA4` (break `/Game/TurnBasedJRPGTemplate/Blueprints/Structs/S_PlayerUnitData` (`BlueprintMapLibrary.Map_Find` (`/Game/TurnBasedJRPGTemplate/Blueprints/Controllers/BP_JRPGPlayerController.playerUnits` _asbp_jrpgplayer_controller) "/Game/TurnBasedJRPGTemplate/Blueprints/Units/PlayerUnits/BP_MagePlayerUnit.BP_MagePlayerUnit_C"))) 125)
    (`/Engine/EditorBlueprintResources/StandardMacros.DoOnce` false
      (:`Completed`
        (`self.OnBuffEnded`)))))

(fn `UserConstructionScript`
  (`parent.UserConstructionScript`))