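; BP_BuffEnemyAttack is a skill buff for the turn-based JRPG battle system that drains target MP and strengthens the attacker.
; ApplyBuff subtracts a fixed amount of MP from the BattleController's current target, without clamping, and spawns BP_DamageText above it flagged as MP damage.
; It then adds a fixed bonus to the attacking unit's Defense; despite the asset name, no Attack stat changes.
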(event `self.ApplyBuff`
  (bind _currenttargetunit (`/Game/TurnBasedJRPGTemplate/Blueprints/Battle/BP_BattleController.currentTargetUnit` (`self.battleController`)))
  (bind _currentattackingunit (`/Game/TurnBasedJRPGTemplate/Blueprints/Battle/BP_BattleController.currentAttackingUnit` (`self.battleController`)))
  (bind (_returnvalue_x _returnvalue_y _returnvalue_z) (`KismetMathLibrary.BreakVector` (`self.K2_GetActorLocation` _currenttargetunit)))
  (set `/Game/TurnBasedJRPGTemplate/Blueprints/Units/BP_UnitBase.currentMP` (- (`/Game/TurnBasedJRPGTemplate/Blueprints/Units/BP_UnitBase.currentMP` _currenttargetunit) 3) _currenttargetunit)
  (`|SpawnActorFromClass` "/Game/TurnBasedJRPGTemplate/Blueprints/Battle/BP_DamageText.BP_DamageText_C" (`KismetMathLibrary.MakeTransform` (`KismetMathLibrary.MakeVector` _returnvalue_x _returnvalue_y (+ _returnvalue_z 250.0))) "Undefined" "MultiplyWithRoot" null 3 null false false true null)
  (set `/Game/TurnBasedJRPGTemplate/Blueprints/Units/BP_UnitBase.defense` (+ (`/Game/TurnBasedJRPGTemplate/Blueprints/Units/BP_UnitBase.defense` _currentattackingunit) 3) _currentattackingunit))

(fn `UserConstructionScript`
  (`parent.UserConstructionScript`))