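; Turn-based battle buff "Behind Me" that flags the attacking enemy unit and is meant to raise attack.
; ApplyBuff and OnBuffEnded add and subtract a fixed min/max attack bonus on the stats struct read from BP_WeakEnemy class defaults, not the unit instance.
; Both also toggle IsBehindMeBuffActive on BP_BattleController's CurrentAttackingUnit, cast to BP_EnemyUnitBase, and print debug messages.
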(event `self.ApplyBuff`
  (bind _firstlevelstats (defaults `/Game/TurnBasedJRPGTemplate/Blueprints/Units/EnemyUnits/BP_WeakEnemy` "/Game/TurnBasedJRPGTemplate/Blueprints/Units/EnemyUnits/BP_WeakEnemy.BP_WeakEnemy_C"))
  (bind ((`minAttack_14_0D64A0224152A597434ECDAF6DFC9964` _minattack) (`maxAttack_15_24D8527844E2DFB657716C9F16A4AE21` _maxattack)) (break `/Game/TurnBasedJRPGTemplate/Blueprints/Structs/S_UnitStats` _firstlevelstats))
  (`KismetSystemLibrary.PrintString` "BUff applied")
  (setmembers `/Game/TurnBasedJRPGTemplate/Blueprints/Structs/S_UnitStats` :`StructRef` _firstlevelstats :`minAttack` (+ _minattack 5) :`maxAttack` (+ _maxattack 5))
  (bind _returnvalue (`GameplayStatics.GetActorOfClass` "/Game/TurnBasedJRPGTemplate/Blueprints/Battle/BP_BattleController.BP_BattleController_C"))
  (bind _asbp_enemy_unit_base (cast `/Game/TurnBasedJRPGTemplate/Blueprints/Units/EnemyUnits/BP_EnemyUnitBase` (`/Game/TurnBasedJRPGTemplate/Blueprints/Battle/BP_BattleController.currentAttackingUnit` _returnvalue)))
  (set `/Game/TurnBasedJRPGTemplate/Blueprints/Units/EnemyUnits/BP_EnemyUnitBase.IsBehindMeBuffActive` true _asbp_enemy_unit_base))

(event `self.OnBuffEnded`
  (bind _firstlevelstats (defaults `/Game/TurnBasedJRPGTemplate/Blueprints/Units/EnemyUnits/BP_WeakEnemy` "/Game/TurnBasedJRPGTemplate/Blueprints/Units/EnemyUnits/BP_WeakEnemy.BP_WeakEnemy_C"))
  (bind ((`minAttack_14_0D64A0224152A597434ECDAF6DFC9964` _minattack) (`maxAttack_15_24D8527844E2DFB657716C9F16A4AE21` _maxattack)) (break `/Game/TurnBasedJRPGTemplate/Blueprints/Structs/S_UnitStats` _firstlevelstats))
  (`KismetSystemLibrary.PrintString` "buff ended")
  (setmembers `/Game/TurnBasedJRPGTemplate/Blueprints/Structs/S_UnitStats` :`StructRef` _firstlevelstats :`minAttack` (- _minattack 5) :`maxAttack` (- _maxattack 5))
  (bind _returnvalue (`GameplayStatics.GetActorOfClass` "/Game/TurnBasedJRPGTemplate/Blueprints/Battle/BP_BattleController.BP_BattleController_C"))
  (bind _asbp_enemy_unit_base (cast `/Game/TurnBasedJRPGTemplate/Blueprints/Units/EnemyUnits/BP_EnemyUnitBase` (`/Game/TurnBasedJRPGTemplate/Blueprints/Battle/BP_BattleController.currentAttackingUnit` _returnvalue)))
  (set `/Game/TurnBasedJRPGTemplate/Blueprints/Units/EnemyUnits/BP_EnemyUnitBase.IsBehindMeBuffActive` false _asbp_enemy_unit_base))

(fn `UserConstructionScript`
  (`parent.UserConstructionScript`))