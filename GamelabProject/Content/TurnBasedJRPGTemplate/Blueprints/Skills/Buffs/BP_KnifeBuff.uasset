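; Knife buff for the turn-based JRPG battle system that raises a unit's attack range and shortens its action time.
; ApplyBuff takes the current target unit from BP_BattleController and stores it for later.
; OnBuffEnded reverses the same fixed offsets on that stored unit.
; Both events read and set the stat struct through the unit's class defaults, not through stats on the unit instance.
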(event `self.ApplyBuff`
  (bind _returnvalue (`GameplayStatics.GetActorOfClass` "/Game/TurnBasedJRPGTemplate/Blueprints/Battle/BP_BattleController.BP_BattleController_C"))
  (bind _output_get (set `self.Current Target Unit` (`/Game/TurnBasedJRPGTemplate/Blueprints/Battle/BP_BattleController.currentTargetUnit` _returnvalue)))
  (bind _firstlevelstats (defaults `Object` (`GameplayStatics.GetObjectClass` _output_get)))
  (bind ((`minAttack_14_0D64A0224152A597434ECDAF6DFC9964` _minattack) (`maxAttack_15_24D8527844E2DFB657716C9F16A4AE21` _maxattack) (`actionTime_31_CD6B6FA04FF3CB1C1BA72A93110B7A28` _actiontime)) (break `/Game/TurnBasedJRPGTemplate/Blueprints/Structs/S_UnitStats` _firstlevelstats))
  (setmembers `/Game/TurnBasedJRPGTemplate/Blueprints/Structs/S_UnitStats` :`StructRef` _firstlevelstats :`minAttack` (+ _minattack 5) :`maxAttack` (+ _maxattack 5) :`actionTime` (- _actiontime 0.2)))

(event `self.OnBuffEnded`
  (bind _firstlevelstats (defaults `Object` (`GameplayStatics.GetObjectClass` (`self.Current Target Unit`))))
  (bind ((`minAttack_14_0D64A0224152A597434ECDAF6DFC9964` _minattack) (`maxAttack_15_24D8527844E2DFB657716C9F16A4AE21` _maxattack) (`actionTime_31_CD6B6FA04FF3CB1C1BA72A93110B7A28` _actiontime)) (break `/Game/TurnBasedJRPGTemplate/Blueprints/Structs/S_UnitStats` _firstlevelstats))
  (setmembers `/Game/TurnBasedJRPGTemplate/Blueprints/Structs/S_UnitStats` :`StructRef` _firstlevelstats :`minAttack` (- _minattack 5) :`maxAttack` (- _maxattack 5) :`actionTime` (+ _actiontime 0.2)))

(fn `UserConstructionScript`
  (`parent.UserConstructionScript`))