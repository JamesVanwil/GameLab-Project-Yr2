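; Damage buff for the turn-based JRPG template, granted through Add Damage tarot items on player units.
; ApplyBuff scans the player controller's PlayerUnits for a matching tarot in any of four sockets, then raises MaxAttack and ActionTime by fixed amounts.
; OnBuffEnded repeats the scan and subtracts the same amounts.
; Both events target stat structs obtained through GetClassDefaults on each unit class key, not spawned unit instances.
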(event `self.ApplyBuff`
  (bind _asbp_jrpgplayer_controller (cast `/Game/TurnBasedJRPGTemplate/Blueprints/Controllers/BP_JRPGPlayerController` (`GameplayStatics.GetPlayerController` 0)))
  (bind _playerunits (`/Game/TurnBasedJRPGTemplate/Blueprints/Controllers/BP_JRPGPlayerController.playerUnits` _asbp_jrpgplayer_controller))
  (bind _keys (`BlueprintMapLibrary.Map_Keys` _playerunits))
  (for _array_element _keys
    (bind ((`HelmTarot1_31_751FB906466EBEC2597E348A40B77276` _helmtarot1) (`BootsTarot2_34_494ABC0E4604C5FA6716CDB909310B09` _bootstarot2) (`TarotSocket3_45_BED5D59A4998303E41DEC9B4897C5719` _tarotsocket3) (`TarotSocket4_46_D6A172B14760122AE2FE539D76A47580` _tarotsocket4)) (break `/Game/TurnBasedJRPGTemplate/Blueprints/Structs/S_PlayerUnitData` (`BlueprintMapLibrary.Map_Find` _playerunits _array_element)))
    (if (or (== _helmtarot1 "/Game/TurnBasedJRPGTemplate/Blueprints/Items/Equipment/Helms/BP_AddDamageTarot.BP_AddDamageTarot_C") (== _bootstarot2 "/Game/TurnBasedJRPGTemplate/Blueprints/Items/Equipment/Helms/BP_AddDamageTarotBoots.BP_AddDamageTarotBoots_C") (== _tarotsocket3 "/Game/TurnBasedJRPGTemplate/Blueprints/Items/Equipment/Helms/BP_AddDamageTarot3.BP_AddDamageTarot3_C") (== _tarotsocket4 "/Game/TurnBasedJRPGTemplate/Blueprints/Items/Equipment/Helms/BP_AddDamageTarot4.BP_AddDamageTarot4_C"))
      (`KismetSystemLibrary.PrintString` "Buff applied")
      (bind _firstlevelstats (defaults `Object` _array_element))
      (bind ((`maxAttack_15_24D8527844E2DFB657716C9F16A4AE21` _maxattack) (`actionTime_31_CD6B6FA04FF3CB1C1BA72A93110B7A28` _actiontime)) (break `/Game/TurnBasedJRPGTemplate/Blueprints/Structs/S_UnitStats` _firstlevelstats))
      (setmembers `/Game/TurnBasedJRPGTemplate/Blueprints/Structs/S_UnitStats` :`StructRef` _firstlevelstats :`maxAttack` (+ _maxattack 20) :`actionTime` (+ _actiontime 0.3)))))

(event `self.OnBuffEnded`
  (`KismetSystemLibrary.PrintString` "Buff Ended")
  (bind _asbp_jrpgplayer_controller (cast `/Game/TurnBasedJRPGTemplate/Blueprints/Controllers/BP_JRPGPlayerController` (`GameplayStatics.GetPlayerController` 0)))
  (bind _playerunits (`/Game/TurnBasedJRPGTemplate/Blueprints/Controllers/BP_JRPGPlayerController.playerUnits` _asbp_jrpgplayer_controller))
  (bind _keys (`BlueprintMapLibrary.Map_Keys` _playerunits))
  (for _array_element _keys
    (bind ((`HelmTarot1_31_751FB906466EBEC2597E348A40B77276` _helmtarot1) (`BootsTarot2_34_494ABC0E4604C5FA6716CDB909310B09` _bootstarot2) (`TarotSocket3_45_BED5D59A4998303E41DEC9B4897C5719` _tarotsocket3) (`TarotSocket4_46_D6A172B14760122AE2FE539D76A47580` _tarotsocket4)) (break `/Game/TurnBasedJRPGTemplate/Blueprints/Structs/S_PlayerUnitData` (`BlueprintMapLibrary.Map_Find` _playerunits _array_element)))
    (if (or (== _helmtarot1 "/Game/TurnBasedJRPGTemplate/Blueprints/Items/Equipment/Helms/BP_AddDamageTarot.BP_AddDamageTarot_C") (== _bootstarot2 "/Game/TurnBasedJRPGTemplate/Blueprints/Items/Equipment/Helms/BP_AddDamageTarotBoots.BP_AddDamageTarotBoots_C") (== _tarotsocket3 "/Game/TurnBasedJRPGTemplate/Blueprints/Items/Equipment/Helms/BP_AddDamageTarot3.BP_AddDamageTarot3_C") (== _tarotsocket4 "/Game/TurnBasedJRPGTemplate/Blueprints/Items/Equipment/Helms/BP_AddDamageTarot4.BP_AddDamageTarot4_C"))
      (bind _firstlevelstats (defaults `Object` _array_element))
      (bind ((`maxAttack_15_24D8527844E2DFB657716C9F16A4AE21` _maxattack) (`actionTime_31_CD6B6FA04FF3CB1C1BA72A93110B7A28` _actiontime)) (break `/Game/TurnBasedJRPGTemplate/Blueprints/Structs/S_UnitStats` _firstlevelstats))
      (setmembers `/Game/TurnBasedJRPGTemplate/Blueprints/Structs/S_UnitStats` :`StructRef` _firstlevelstats :`maxAttack` (- _maxattack 20) :`actionTime` (- _actiontime 0.3)))))

(fn `UserConstructionScript`
  (`parent.UserConstructionScript`))