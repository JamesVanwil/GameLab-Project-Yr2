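; BP_BuffPlacidaTarot1 is a skill buff that raises the target unit's MaxAttack by one while active.
; ApplyBuff caches the current MaxAttack in MaxAttackDefault, then adds the bonus.
; OnBuffEnded writes the cached value back rather than subtracting the bonus, so other MaxAttack changes made during the buff are overwritten.
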(event `self.ApplyBuff`
  (bind _targetunit (`self.targetUnit`))
  (bind _maxattack (`/Game/TurnBasedJRPGTemplate/Blueprints/Units/BP_UnitBase.maxAttack` _targetunit))
  (set `self.Max Attack Default` _maxattack)
  (set `/Game/TurnBasedJRPGTemplate/Blueprints/Units/BP_UnitBase.maxAttack` (+ _maxattack 1) _targetunit))

(event `self.OnBuffEnded`
  (set `/Game/TurnBasedJRPGTemplate/Blueprints/Units/BP_UnitBase.maxAttack` (`self.Max Attack Default`) (`self.targetUnit`)))

(fn `UserConstructionScript`
  (`parent.UserConstructionScript`))