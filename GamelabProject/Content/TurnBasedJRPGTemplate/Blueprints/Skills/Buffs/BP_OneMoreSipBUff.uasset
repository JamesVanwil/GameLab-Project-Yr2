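; "One More Sip" buff for the mage in the turn-based JRPG, trading Defense for higher attack.
; ApplyBuff sets a flag and edits stat values read from the BP_MagePlayerUnit class defaults rather than a unit instance.
; If the player controller holds Alchohol, it consumes one and adds MP to the mage's looked-up unit data.
; OnBuffEnded clears the flag and applies the opposite stat offsets.
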(event `self.ApplyBuff`
  (bind _firstlevelstats (defaults `/Game/TurnBasedJRPGTemplate/Blueprints/Units/PlayerUnits/BP_MagePlayerUnit` "/Game/TurnBasedJRPGTemplate/Blueprints/Units/PlayerUnits/BP_MagePlayerUnit.BP_MagePlayerUnit_C"))
  (bind ((`minAttack_14_0D64A0224152A597434ECDAF6DFC9964` _minattack) (`maxAttack_15_24D8527844E2DFB657716C9F16A4AE21` _maxattack) (`defense_16_FEA01B2E4A985F64F6B9359A13E3F651` _defense)) (break `/Game/TurnBasedJRPGTemplate/Blueprints/Structs/S_UnitStats` _firstlevelstats))
  (set `self.IsOneMoreSpiffBuffApplied?` true)
  (setmembers `/Game/TurnBasedJRPGTemplate/Blueprints/Structs/S_UnitStats` :`StructRef` _firstlevelstats :`minAttack` (+ _minattack 15) :`maxAttack` (+ _maxattack 15) :`defense` (- _defense 10))
  (bind _asbp_jrpgplayer_controller (cast `/Game/TurnBasedJRPGTemplate/Blueprints/Controllers/BP_JRPGPlayerController` (`GameplayStatics.GetPlayerController` 0)))
  (if (>= (`BlueprintMapLibrary.Map_Find` (`/Game/TurnBasedJRPGTemplate/Blueprints/Controllers/BP_JRPGPlayerController.usableItems` _asbp_jrpgplayer_controller) "/Game/TurnBasedJRPGTemplate/Blueprints/Items/UsableItems/BP_Alchohol.BP_Alchohol_C") 1)
    (`/Game/TurnBasedJRPGTemplate/Blueprints/Controllers/BP_JRPGPlayerController.RemoveItemFromInventory` _asbp_jrpgplayer_controller "/Game/TurnBasedJRPGTemplate/Blueprints/Items/UsableItems/BP_Alchohol.BP_Alchohol_C" 1)
    (bind _value (`BlueprintMapLibrary.Map_Find` (`/Game/TurnBasedJRPGTemplate/Blueprints/Controllers/BP_JRPGPlayerController.playerUnits` _asbp_jrpgplayer_controller) "/Game/TurnBasedJRPGTemplate/Blueprints/Units/PlayerUnits/BP_MagePlayerUnit.BP_MagePlayerUnit_C"))
    (setmembers `/Game/TurnBasedJRPGTemplate/Blueprints/Structs/S_PlayerUnitData` :`StructRef` _value :`curentMP` (+ (`.curentMP_6_79399572456CC89F79B2DA9F0A8BB445` (break `/Game/TurnBasedJRPGTemplate/Blueprints/Structs/S_PlayerUnitData` _value)) 10))))

(event `self.OnBuffEnded`
  (bind _firstlevelstats (defaults `/Game/TurnBasedJRPGTemplate/Blueprints/Units/PlayerUnits/BP_MagePlayerUnit` "/Game/TurnBasedJRPGTemplate/Blueprints/Units/PlayerUnits/BP_MagePlayerUnit.BP_MagePlayerUnit_C"))
  (bind ((`minAttack_14_0D64A0224152A597434ECDAF6DFC9964` _minattack) (`maxAttack_15_24D8527844E2DFB657716C9F16A4AE21` _maxattack) (`defense_16_FEA01B2E4A985F64F6B9359A13E3F651` _defense)) (break `/Game/TurnBasedJRPGTemplate/Blueprints/Structs/S_UnitStats` _firstlevelstats))
  (set `self.IsOneMoreSpiffBuffApplied?` false)
  (setmembers `/Game/TurnBasedJRPGTemplate/Blueprints/Structs/S_UnitStats` :`StructRef` _firstlevelstats :`minAttack` (- _minattack 15) :`maxAttack` (- _maxattack 15) :`defense` (+ _defense 10)))

(fn `UserConstructionScript`
  (`parent.UserConstructionScript`))