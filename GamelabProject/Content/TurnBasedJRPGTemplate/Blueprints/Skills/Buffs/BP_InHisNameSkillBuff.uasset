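; In His Name skill buff for the turn-based JRPG, meant to raise the targeted unit's MaxAttack by 8 until it ends.
; ApplyBuff finds the BattleController and takes its CurrentTargetUnit, and OnBuffEnded uses that controller target reference to subtract the 8.
; Both events read and set the stats struct through the unit's class defaults, not the unit instance's own stats.
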(event `self.ApplyBuff`
  (bind _returnvalue (`GameplayStatics.GetActorOfClass` "/Game/TurnBasedJRPGTemplate/Blueprints/Battle/BP_BattleController.BP_BattleController_C"))
  (bind _output_get (set `self.Current Target Unit` (`/Game/TurnBasedJRPGTemplate/Blueprints/Battle/BP_BattleController.currentTargetUnit` _returnvalue)))
  (bind _firstlevelstats (defaults `Object` (`GameplayStatics.GetObjectClass` _output_get)))
  (setmembers `/Game/TurnBasedJRPGTemplate/Blueprints/Structs/S_UnitStats` :`StructRef` _firstlevelstats :`maxAttack` (+ (`.maxAttack_15_24D8527844E2DFB657716C9F16A4AE21` (break `/Game/TurnBasedJRPGTemplate/Blueprints/Structs/S_UnitStats` _firstlevelstats)) 8)))

(event `self.OnBuffEnded`
  (bind _firstlevelstats (defaults `Object` (`GameplayStatics.GetObjectClass` (`self.Current Target Unit`))))
  (setmembers `/Game/TurnBasedJRPGTemplate/Blueprints/Structs/S_UnitStats` :`StructRef` _firstlevelstats :`maxAttack` (- (`.maxAttack_15_24D8527844E2DFB657716C9F16A4AE21` (break `/Game/TurnBasedJRPGTemplate/Blueprints/Structs/S_UnitStats` _firstlevelstats)) 8)))

(fn `UserConstructionScript`
  (`parent.UserConstructionScript`))