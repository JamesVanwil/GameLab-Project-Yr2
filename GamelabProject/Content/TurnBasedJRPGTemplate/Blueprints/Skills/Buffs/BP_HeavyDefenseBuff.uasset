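; BP_HeavyDefenseBuff is a turn-based battle skill buff that trades a higher Defense for a longer ActionTime on the targeted unit.
; ApplyBuff flags the buff as applied, caches the battle controller's current target and adds fixed amounts to both stats.
; OnBuffEnded clears the flag and subtracts the same amounts using that cached unit.
; Both events target stats read from the unit's class defaults, not its instance variables.
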(event `self.ApplyBuff`
  (set `self.HasHeavyDefBuffBeenApplied?` true)
  (bind _returnvalue (`GameplayStatics.GetActorOfClass` "/Game/TurnBasedJRPGTemplate/Blueprints/Battle/BP_BattleController.BP_BattleController_C"))
  (bind _output_get (set `self.Current Target Unit` (`/Game/TurnBasedJRPGTemplate/Blueprints/Battle/BP_BattleController.currentTargetUnit` _returnvalue)))
  (bind _firstlevelstats (defaults `Object` (`GameplayStatics.GetObjectClass` _output_get)))
  (bind ((`defense_16_FEA01B2E4A985F64F6B9359A13E3F651` _defense) (`actionTime_31_CD6B6FA04FF3CB1C1BA72A93110B7A28` _actiontime)) (break `/Game/TurnBasedJRPGTemplate/Blueprints/Structs/S_UnitStats` _firstlevelstats))
  (setmembers `/Game/TurnBasedJRPGTemplate/Blueprints/Structs/S_UnitStats` :`StructRef` _firstlevelstats :`defense` (+ _defense 15) :`actionTime` (+ _actiontime 0.3)))

(event `self.OnBuffEnded`
  (bind _firstlevelstats (defaults `Object` (`GameplayStatics.GetObjectClass` (`self.Current Target Unit`))))
  (bind ((`defense_16_FEA01B2E4A985F64F6B9359A13E3F651` _defense) (`actionTime_31_CD6B6FA04FF3CB1C1BA72A93110B7A28` _actiontime)) (break `/Game/TurnBasedJRPGTemplate/Blueprints/Structs/S_UnitStats` _firstlevelstats))
  (set `self.HasHeavyDefBuffBeenApplied?` false)
  (setmembers `/Game/TurnBasedJRPGTemplate/Blueprints/Structs/S_UnitStats` :`StructRef` _firstlevelstats :`defense` (- _defense 15) :`actionTime` (- _actiontime 0.3)))

(fn `UserConstructionScript`
  (`parent.UserConstructionScript`))