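; United We Stand buff for the turn-based JRPG template, meant to raise a unit's Defense and Magic Defense by a flat amount.
; ApplyBuff flags itself as applied, stores the battle controller's current target, and adds the bonus to both stats.
; OnBuffEnded clears the flag and subtracts the same amount for the stored unit.
; Both events read and set the stat struct through the unit's class defaults, not its instance variables.
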(event `self.ApplyBuff`
  (set `self.HasUnitedWeStandBuffBeenApplied?` true)
  (bind _returnvalue (`GameplayStatics.GetActorOfClass` "/Game/TurnBasedJRPGTemplate/Blueprints/Battle/BP_BattleController.BP_BattleController_C"))
  (bind _output_get (set `self.Current Target Unit` (`/Game/TurnBasedJRPGTemplate/Blueprints/Battle/BP_BattleController.currentTargetUnit` _returnvalue)))
  (bind _firstlevelstats (defaults `Object` (`GameplayStatics.GetObjectClass` _output_get)))
  (bind ((`defense_16_FEA01B2E4A985F64F6B9359A13E3F651` _defense) (`magicDefense_25_FE826AEB41C90F001AB72DA466AF2D63` _magicdefense)) (break `/Game/TurnBasedJRPGTemplate/Blueprints/Structs/S_UnitStats` _firstlevelstats))
  (setmembers `/Game/TurnBasedJRPGTemplate/Blueprints/Structs/S_UnitStats` :`StructRef` _firstlevelstats :`defense` (+ _defense 10) :`magicDefense` (+ _magicdefense 10)))

(event `self.OnBuffEnded`
  (bind _firstlevelstats (defaults `Object` (`GameplayStatics.GetObjectClass` (`self.Current Target Unit`))))
  (bind ((`defense_16_FEA01B2E4A985F64F6B9359A13E3F651` _defense) (`magicDefense_25_FE826AEB41C90F001AB72DA466AF2D63` _magicdefense)) (break `/Game/TurnBasedJRPGTemplate/Blueprints/Structs/S_UnitStats` _firstlevelstats))
  (set `self.HasUnitedWeStandBuffBeenApplied?` false)
  (setmembers `/Game/TurnBasedJRPGTemplate/Blueprints/Structs/S_UnitStats` :`StructRef` _firstlevelstats :`defense` (- _defense 10) :`magicDefense` (- _magicdefense 10)))

(fn `UserConstructionScript`
  (`parent.UserConstructionScript`))