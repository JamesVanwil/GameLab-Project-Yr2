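; Tarot 3 buff for the turn-based JRPG that toggles tarot effects on player units with a matching tarot equipped.
; ApplyBuff checks each unit's helm, boots and two socket slots, flags the first matching tarot actor active, and lowers attack, magical attack and action time on class-default FirstLevelStats.
; OnBuffEnded clears the flag and adds those amounts back.
; TestAddTurn increments the duration turn counter.
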(event `TestAddTurn`
  ;[1 1 1] Turn counter
  (set `self.durationTurn` (+ (`self.durationTurn`) 1)))

(event `self.ApplyBuff`
  ;[1 1 1] Buff Applied
  (bind _asbp_jrpgplayer_controller (cast `/Game/TurnBasedJRPGTemplate/Blueprints/Controllers/BP_JRPGPlayerController` (`GameplayStatics.GetPlayerController` 0)))
  (bind _playerunits (`/Game/TurnBasedJRPGTemplate/Blueprints/Controllers/BP_JRPGPlayerController.playerUnits` _asbp_jrpgplayer_controller))
  (bind _keys (`BlueprintMapLibrary.Map_Keys` _playerunits))
  (for _array_element _keys
    (bind ((`HelmTarot1_31_751FB906466EBEC2597E348A40B77276` _helmtarot1) (`BootsTarot2_34_494ABC0E4604C5FA6716CDB909310B09` _bootstarot2) (`TarotSocket3_45_BED5D59A4998303E41DEC9B4897C5719` _tarotsocket3) (`TarotSocket4_46_D6A172B14760122AE2FE539D76A47580` _tarotsocket4)) (break `/Game/TurnBasedJRPGTemplate/Blueprints/Structs/S_PlayerUnitData` (`BlueprintMapLibrary.Map_Find` _playerunits _array_element)))
    (if (== _helmtarot1 "/Game/TurnBasedJRPGTemplate/Blueprints/Items/Equipment/TarotSocket3/Tarot3Helm.Tarot3Helm_C")
      (bind _returnvalue (`GameplayStatics.GetActorOfClass` _helmtarot1))
      (set `/Game/TurnBasedJRPGTemplate/Blueprints/Items/Equipment/Helms/BP_HelmBase.isTarotActive?` true _returnvalue)
      (`KismetSystemLibrary.PrintString` "Buff applied" :!label _label)
      (bind (_isdreadful_ _firstlevelstats) (defaults `Object` _array_element))
      (bind ((`maxAttack_15_24D8527844E2DFB657716C9F16A4AE21` _maxattack) (`maxMagicalAttack_24_C0C7731143A09315B418E7876A1F2F19` _maxmagicalattack) (`actionTime_31_CD6B6FA04FF3CB1C1BA72A93110B7A28` _actiontime)) (break `/Game/TurnBasedJRPGTemplate/Blueprints/Structs/S_UnitStats` _firstlevelstats))
      (setmembers `/Game/TurnBasedJRPGTemplate/Blueprints/Structs/S_UnitStats` :`StructRef` _firstlevelstats :`maxAttack` (- _maxattack 10) :`maxMagicalAttack` (- _maxmagicalattack 10) :`actionTime` (- _actiontime 0.5))
      (elif (== _bootstarot2 "/Game/TurnBasedJRPGTemplate/Blueprints/Items/Equipment/TarotSocket3/Tarot3Boots.Tarot3Boots_C")
        (bind _returnvalue_2 (`GameplayStatics.GetActorOfClass` _bootstarot2))
        (set `/Game/TurnBasedJRPGTemplate/Blueprints/Items/Equipment/Boots/BP_BootsBase.isTarotActive?` true _returnvalue_2)
        (goto _label)
        (elif (== _tarotsocket3 "/Game/TurnBasedJRPGTemplate/Blueprints/Items/Equipment/TarotSocket3/Tarot3.Tarot3_C")
          (bind _returnvalue_3 (`GameplayStatics.GetActorOfClass` _tarotsocket3))
          (set `/Game/TurnBasedJRPGTemplate/Blueprints/Items/Equipment/TarotSocket3/TarotSocket3_Base.isTarotActive?` true _returnvalue_3)
          (goto _label)
          (elif (== _tarotsocket4 "/Game/TurnBasedJRPGTemplate/Blueprints/Items/Equipment/TarotSocket3/Tarot3_4.Tarot3_4_C")
            (bind _returnvalue_4 (`GameplayStatics.GetActorOfClass` _tarotsocket4))
            (set `/Game/TurnBasedJRPGTemplate/Blueprints/Items/Equipment/TarotSocket4/TarotSocket4_Base.isTarotActive?` true _returnvalue_4)
            (goto _label)))))))

(event `self.OnBuffEnded`
  ;[1 1 1] Buff Ended
  (bind _asbp_jrpgplayer_controller (cast `/Game/TurnBasedJRPGTemplate/Blueprints/Controllers/BP_JRPGPlayerController` (`GameplayStatics.GetPlayerController` 0)))
  (bind _playerunits (`/Game/TurnBasedJRPGTemplate/Blueprints/Controllers/BP_JRPGPlayerController.playerUnits` _asbp_jrpgplayer_controller))
  (bind _keys (`BlueprintMapLibrary.Map_Keys` _playerunits))
  (for _array_element _keys
    (bind ((`HelmTarot1_31_751FB906466EBEC2597E348A40B77276` _helmtarot1) (`BootsTarot2_34_494ABC0E4604C5FA6716CDB909310B09` _bootstarot2) (`TarotSocket3_45_BED5D59A4998303E41DEC9B4897C5719` _tarotsocket3) (`TarotSocket4_46_D6A172B14760122AE2FE539D76A47580` _tarotsocket4)) (break `/Game/TurnBasedJRPGTemplate/Blueprints/Structs/S_PlayerUnitData` (`BlueprintMapLibrary.Map_Find` _playerunits _array_element)))
    (if (== _helmtarot1 "/Game/TurnBasedJRPGTemplate/Blueprints/Items/Equipment/TarotSocket3/Tarot3Helm.Tarot3Helm_C")
      (bind _returnvalue (`GameplayStatics.GetActorOfClass` _helmtarot1))
      (set `/Game/TurnBasedJRPGTemplate/Blueprints/Items/Equipment/Helms/BP_HelmBase.isTarotActive?` false _returnvalue)
      (`KismetSystemLibrary.PrintString` "Buff Ended" :!label _label_2)
      (bind (_isdreadful_ _firstlevelstats) (defaults `Object` _array_element))
      (bind ((`maxAttack_15_24D8527844E2DFB657716C9F16A4AE21` _maxattack) (`maxMagicalAttack_24_C0C7731143A09315B418E7876A1F2F19` _maxmagicalattack) (`actionTime_31_CD6B6FA04FF3CB1C1BA72A93110B7A28` _actiontime)) (break `/Game/TurnBasedJRPGTemplate/Blueprints/Structs/S_UnitStats` _firstlevelstats))
      (setmembers `/Game/TurnBasedJRPGTemplate/Blueprints/Structs/S_UnitStats` :`StructRef` _firstlevelstats :`maxAttack` (+ _maxattack 10) :`maxMagicalAttack` (+ _maxmagicalattack 10) :`actionTime` (+ _actiontime 0.5))
      (elif (== _bootstarot2 "/Game/TurnBasedJRPGTemplate/Blueprints/Items/Equipment/TarotSocket3/Tarot3Boots.Tarot3Boots_C")
        (bind _returnvalue_2 (`GameplayStatics.GetActorOfClass` _bootstarot2))
        (set `/Game/TurnBasedJRPGTemplate/Blueprints/Items/Equipment/Boots/BP_BootsBase.isTarotActive?` false _returnvalue_2)
        (goto _label_2)
        (elif (== _tarotsocket3 "/Game/TurnBasedJRPGTemplate/Blueprints/Items/Equipment/TarotSocket3/Tarot3.Tarot3_C")
          (bind _returnvalue_3 (`GameplayStatics.GetActorOfClass` _tarotsocket3))
          (set `/Game/TurnBasedJRPGTemplate/Blueprints/Items/Equipment/TarotSocket3/TarotSocket3_Base.isTarotActive?` false _returnvalue_3)
          (goto _label_2)
          (elif (== _tarotsocket4 "/Game/TurnBasedJRPGTemplate/Blueprints/Items/Equipment/TarotSocket3/Tarot3_4.Tarot3_4_C")
            (bind _returnvalue_4 (`GameplayStatics.GetActorOfClass` _tarotsocket4))
            (set `/Game/TurnBasedJRPGTemplate/Blueprints/Items/Equipment/TarotSocket4/TarotSocket4_Base.isTarotActive?` false _returnvalue_4)
            (goto _label_2)))))))

(fn `UserConstructionScript`
  (`parent.UserConstructionScript`))