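; BP_BuffTarot7 is a JRPG buff that raises max attack for player units with a Tarot 7 item equipped.
; ApplyBuff loops over the player controller's PlayerUnits map, checking each unit's helm, boots and two tarot sockets for Tarot 7 variants.
; Matches get a flat MaxAttack increase set on stats read from the unit's class defaults, and OnBuffEnded repeats the check to subtract it.
; Both events print debug messages.
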(event `self.ApplyBuff`
  (bind _asbp_jrpgplayer_controller (cast `/Game/TurnBasedJRPGTemplate/Blueprints/Controllers/BP_JRPGPlayerController` (`GameplayStatics.GetPlayerController` 0)))
  (bind _playerunits (`/Game/TurnBasedJRPGTemplate/Blueprints/Controllers/BP_JRPGPlayerController.playerUnits` _asbp_jrpgplayer_controller))
  (bind _keys (`BlueprintMapLibrary.Map_Keys` _playerunits))
  (for _array_element _keys
    (bind ((`HelmTarot1_31_751FB906466EBEC2597E348A40B77276` _helmtarot1) (`BootsTarot2_34_494ABC0E4604C5FA6716CDB909310B09` _bootstarot2) (`TarotSocket3_45_BED5D59A4998303E41DEC9B4897C5719` _tarotsocket3) (`TarotSocket4_46_D6A172B14760122AE2FE539D76A47580` _tarotsocket4)) (break `/Game/TurnBasedJRPGTemplate/Blueprints/Structs/S_PlayerUnitData` (`BlueprintMapLibrary.Map_Find` _playerunits _array_element)))
    (if (or (== _helmtarot1 "/Game/TurnBasedJRPGTemplate/Blueprints/Items/Equipment/Tarot_7/BP_Tarot7Helm.BP_Tarot7Helm_C") (== _bootstarot2 "/Game/TurnBasedJRPGTemplate/Blueprints/Items/Equipment/Tarot_7/BP_Tarot7Boots.BP_Tarot7Boots_C") (== _tarotsocket3 "/Game/TurnBasedJRPGTemplate/Blueprints/Items/Equipment/Tarot_7/BP_Tarot7-3.BP_Tarot7-3_C") (== _tarotsocket4 "/Game/TurnBasedJRPGTemplate/Blueprints/Items/Equipment/Tarot_7/BP_Tarot7-4.BP_Tarot7-4_C"))
      (`KismetSystemLibrary.PrintString` "Buff applied")
      (bind _firstlevelstats (defaults `Object` _array_element))
      (setmembers `/Game/TurnBasedJRPGTemplate/Blueprints/Structs/S_UnitStats` :`StructRef` _firstlevelstats :`maxAttack` (+ (`.maxAttack_15_24D8527844E2DFB657716C9F16A4AE21` (break `/Game/TurnBasedJRPGTemplate/Blueprints/Structs/S_UnitStats` _firstlevelstats)) 10)))))

(event `self.OnBuffEnded`
  (`KismetSystemLibrary.PrintString` "Buff Ended")
  (bind _asbp_jrpgplayer_controller (cast `/Game/TurnBasedJRPGTemplate/Blueprints/Controllers/BP_JRPGPlayerController` (`GameplayStatics.GetPlayerController` 0)))
  (bind _playerunits (`/Game/TurnBasedJRPGTemplate/Blueprints/Controllers/BP_JRPGPlayerController.playerUnits` _asbp_jrpgplayer_controller))
  (bind _keys (`BlueprintMapLibrary.Map_Keys` _playerunits))
  (for _array_element _keys
    (bind ((`HelmTarot1_31_751FB906466EBEC2597E348A40B77276` _helmtarot1) (`BootsTarot2_34_494ABC0E4604C5FA6716CDB909310B09` _bootstarot2) (`TarotSocket3_45_BED5D59A4998303E41DEC9B4897C5719` _tarotsocket3) (`TarotSocket4_46_D6A172B14760122AE2FE539D76A47580` _tarotsocket4)) (break `/Game/TurnBasedJRPGTemplate/Blueprints/Structs/S_PlayerUnitData` (`BlueprintMapLibrary.Map_Find` _playerunits _array_element)))
    (if (or (== _helmtarot1 "/Game/TurnBasedJRPGTemplate/Blueprints/Items/Equipment/Tarot_7/BP_Tarot7Helm.BP_Tarot7Helm_C") (== _bootstarot2 "/Game/TurnBasedJRPGTemplate/Blueprints/Items/Equipment/Tarot_7/BP_Tarot7Boots.BP_Tarot7Boots_C") (== _tarotsocket3 "/Game/TurnBasedJRPGTemplate/Blueprints/Items/Equipment/Tarot_7/BP_Tarot7-3.BP_Tarot7-3_C") (== _tarotsocket4 "/Game/TurnBasedJRPGTemplate/Blueprints/Items/Equipment/Tarot_7/BP_Tarot7-4.BP_Tarot7-4_C"))
      (bind _firstlevelstats (defaults `Object` _array_element))
      (setmembers `/Game/TurnBasedJRPGTemplate/Blueprints/Structs/S_UnitStats` :`StructRef` _firstlevelstats :`maxAttack` (- (`.maxAttack_15_24D8527844E2DFB657716C9F16A4AE21` (break `/Game/TurnBasedJRPGTemplate/Blueprints/Structs/S_UnitStats` _firstlevelstats)) 10)))))

(fn `UserConstructionScript`
  (`parent.UserConstructionScript`))