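; Basic attack skill for the turn-based JRPG template that damages the battle controller's current target.
; Highlights the target with a damage overlay, optionally moves the attacker to it, then plays the skill animation.
; The animation notify deals multiplier-based damage and refreshes the combat UI on success.
; When the animation ends, it clears the overlay, moves the attacker back if needed and signals completion; the ApplyBuffs call is unwired.
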(event `/Game/TurnBasedJRPGTemplate/Blueprints/Skills/BP_SkillBase.UseSkill`
  ;[1 1 1] Move to target
  (`MeshComponent.SetOverlayMaterial` (`/Game/TurnBasedJRPGTemplate/Blueprints/Units/BP_UnitBase.SkeletalMesh` (`/Game/TurnBasedJRPGTemplate/Blueprints/Battle/BP_BattleController.currentTargetUnit` (`self.battleController`))) "/Game/Effects/Materials/Damage_Material.Damage_Material")
  (if (`/Game/TurnBasedJRPGTemplate/Blueprints/Battle/BP_BattleController.shouldUnitsMoveToTarget` (`self.battleController`))
    (`/Game/TurnBasedJRPGTemplate/Blueprints/Battle/BP_BattleController.MoveToTarget` (`self.battleController`) (`SceneComponent.K2_GetComponentLocation` (`/Game/TurnBasedJRPGTemplate/Blueprints/Units/BP_UnitBase.AttackerLocation` (`/Game/TurnBasedJRPGTemplate/Blueprints/Battle/BP_BattleController.currentTargetUnit` (`self.battleController`)))) (delegate `OnUnitMovedToTargetHandler`) true)
    (else
      (`self.PlaySkillAnimation` :!label _label))))

(event `OnUnitMovedToTargetHandler`
  ;[1 1 1] Move to target
  (goto _label))

(event `self.UseSkillOnNotify`
  ;[1 1 1] Attack
  (bind _ishit (`/Game/TurnBasedJRPGTemplate/Blueprints/Battle/BP_BattleController.DealDamage` (`self.battleController`) 0 (`self.damageMultiplier`)))
  (if _ishit
    (`/Game/CommonUI/BattleUI/CWB_BattleUI.MidTurnInitEverything` (`self.CombatUIRef`))))

(event `self.OnSkillAnimationEnded`
  ;[1 1 1] Attack
  (`MeshComponent.SetOverlayMaterial` (`/Game/TurnBasedJRPGTemplate/Blueprints/Units/BP_UnitBase.SkeletalMesh` (`/Game/TurnBasedJRPGTemplate/Blueprints/Battle/BP_BattleController.currentTargetUnit` (`self.battleController`))) null)
  (if (`/Game/TurnBasedJRPGTemplate/Blueprints/Battle/BP_BattleController.shouldUnitsMoveToTarget` (`self.battleController`))
    (`/Game/TurnBasedJRPGTemplate/Blueprints/Battle/BP_BattleController.MoveToTarget` (`self.battleController`) (`/Game/TurnBasedJRPGTemplate/Blueprints/Units/BP_UnitBase.initialLocation` (`/Game/TurnBasedJRPGTemplate/Blueprints/Battle/BP_BattleController.currentAttackingUnit` (`self.battleController`))) (delegate `OnUnitMovedBackHandler`) false)
    (else
      (`self.OnSkillUsed` :!label _label_2))))

(event `OnUnitMovedBackHandler`
  ;[1 1 1] Attack
  (goto _label_2))

(fn `UserConstructionScript`
  (`parent.UserConstructionScript`))