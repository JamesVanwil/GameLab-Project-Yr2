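; Precision Shot battle skill that consumes one bullet item to fire a projectile at the current target; without bullets the animation never plays.
; A Roland static tarot in either Mage socket raises the damage multiplier when the Mage attacks.
; The animation notify spawns a BP_Arrow at a random diagonal offset around the target, whose hit callback deals damage through the BattleController if the target lives.
; A damage overlay material marks the target during the shot.
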(event `Roland Static Tarot Check`
  (bind _returnvalue (== (`GameplayStatics.GetObjectClass` (`/Game/TurnBasedJRPGTemplate/Blueprints/Battle/BP_BattleController.currentAttackingUnit` (`self.battleController`))) "/Game/TurnBasedJRPGTemplate/Blueprints/Units/PlayerUnits/BP_MagePlayerUnit.BP_MagePlayerUnit_C"))
  ;[1 1 1] Roland Static Tarot Check
  (bind _asbp_jrpgplayer_controller (cast `/Game/TurnBasedJRPGTemplate/Blueprints/Controllers/BP_JRPGPlayerController` (`GameplayStatics.GetPlayerController` 0)))
  (bind ((`StaticTarotSocket1_49_386CDF41496C8A1A94652D804435853A` _statictarotsocket1) (`StaticTarotSocket2_52_C805DEBE4D5F6DCAF20172BE33318FDF` _statictarotsocket2)) (break `/Game/TurnBasedJRPGTemplate/Blueprints/Structs/S_PlayerUnitData` (`BlueprintMapLibrary.Map_Find` (`/Game/TurnBasedJRPGTemplate/Blueprints/Controllers/BP_JRPGPlayerController.playerUnits` _asbp_jrpgplayer_controller) "/Game/TurnBasedJRPGTemplate/Blueprints/Units/PlayerUnits/BP_MagePlayerUnit.BP_MagePlayerUnit_C")))
  (if (and (== _statictarotsocket1 "/Game/TurnBasedJRPGTemplate/Blueprints/Items/Equipment/StatictTarot1/Roland/BP_StaticTarot1Roland.BP_StaticTarot1Roland_C") _returnvalue)
    (set `self.damageMultiplier` 1.8)
    (elif (and (== _statictarotsocket2 "/Game/TurnBasedJRPGTemplate/Blueprints/Items/Equipment/StaticTarot2/Roland/BP_StaticTarot2Roland.BP_StaticTarot2Roland_C") _returnvalue)
      (set `self.damageMultiplier` 2.0))))

(event `self.UseSkill`
  ;[1 1 1] Spawn 2 bullets
  (`self.Roland Static Tarot Check`)
  (`MeshComponent.SetOverlayMaterial` (`/Game/TurnBasedJRPGTemplate/Blueprints/Units/BP_UnitBase.SkeletalMesh` (`/Game/TurnBasedJRPGTemplate/Blueprints/Battle/BP_BattleController.currentTargetUnit` (`self.battleController`))) "/Game/Effects/Materials/Damage_Material.Damage_Material")
  (`KismetSystemLibrary.PrintString` (`KismetStringLibrary.Conv_DoubleToString` (`self.damageMultiplier`)))
  (if (>= (`BlueprintMapLibrary.Map_Find` (`/Game/TurnBasedJRPGTemplate/Blueprints/Controllers/BP_JRPGPlayerController.miscItems` (`self.jRPGPlayerController`)) "/Game/TurnBasedJRPGTemplate/Blueprints/Items/MiscItems/BP_Bullet.BP_Bullet_C") 1)
    (`/Game/TurnBasedJRPGTemplate/Blueprints/Controllers/BP_JRPGPlayerController.RemoveMiscItem` (`self.jRPGPlayerController`) "/Game/TurnBasedJRPGTemplate/Blueprints/Items/MiscItems/BP_Bullet.BP_Bullet_C" 1)
    (`self.PlaySkillAnimation`)))

(event `self.UseSkillOnNotify`
  ;[1 1 1] Spawn 2 bullets
  (`self.SpawnFireBall`)
  (`GameplayStatics.PlaySound2D` "/Game/Audio/Shooting_Revolver.Shooting_Revolver" 1.0 1.0 0.0 null null)
  (`KismetSystemLibrary.Delay` 0.5)
  (`MeshComponent.SetOverlayMaterial` (`/Game/TurnBasedJRPGTemplate/Blueprints/Units/BP_UnitBase.SkeletalMesh` (`/Game/TurnBasedJRPGTemplate/Blueprints/Battle/BP_BattleController.currentTargetUnit` (`self.battleController`))) null)
  (`self.OnSkillUsed`))

(event `SpawnFireBall`
  ;[1 1 1] Bullets deal damage
  (bind _returnvalue (`|SpawnActorFromClass` "/Game/TurnBasedJRPGTemplate/Blueprints/Projectiles/BP_Arrow.BP_Arrow_C" (`KismetMathLibrary.MakeTransform` (+ (`self.K2_GetActorLocation` (`/Game/TurnBasedJRPGTemplate/Blueprints/Battle/BP_BattleController.currentTargetUnit` (`self.battleController`))) (`KismetMathLibrary.MakeVector` (* (`KismetMathLibrary.RandomFloatInRange` 150.0 250.0) (select `bool` (`KismetMathLibrary.RandomBool`) :`false` 1.0 :`true` -1.0)) (* (`KismetMathLibrary.RandomFloatInRange` 150.0 250.0) (select `bool` (`KismetMathLibrary.RandomBool`) :`false` 1.0 :`true` -1.0))))) "Undefined" "OverrideRootScale" null (`/Game/TurnBasedJRPGTemplate/Blueprints/Battle/BP_BattleController.currentTargetUnit` (`self.battleController`)) null))
  (add `/Game/TurnBasedJRPGTemplate/Blueprints/Projectiles/BP_ProjectileBase.OnProjectileHit` _returnvalue (delegate `OnProjectilHitHandler`))
  (`/Game/TurnBasedJRPGTemplate/Blueprints/Projectiles/BP_ProjectileBase.MoveProjectileToTarget` _returnvalue))

(event `OnProjectilHitHandler`
  ;[1 1 1] Bullets deal damage
  (bind _isunitdead (`/Game/TurnBasedJRPGTemplate/Blueprints/Units/BP_UnitBase.IsUnitDead` (`/Game/TurnBasedJRPGTemplate/Blueprints/Battle/BP_BattleController.currentTargetUnit` (`self.battleController`))))
  (if (not _isunitdead)
    (`/Game/TurnBasedJRPGTemplate/Blueprints/Battle/BP_BattleController.DealDamage` (`self.battleController`) 0 (`self.damageMultiplier`))))

(fn `UserConstructionScript`
  (`parent.UserConstructionScript`))