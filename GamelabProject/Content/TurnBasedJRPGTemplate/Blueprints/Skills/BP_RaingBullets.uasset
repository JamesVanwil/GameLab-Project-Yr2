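; Turn-based JRPG skill that fires a six-shot bullet barrage at the current target, consuming six bullet items and doing nothing if fewer are held.
; The animation notify spawns timed BP_Arrow projectiles with revolver sounds, then signals skill completion.
; Each projectile starts at a random horizontal offset around the target, homes toward it, and deals multiplier-based damage through the BattleController on hit if the target is alive.
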(event `self.UseSkill`
  ;[1 1 1] Spawn 3 bullets
  (if (>= (`BlueprintMapLibrary.Map_Find` (`/Game/TurnBasedJRPGTemplate/Blueprints/Controllers/BP_JRPGPlayerController.miscItems` (`self.jRPGPlayerController`)) "/Game/TurnBasedJRPGTemplate/Blueprints/Items/MiscItems/BP_Bullet.BP_Bullet_C") 6)
    (`/Game/TurnBasedJRPGTemplate/Blueprints/Controllers/BP_JRPGPlayerController.RemoveMiscItem` (`self.jRPGPlayerController`) "/Game/TurnBasedJRPGTemplate/Blueprints/Items/MiscItems/BP_Bullet.BP_Bullet_C" 6)
    (`self.PlaySkillAnimation`)))

(event `self.UseSkillOnNotify`
  ;[1 1 1] Spawn 3 bullets
  (`self.SpawnFireBall`)
  (`GameplayStatics.PlaySound2D` "/Game/Audio/Shooting_Revolver.Shooting_Revolver" 1.0 1.0 0.0 null null)
  (`KismetSystemLibrary.Delay` 0.5)
  (`self.SpawnFireBall`)
  (`GameplayStatics.PlaySound2D` "/Game/Audio/Shooting_Revolver.Shooting_Revolver" 1.0 1.0 0.0 null null)
  (`KismetSystemLibrary.Delay` 0.5)
  (`self.SpawnFireBall`)
  (`GameplayStatics.PlaySound2D` "/Game/Audio/Shooting_Revolver.Shooting_Revolver" 1.0 1.0 0.0 null null)
  (`KismetSystemLibrary.Delay` 0.5)
  (`self.SpawnFireBall`)
  (`GameplayStatics.PlaySound2D` "/Game/Audio/Shooting_Revolver.Shooting_Revolver" 1.0 1.0 0.0 null null)
  (`KismetSystemLibrary.Delay` 0.5)
  (`self.SpawnFireBall`)
  (`GameplayStatics.PlaySound2D` "/Game/Audio/Shooting_Revolver.Shooting_Revolver" 1.0 1.0 0.0 null null)
  (`KismetSystemLibrary.Delay` 0.5)
  (`self.SpawnFireBall`)
  (`GameplayStatics.PlaySound2D` "/Game/Audio/Shooting_Revolver.Shooting_Revolver" 1.0 1.0 0.0 null null)
  (`KismetSystemLibrary.Delay` 1.5)
  (`self.OnSkillUsed`))

(event `SpawnFireBall`
  ;[1 1 1] Bullets deal damage
  (bind _returnvalue (`|SpawnActorFromClass` "/Game/TurnBasedJRPGTemplate/Blueprints/Projectiles/BP_Arrow.BP_Arrow_C" (`KismetMathLibrary.MakeTransform` (+ (`self.K2_GetActorLocation` (`/Game/TurnBasedJRPGTemplate/Blueprints/Battle/BP_BattleController.currentTargetUnit` (`self.battleController`))) (`KismetMathLibrary.MakeVector` (* (`KismetMathLibrary.RandomFloatInRange` 150.0 250.0) (select `bool` (`KismetMathLibrary.RandomBool`) :`false` 1.0 :`true` -1.0)) (* (`KismetMathLibrary.RandomFloatInRange` 150.0 250.0) (select `bool` (`KismetMathLibrary.RandomBool`) :`false` 1.0 :`true` -1.0))))) "Undefined" "OverrideRootScale" null (`/Game/TurnBasedJRPGTemplate/Blueprints/Battle/BP_BattleController.currentTargetUnit` (`self.battleController`)) null))
  (add `/Game/TurnBasedJRPGTemplate/Blueprints/Projectiles/BP_ProjectileBase.OnProjectileHit` _returnvalue (delegate `OnProjectilHitHandler`))
  (`/Game/TurnBasedJRPGTemplate/Blueprints/Projectiles/BP_ProjectileBase.MoveProjectileToTarget` _returnvalue))

(event `OnProjectilHitHandler`
  ;[1 1 1] Bullets deal damage
  (bind _isunitdead (`/Game/TurnBasedJRPGTemplate/Blueprints/Units/BP_UnitBase.IsUnitDead` (`/Game/TurnBasedJRPGTemplate/Blueprints/Battle/BP_BattleController.currentTargetUnit` (`self.battleController`))))
  (if (not _isunitdead)
    (`/Game/TurnBasedJRPGTemplate/Blueprints/Battle/BP_BattleController.DealDamage` (`self.battleController`) 0 (`self.damageMultiplier`))))

(fn `UserConstructionScript`
  (`parent.UserConstructionScript`))