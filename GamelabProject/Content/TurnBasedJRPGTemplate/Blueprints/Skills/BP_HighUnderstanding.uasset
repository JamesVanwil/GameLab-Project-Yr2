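; BP_HighUnderstanding is a turn-based battle skill that buffs the current target unit.
; When used, it optionally moves the caster to the target through the BattleController, then plays the skill animation.
; An animation notify briefly flashes a shield overlay material on the target's mesh before applying buffs.
; When the animation ends, the caster returns to its initial location if it moved, then the skill reports completion.
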(event `/Game/TurnBasedJRPGTemplate/Blueprints/Skills/BP_SkillBase.UseSkill`
  (if (`/Game/TurnBasedJRPGTemplate/Blueprints/Battle/BP_BattleController.shouldUnitsMoveToTarget` (`self.battleController`))
    (`/Game/TurnBasedJRPGTemplate/Blueprints/Battle/BP_BattleController.MoveToTarget` (`self.battleController`) (`SceneComponent.K2_GetComponentLocation` (`/Game/TurnBasedJRPGTemplate/Blueprints/Units/BP_UnitBase.AttackerLocation` (`/Game/TurnBasedJRPGTemplate/Blueprints/Battle/BP_BattleController.currentTargetUnit` (`self.battleController`)))) (delegate `OnUnitMovedToTargetHandler`) true)
    (else
      (`self.PlaySkillAnimation` :!label _label))))

(event `OnUnitMovedToTargetHandler`
  (goto _label))

(event `self.UseSkillOnNotify`
  (`MeshComponent.SetOverlayMaterial` (`/Game/TurnBasedJRPGTemplate/Blueprints/Units/BP_UnitBase.SkeletalMesh` (`/Game/TurnBasedJRPGTemplate/Blueprints/Battle/BP_BattleController.currentTargetUnit` (`self.battleController`))) "/Game/Effects/Materials/Shield_Material.Shield_Material")
  (`KismetSystemLibrary.Delay` 1.25)
  (`MeshComponent.SetOverlayMaterial` (`/Game/TurnBasedJRPGTemplate/Blueprints/Units/BP_UnitBase.SkeletalMesh` (`/Game/TurnBasedJRPGTemplate/Blueprints/Battle/BP_BattleController.currentTargetUnit` (`self.battleController`))) null)
  (`self.ApplyBuffs` (`|MakeArray` (`/Game/TurnBasedJRPGTemplate/Blueprints/Battle/BP_BattleController.currentTargetUnit` (`self.battleController`)))))

(event `self.OnSkillAnimationEnded`
  (if (`/Game/TurnBasedJRPGTemplate/Blueprints/Battle/BP_BattleController.shouldUnitsMoveToTarget` (`self.battleController`))
    (`/Game/TurnBasedJRPGTemplate/Blueprints/Battle/BP_BattleController.MoveToTarget` (`self.battleController`) (`/Game/TurnBasedJRPGTemplate/Blueprints/Units/BP_UnitBase.initialLocation` (`/Game/TurnBasedJRPGTemplate/Blueprints/Battle/BP_BattleController.currentAttackingUnit` (`self.battleController`))) (delegate `OnUnitMovedBackHandler`) false)
    (else
      (`self.OnSkillUsed` :!label _label_2))))

(event `OnUnitMovedBackHandler`
  (goto _label_2))

(fn `UserConstructionScript`
  (`parent.UserConstructionScript`))