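; First Aid skill for the turn-based JRPG battle system, healing the current target unit.
; It optionally moves the caster to the target, plays the skill animation, then moves it back afterward.
; The notify event briefly applies a heal overlay material, then heals, consuming a Gauze from inventory when available for a stronger effect.
; Both the delayed notify path, after refreshing combat UI, and the animation-end path call OnSkillUsed.
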(event `self.UseSkill`
  (if (`/Game/TurnBasedJRPGTemplate/Blueprints/Battle/BP_BattleController.shouldUnitsMoveToTarget` (`self.battleController`))
    (`/Game/TurnBasedJRPGTemplate/Blueprints/Battle/BP_BattleController.MoveToTarget` (`self.battleController`) (`SceneComponent.K2_GetComponentLocation` (`/Game/TurnBasedJRPGTemplate/Blueprints/Units/BP_UnitBase.AttackerLocation` (`/Game/TurnBasedJRPGTemplate/Blueprints/Battle/BP_BattleController.currentTargetUnit` (`self.battleController`)))) (delegate `OnUnitMovedToTargetHandler`) true)
    (else
      (`self.PlaySkillAnimation` :!label _label))))

(event `OnUnitMovedToTargetHandler`
  (goto _label))

(event `self.UseSkillOnNotify`
  (`MeshComponent.SetOverlayMaterial` (`/Game/TurnBasedJRPGTemplate/Blueprints/Units/BP_UnitBase.SkeletalMesh` (`/Game/TurnBasedJRPGTemplate/Blueprints/Battle/BP_BattleController.currentTargetUnit` (`self.battleController`))) "/Game/Effects/Materials/Heal_Material.Heal_Material")
  (`KismetSystemLibrary.Delay` 1.25)
  (`MeshComponent.SetOverlayMaterial` (`/Game/TurnBasedJRPGTemplate/Blueprints/Units/BP_UnitBase.SkeletalMesh` (`/Game/TurnBasedJRPGTemplate/Blueprints/Battle/BP_BattleController.currentTargetUnit` (`self.battleController`))) null)
  (if (>= (`BlueprintMapLibrary.Map_Find` (`/Game/TurnBasedJRPGTemplate/Blueprints/Controllers/BP_JRPGPlayerController.usableItems` (`self.jRPGPlayerController`)) "/Game/TurnBasedJRPGTemplate/Blueprints/Items/UsableItems/BP_Gauze.BP_Gauze_C") 1)
    (`/Game/TurnBasedJRPGTemplate/Blueprints/Controllers/BP_JRPGPlayerController.RemoveItemFromInventory` (`self.jRPGPlayerController`) "/Game/TurnBasedJRPGTemplate/Blueprints/Items/UsableItems/BP_Gauze.BP_Gauze_C" 1)
    (`/Game/TurnBasedJRPGTemplate/Blueprints/Units/BP_UnitBase.Heal` (`/Game/TurnBasedJRPGTemplate/Blueprints/Battle/BP_BattleController.currentTargetUnit` (`self.battleController`)) 50)
    (else
      (`/Game/TurnBasedJRPGTemplate/Blueprints/Units/BP_UnitBase.Heal` (`/Game/TurnBasedJRPGTemplate/Blueprints/Battle/BP_BattleController.currentTargetUnit` (`self.battleController`)) 25)))
  (`/Game/CommonUI/BattleUI/CWB_BattleUI.MidTurnInitEverything` (`self.CombatUIRef`))
  (`KismetSystemLibrary.Delay` 1.5)
  (`self.OnSkillUsed`))

(event `self.OnSkillAnimationEnded`
  (if (`/Game/TurnBasedJRPGTemplate/Blueprints/Battle/BP_BattleController.shouldUnitsMoveToTarget` (`self.battleController`))
    (`/Game/TurnBasedJRPGTemplate/Blueprints/Battle/BP_BattleController.MoveToTarget` (`self.battleController`) (`/Game/TurnBasedJRPGTemplate/Blueprints/Units/BP_UnitBase.initialLocation` (`/Game/TurnBasedJRPGTemplate/Blueprints/Battle/BP_BattleController.currentAttackingUnit` (`self.battleController`))) (delegate `OnUnitMovedBackHandler`) false)
    (else
      (`self.OnSkillUsed` :!label _label_2))))

(event `OnUnitMovedBackHandler`
  (goto _label_2))

(fn `UserConstructionScript`
  (`parent.UserConstructionScript`))