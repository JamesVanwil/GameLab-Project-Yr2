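; Player-controlled mage unit for the turn-based JRPG battles, treated as the main character whose death loses the fight.
; Its OnDied override waits briefly, strips equipment meshes, tells the battle controller the enemy won, switches to explore mode and destroys the actor.
; Projectiles spawn from the skeletal mesh's ProjectileSocket transform.
; The remaining event graph logic is disconnected test code for MP, HP and stat lookups.
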(event `self.ReceiveTick`
  (params (DeltaSeconds :type "Float (single-precision)")))

(event `self.ReceiveBeginPlay`
  (`parent.ReceiveBeginPlay`))

(event `self.OnDied`
  (bind _battlecontroller (`self.battleController`))
  ;[1 1 1] Override the event to finish the game when main character dies
  (`KismetSystemLibrary.Delay` 1.0)
  (`self.RemoveAllEquipmentMesh`)
  (`/Game/TurnBasedJRPGTemplate/Blueprints/Battle/BP_BattleController.EnemyWon` _battlecontroller)
  (`/Game/TurnBasedJRPGTemplate/Blueprints/Battle/BP_BattleController.SwitchToExploreMode` _battlecontroller)
  (`self.K2_DestroyActor`))

(fn `GetProjectileSpawnTransform`
  (returns (projectileSpawnTransform :type "Transform Structure"))
  (return (`SceneComponent.GetSocketTransform` (`self.SkeletalMesh`) "ProjectileSocket" "RTS_World")))

(fn `UserConstructionScript`
  (`parent.UserConstructionScript`))