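; Priest player unit for a turn-based JRPG that escalates its tarot equipment when MP runs out, then dies when it runs out again.
; Tick polls the unit's MP in the player controller's PlayerUnits map; the first depletion swaps in the Stage 2 Placida tarot, refills some MP and sets IsDreadful.
; While dreadful, a delayed check calls Die once MP is again zero, with DoOnce guarding both transitions.
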(event `self.ReceiveTick`
  (params (DeltaSeconds :type "Float (single-precision)"))
  (`self.DeactivateTarot1`)
  (if (`self.IsDreadful?`)
    (`self.DeacitvateTarot2`)))

(event `DeactivateTarot1`
  (bind _asbp_jrpgplayer_controller (cast `/Game/TurnBasedJRPGTemplate/Blueprints/Controllers/BP_JRPGPlayerController` (`GameplayStatics.GetPlayerController` 0)))
  (if (== (`.curentMP_6_79399572456CC89F79B2DA9F0A8BB445` (break `/Game/TurnBasedJRPGTemplate/Blueprints/Structs/S_PlayerUnitData` (`BlueprintMapLibrary.Map_Find` (`/Game/TurnBasedJRPGTemplate/Blueprints/Controllers/BP_JRPGPlayerController.playerUnits` _asbp_jrpgplayer_controller) "BP_PriestPlayerUnit_C"))) 0)
    (`/Engine/EditorBlueprintResources/StandardMacros.DoOnce` false
      (:`Completed`
        (`/Game/TurnBasedJRPGTemplate/Blueprints/Controllers/BP_JRPGPlayerController.RemoveEquipmentOnUnit` _asbp_jrpgplayer_controller null "NewEnumerator8")
        (`/Game/TurnBasedJRPGTemplate/Blueprints/Controllers/BP_JRPGPlayerController.WearEquipmentOnUnit` _asbp_jrpgplayer_controller "BP_PriestPlayerUnit_C" "/Game/TurnBasedJRPGTemplate/Blueprints/Items/Equipment/StatictTarot1/Placida/BP_StaticTarot1Stage2Placida.BP_StaticTarot1Stage2Placida_C")
        (bind _returnvalue (`GameplayStatics.GetActorOfClass` "BP_PriestPlayerUnit_C"))
        (`self.SetMP` _returnvalue 20)
        (set `self.IsDreadful?` true)))))

(event `DeacitvateTarot2`
  (`KismetSystemLibrary.Delay` 5.0)
  (bind _asbp_jrpgplayer_controller (cast `/Game/TurnBasedJRPGTemplate/Blueprints/Controllers/BP_JRPGPlayerController` (`GameplayStatics.GetPlayerController` 0)))
  (if (== (`.curentMP_6_79399572456CC89F79B2DA9F0A8BB445` (break `/Game/TurnBasedJRPGTemplate/Blueprints/Structs/S_PlayerUnitData` (`BlueprintMapLibrary.Map_Find` (`/Game/TurnBasedJRPGTemplate/Blueprints/Controllers/BP_JRPGPlayerController.playerUnits` _asbp_jrpgplayer_controller) "BP_PriestPlayerUnit_C"))) 0)
    (`/Engine/EditorBlueprintResources/StandardMacros.DoOnce` false
      (:`Completed`
        (`self.Die`)))))

(fn `UserConstructionScript`
  (`parent.UserConstructionScript`))