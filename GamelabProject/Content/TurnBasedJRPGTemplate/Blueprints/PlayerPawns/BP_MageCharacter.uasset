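; Player mage pawn that handles NPC interaction, a battery-powered flashlight, a bullet count and an orbit camera.
; InteractRadius overlaps track one BPI_Interactable, which F triggers, switching to UI input until ConversationClosed.
; Once picked up, the flashlight toggles on key 1 and drains through a self-calling Delay loop, with battery pickups and a debug refill.
; The wheel sets spring arm zoom, interpolated on Tick, and right-mouse drag rotates with clamped pitch.
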(event `Key|F`
  (params (Key :type "Key Structure"))
  ;[1 1 1] Player interact with NPC setup
  (:`Pressed`
    (`/Engine/EditorBlueprintResources/StandardMacros.IsValid` (`self.Interactable`)
      (:`Is Valid`
        (message `/Game/DialogueSystem/Blueprints/BPI_Interactable.Interact` (`self.Interactable`) self)
        (`WidgetBlueprintLibrary.SetInputMode_UIOnlyEx` (`GameplayStatics.GetPlayerController` 0) null)
        (set `PlayerController.bShowMouseCursor` true (`GameplayStatics.GetPlayerController` 0))))))

(event `self.InteractRadius.OnComponentBeginOverlap`
  (params (OverlappedComponent :type "PrimitiveComponent Object Reference") (OtherActor :type "Actor Object Reference") (OtherComp :type "PrimitiveComponent Object Reference") (OtherBodyIndex :type Integer) (bFromSweep :type Boolean) (SweepResult :type "HitResult Structure (by ref)"))
  ;[1 1 1] Player interact with NPC setup
  (`KismetSystemLibrary.PrintString` "sus")
  (if (!= OtherActor self)
    (if (`KismetSystemLibrary.DoesImplementInterface` OtherActor "/Game/DialogueSystem/Blueprints/BPI_Interactable.BPI_Interactable_C")
      (`/Engine/EditorBlueprintResources/StandardMacros.IsValid` (`self.Interactable`)
        (:`Is Valid`
          (message `/Game/DialogueSystem/Blueprints/BPI_Interactable.SetInteractableState` (`self.Interactable`) false)
          (set `self.Interactable` null))
        (:`Is Not Valid`
          _))
      (set `self.Interactable` OtherActor)
      (message `/Game/DialogueSystem/Blueprints/BPI_Interactable.SetInteractableState` (`self.Interactable`) true))))

(event `self.InteractRadius.OnComponentEndOverlap`
  (params (OverlappedComponent :type "PrimitiveComponent Object Reference") (OtherActor :type "Actor Object Reference") (OtherComp :type "PrimitiveComponent Object Reference") (OtherBodyIndex :type Integer))
  ;[1 1 1] Player interact with NPC setup
  (`KismetSystemLibrary.PrintString` "sussy")
  (if (and (!= OtherActor self) (== (`self.Interactable`) OtherActor))
    (message `/Game/DialogueSystem/Blueprints/BPI_Interactable.SetInteractableState` (`self.Interactable`) false)
    (set `self.Interactable` null)))

(event `/Game/DialogueSystem/Blueprints/BPI_Interactable.ConversationClosed`
  (bind _returnvalue (`GameplayStatics.GetPlayerController` 0))
  ;[1 1 1] Player interact with NPC setup
  (set `PlayerController.bShowMouseCursor` false _returnvalue)
  (`WidgetBlueprintLibrary.SetInputMode_GameOnly` _returnvalue))

(event `self.ReceiveBeginPlay`
  ;[1 1 1] Add UI Flashlight and Torch, door???
  (`SceneComponent.SetVisibility` (`self.FlashLight`) false false)
  (`SceneComponent.SetVisibility` (`self.TorchLight`) false false)
  (bind _returnvalue (`|CreateWidget` "/Game/WBP_InteractionsUI.WBP_InteractionsUI_C"))
  (`UserWidget.AddToViewport` _returnvalue 0))

(event `Key|Two`
  (params (Key :type "Key Structure"))
  ;[1 1 1] Torch Input
)

(event `Key|One`
  (params (Key :type "Key Structure"))
  ;[1 1 1] Input for flashlight and battery drain
  (:`Pressed`
    (if (`self.HasFlashlightBeenPickedUp`)
      (if (> (`self.FlashLightCharge`) 0.0)
        (`/Engine/EditorBlueprintResources/StandardMacros.FlipFlop`
          (:`A`
            (`SceneComponent.SetVisibility` (`self.FlashLight`) true false)
            (set `self.IsFlashlightActive` true)
            (`self.BatteryDrain`))
          (:`B`
            (`SceneComponent.SetVisibility` (`self.FlashLight`) false false :!label _label)
            (set `self.IsFlashlightActive` false)))))))

(event `FlashlightPickedUp`
  ;[1 1 1] Input for flashlight and battery drain
  (bind _returnvalue (`|CreateWidget` "/Game/BattleSystem/Blueprints/BP_HUDEnemy1_Battery.BP_HUDEnemy1_Battery_C" null null))
  (`UserWidget.AddToViewport` _returnvalue 0)
  (set `self.HasFlashlightBeenPickedUp` true))

(event `FlashUnequiped`
  ;[1 1 1] Input for flashlight and battery drain
  (`Widget.RemoveFromParent` (stale `FlashlightPickedUp` _returnvalue))
  (set `self.HasFlashlightBeenPickedUp` false))

(event `BatteryDrain`
  ;[1 1 1] Input for flashlight and battery drain
  (if (`self.IsFlashlightActive`)
    (bind _output_get (set `self.FlashLightCharge` (- (`self.FlashLightCharge`) 0.1)))
    (if (> _output_get 0.0)
      (`KismetSystemLibrary.Delay` 0.01)
      (`self.BatteryDrain`)
      (else
        (goto _label)))))

(event `BatteryPickUp`
  ;[1 1 1] Pick up battery
  (bind _output_get (set `self.FlashLightCharge` (+ (`self.FlashLightCharge`) 50)))
  (if (>= _output_get (`self.FlashLightMaxCharge`))
    (set `self.FlashLightCharge` (`self.FlashLightMaxCharge`))))

(event `InputAction|FlashlightRefill`
  (params (Key :type "Key Structure"))
  ;[1 1 1] Hacks
  (:`Pressed`
    (set `self.FlashLightCharge` 100.0)))

(event `InputAxisKey|MouseWheelAxis`
  (params (AxisValue :type "Float (single-precision)"))
  (bind _maxcameraposition (`self.maxCameraPosition`))
  (bind _maxcameraposition_2 (`self.maxCameraPosition`))
  ;[1 1 1] Camera Zoom in/out
  (if (> AxisValue 0.0)
    (bind _result (`/Engine/EditorBlueprintResources/StandardMacros.IncrementInt` (`self.cameraPosition`))
      (:`  `
        (set `self.cameraPosition` (`KismetMathLibrary.Clamp` _result (* _maxcameraposition -1) _maxcameraposition))))
    (elif (< AxisValue 0.0)
      (bind _result_2 (`/Engine/EditorBlueprintResources/StandardMacros.DecrementInt` (`self.cameraPosition`))
        (:`  `
          (set `self.cameraPosition` (`KismetMathLibrary.Clamp` _result_2 (* _maxcameraposition_2 -4) _maxcameraposition_2)))))))

(event `self.ReceiveTick`
  (params (DeltaSeconds :type "Float (single-precision)"))
  (bind _springarm (`self.SpringArm`))
  ;[1 1 1] Camera Zoom in/out
  (set `SpringArmComponent.TargetArmLength` (`KismetMathLibrary.FInterpTo` (`SpringArmComponent.TargetArmLength` _springarm) (+ (`self.defaultSpringArmLength`) (* (* (`self.cameraZoomDifference`) (`self.cameraPosition`)) -0.5)) DeltaSeconds 2.0) _springarm))

(event `InputAxis|LookYaw`
  (params (AxisValue :type "Float (single-precision)"))
  ;[1 1 1] Rotate Camera on RMB
  (if (`PlayerController.IsInputKeyDown` (`GameplayStatics.GetPlayerController` 0) "RightMouseButton")
    (`SceneComponent.K2_AddWorldRotation` (`self.SpringArm`) (`KismetMathLibrary.MakeRotator` 0.0 0.0 (* (`self.GetInputAxisValue`) (`self.CameraRotationMultiplier`))) false false)))

(event `InputAxis|LookPitch`
  (params (AxisValue :type "Float (single-precision)"))
  (bind _springarm (`self.SpringArm`))
  (bind (_relativerotation_roll _relativerotation_pitch _relativerotation_yaw) (`KismetMathLibrary.BreakRotator` (`SceneComponent.RelativeRotation` _springarm)))
  ;[1 1 1] Rotate Camera on RMB
  (if (`PlayerController.IsInputKeyDown` (`GameplayStatics.GetPlayerController` 0) "RightMouseButton")
    (`SceneComponent.K2_SetRelativeRotation` _springarm (`KismetMathLibrary.MakeRotator` _relativerotation_roll (`KismetMathLibrary.FClamp` (+ _relativerotation_pitch (* (`self.GetInputAxisValue`) (`self.CameraRotationMultiplier`))) -75.0 -40.0) _relativerotation_yaw) false false)))

(event `AddBulletsToInventory`
  ;[1 1 1] Add bullets to player
  (set `self.BulletAmount` (+ (`self.BulletAmount`) 6)))

(fn `GetInteractionInstigator`
  (returns (InteractionInstigator :type "Actor Object Reference"))
  (return null))

(fn `UserConstructionScript`
  (`parent.UserConstructionScript`))