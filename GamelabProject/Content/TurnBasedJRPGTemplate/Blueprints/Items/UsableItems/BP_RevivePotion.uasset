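; Usable revive potion that brings a player unit back with full HP and MP, in or out of battle.
; In battle, it respawns the unit at its saved death transform, re-registers it with the battle, and updates the unit list and turn order UI.
; Both paths write max stats into the player controller's unit map, the only change needed outside battle.
; Each then signals item use, delayed briefly in battle.
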(event `self.OnUsedInBattle`
  (params (unit :type "/Game/TurnBasedJRPGTemplate/Blueprints/Units/BP_UnitBase Object Reference") (unitClass :type "/Game/TurnBasedJRPGTemplate/Blueprints/Units/BP_UnitBase Class Reference"))
  (bind _battlecontroller (`self.battleController`))
  (bind _currentbattle (`/Game/TurnBasedJRPGTemplate/Blueprints/Battle/BP_BattleController.currentBattle` _battlecontroller))
  (bind _currentbattle_2 (`/Game/TurnBasedJRPGTemplate/Blueprints/Battle/BP_BattleController.currentBattle` (`self.battleController`)))
  ;[1 1 1] Revive unit in battle
  (bind _output_get (set `self.playerUnitClass` (castclass `/Game/TurnBasedJRPGTemplate/Blueprints/Units/PlayerUnits/BP_PlayerUnitBase` unitClass :!pure true)))
  (bind (_playerunitstats _level) (`/Game/TurnBasedJRPGTemplate/Blueprints/Controllers/BP_JRPGFunctionLibrary.GetPlayerUnitStatsFromData` _output_get (`BlueprintMapLibrary.Map_Find` (`/Game/TurnBasedJRPGTemplate/Blueprints/Controllers/BP_JRPGPlayerController.playerUnits` (`self.jRPGPlayerController`)) (`self.playerUnitClass`))))
  (bind _returnvalue (`|SpawnActorFromClass` (`self.playerUnitClass`) (`BlueprintMapLibrary.Map_Find` (`/Game/TurnBasedJRPGTemplate/Blueprints/Battle/BP_BattleBase.deadPlayerUnits` _currentbattle_2) (`self.playerUnitClass`)) "Undefined" "SelectDefaultAtRuntime" null _level _currentbattle_2 null))
  (`KismetArrayLibrary.Array_Add` (`/Game/TurnBasedJRPGTemplate/Blueprints/Battle/BP_BattleBase.playerUnits` _currentbattle_2) _returnvalue)
  (bind (_maxhp _maxmp) (break `/Game/TurnBasedJRPGTemplate/Blueprints/Structs/S_UnitStats` _playerunitstats))
  (bind _structout (setmembers `/Game/TurnBasedJRPGTemplate/Blueprints/Structs/S_PlayerUnitData` :`StructRef` (`BlueprintMapLibrary.Map_Find` (`/Game/TurnBasedJRPGTemplate/Blueprints/Controllers/BP_JRPGPlayerController.playerUnits` (`self.jRPGPlayerController`)) (`self.playerUnitClass`)) :`currentHP` _maxhp :`curentMP` _maxmp))
  (`BlueprintMapLibrary.Map_Add` (`/Game/TurnBasedJRPGTemplate/Blueprints/Controllers/BP_JRPGPlayerController.playerUnits` (`self.jRPGPlayerController`)) (`self.playerUnitClass`) _structout)
  (`/Game/TurnBasedJRPGTemplate/Blueprints/Battle/BP_BattleBase.InitPlayerUnit` _currentbattle _returnvalue)
  (`/Game/TurnBasedJRPGTemplate/Blueprints/UI/BP_PlayerUnitListUI.DisplayUnitUI` (`/Game/TurnBasedJRPGTemplate/Blueprints/UI/BP_BattleUI.BP_PlayerUnitListUI` (`/Game/TurnBasedJRPGTemplate/Blueprints/Battle/BP_BattleController.battleUI` _battlecontroller)) _returnvalue (`self.battleController`))
  (`BlueprintMapLibrary.Map_Remove` (`/Game/TurnBasedJRPGTemplate/Blueprints/Battle/BP_BattleBase.deadPlayerUnits` _currentbattle) (`self.playerUnitClass`))
  (`/Game/TurnBasedJRPGTemplate/Blueprints/UI/BP_TurnOrderList.SetRevivedUnit` (`/Game/TurnBasedJRPGTemplate/Blueprints/UI/BP_BattleUI.BP_TurnOrderList` (`/Game/TurnBasedJRPGTemplate/Blueprints/Battle/BP_BattleController.battleUI` (`self.battleController`))) _returnvalue)
  (`KismetSystemLibrary.Delay` 1.5)
  (`self.OnItemUsed`))

(event `self.OnUsedOutsideBattle`
  (params (playerUnit :type "/Game/TurnBasedJRPGTemplate/Blueprints/Units/PlayerUnits/BP_PlayerUnitBase Class Reference"))
  (bind _value (`BlueprintMapLibrary.Map_Find` (`/Game/TurnBasedJRPGTemplate/Blueprints/Controllers/BP_JRPGPlayerController.playerUnits` (`self.jRPGPlayerController`)) playerUnit))
  ;[1 1 1] Revive unit outside battle
  (bind _playerunitstats (`/Game/TurnBasedJRPGTemplate/Blueprints/Controllers/BP_JRPGFunctionLibrary.GetPlayerUnitStatsFromData` playerUnit _value))
  (bind ((`maxHP_2_41B41BC24C39ED8CDC0C58B3398B651D` _maxhp) (`maxMP_4_402F570E47A131E33E462B9D0D778331` _maxmp)) (break `/Game/TurnBasedJRPGTemplate/Blueprints/Structs/S_UnitStats` _playerunitstats))
  (bind _structout (setmembers `/Game/TurnBasedJRPGTemplate/Blueprints/Structs/S_PlayerUnitData` :`StructRef` _value :`currentHP` _maxhp :`curentMP` _maxmp))
  (`BlueprintMapLibrary.Map_Add` (`/Game/TurnBasedJRPGTemplate/Blueprints/Controllers/BP_JRPGPlayerController.playerUnits` (`self.jRPGPlayerController`)) playerUnit _structout)
  (`self.OnItemUsed`))

(fn `UserConstructionScript`
  (`parent.UserConstructionScript`))