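; Blueprint for the Mage's Static Tarot 2 equipment item in the turn-based JRPG template, apparently an unfinished stub.
; Its activation and deactivation events are empty, and the construction script only calls the parent.
; Two disconnected, never-executed chains read Mage unit stats and set scaled attack and speed values on class-default structs, so the graph applies no stat change.
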(event `StaticTarot2Mage`
  ;[1 1 1] Static Tarot 2
)

(event `DeactivationStaticTarot2`
  ;[1 1 1] Deactivation of Static Tarot 2
)

(fn `UserConstructionScript`
  (`parent.UserConstructionScript`))