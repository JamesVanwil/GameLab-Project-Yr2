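; Buff Blueprint for the stage 2 Roland static tarot in socket 2, trading MaxMP against ActionTime on player units.
; ApplyBuff loops over the controller's PlayerUnits keys, always testing the Mage unit's socket, and sets stats on each key's class-default struct to lower MaxMP and raise ActionTime.
; OnBuffEnded repeats this, restoring MaxMP but raising ActionTime again rather than reversing it.
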(event `self.ApplyBuff`
  ;[1 1 1] Apply Tarot 1 Buff
  (bind _asbp_jrpgplayer_controller (cast `/Game/TurnBasedJRPGTemplate/Blueprints/Controllers/BP_JRPGPlayerController` (`GameplayStatics.GetPlayerController` 0)))
  (bind _playerunits (`/Game/TurnBasedJRPGTemplate/Blueprints/Controllers/BP_JRPGPlayerController.playerUnits` _asbp_jrpgplayer_controller))
  (bind _keys (`BlueprintMapLibrary.Map_Keys` _playerunits))
  (for _array_element _keys
    (if (== (`.StaticTarotSocket2_52_C805DEBE4D5F6DCAF20172BE33318FDF` (break `/Game/TurnBasedJRPGTemplate/Blueprints/Structs/S_PlayerUnitData` (`BlueprintMapLibrary.Map_Find` _playerunits "/Game/TurnBasedJRPGTemplate/Blueprints/Units/PlayerUnits/BP_MagePlayerUnit.BP_MagePlayerUnit_C"))) "/Game/TurnBasedJRPGTemplate/Blueprints/Items/Equipment/StaticTarot2/Roland/BP_StatictTarot2Stage2Roland.BP_StatictTarot2Stage2Roland_C")
      (bind _firstlevelstats (defaults `Object` _array_element))
      (bind ((`maxMP_4_402F570E47A131E33E462B9D0D778331` _maxmp) (`actionTime_31_CD6B6FA04FF3CB1C1BA72A93110B7A28` _actiontime)) (break `/Game/TurnBasedJRPGTemplate/Blueprints/Structs/S_UnitStats` _firstlevelstats))
      (setmembers `/Game/TurnBasedJRPGTemplate/Blueprints/Structs/S_UnitStats` :`StructRef` _firstlevelstats :`maxMP` (- _maxmp 5) :`actionTime` (+ _actiontime 0.4)))))

(event `self.OnBuffEnded`
  ;[1 1 1] Remove Tarot 1 buff
  (bind _asbp_jrpgplayer_controller (cast `/Game/TurnBasedJRPGTemplate/Blueprints/Controllers/BP_JRPGPlayerController` (`GameplayStatics.GetPlayerController` 0)))
  (bind _playerunits (`/Game/TurnBasedJRPGTemplate/Blueprints/Controllers/BP_JRPGPlayerController.playerUnits` _asbp_jrpgplayer_controller))
  (bind _keys (`BlueprintMapLibrary.Map_Keys` _playerunits))
  (for _array_element _keys
    (if (== (`.StaticTarotSocket2_52_C805DEBE4D5F6DCAF20172BE33318FDF` (break `/Game/TurnBasedJRPGTemplate/Blueprints/Structs/S_PlayerUnitData` (`BlueprintMapLibrary.Map_Find` _playerunits "/Game/TurnBasedJRPGTemplate/Blueprints/Units/PlayerUnits/BP_MagePlayerUnit.BP_MagePlayerUnit_C"))) "/Game/TurnBasedJRPGTemplate/Blueprints/Items/Equipment/StaticTarot2/Roland/BP_StatictTarot2Stage2Roland.BP_StatictTarot2Stage2Roland_C")
      (bind _firstlevelstats (defaults `Object` _array_element))
      (bind ((`maxMP_4_402F570E47A131E33E462B9D0D778331` _maxmp) (`actionTime_31_CD6B6FA04FF3CB1C1BA72A93110B7A28` _actiontime)) (break `/Game/TurnBasedJRPGTemplate/Blueprints/Structs/S_UnitStats` _firstlevelstats))
      (setmembers `/Game/TurnBasedJRPGTemplate/Blueprints/Structs/S_UnitStats` :`StructRef` _firstlevelstats :`maxMP` (+ _maxmp 5) :`actionTime` (+ _actiontime 0.4)))))

(fn `UserConstructionScript`
  (`parent.UserConstructionScript`))