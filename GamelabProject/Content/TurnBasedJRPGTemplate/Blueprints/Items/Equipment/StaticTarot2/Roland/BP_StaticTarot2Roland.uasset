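; Roland's second static Tarot equipment item in its first stage, which swaps itself for the stage 2 version when the mage runs out of MP.
; Every Tick it reads the mage unit's current MP from the JRPG player controller's PlayerUnits map.
; At zero MP, a DoOnce prints a deactivation message, removes the equipment by slot type and equips the stage 2 Tarot on the mage.
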(event `self.ReceiveTick`
  (params (DeltaSeconds :type "Float (single-precision)"))
  (bind _asbp_jrpgplayer_controller (cast `/Game/TurnBasedJRPGTemplate/Blueprints/Controllers/BP_JRPGPlayerController` (`GameplayStatics.GetPlayerController` 0)))
  (if (== (`.curentMP_6_79399572456CC89F79B2DA9F0A8BB445` (break `/Game/TurnBasedJRPGTemplate/Blueprints/Structs/S_PlayerUnitData` (`BlueprintMapLibrary.Map_Find` (`/Game/TurnBasedJRPGTemplate/Blueprints/Controllers/BP_JRPGPlayerController.playerUnits` _asbp_jrpgplayer_controller) "/Game/TurnBasedJRPGTemplate/Blueprints/Units/PlayerUnits/BP_MagePlayerUnit.BP_MagePlayerUnit_C"))) 0)
    (`/Engine/EditorBlueprintResources/StandardMacros.DoOnce` false
      (:`Completed`
        (`KismetSystemLibrary.PrintString` "Tarot 2 stage 1 has been deactivated")
        (`/Game/TurnBasedJRPGTemplate/Blueprints/Controllers/BP_JRPGPlayerController.RemoveEquipmentOnUnit` _asbp_jrpgplayer_controller null "NewEnumerator9")
        (`/Game/TurnBasedJRPGTemplate/Blueprints/Controllers/BP_JRPGPlayerController.WearEquipmentOnUnit` _asbp_jrpgplayer_controller "/Game/TurnBasedJRPGTemplate/Blueprints/Units/PlayerUnits/BP_MagePlayerUnit.BP_MagePlayerUnit_C" "/Game/TurnBasedJRPGTemplate/Blueprints/Items/Equipment/StaticTarot2/Roland/BP_StatictTarot2Stage2Roland.BP_StatictTarot2Stage2Roland_C")))))

(fn `UserConstructionScript`
  (`parent.UserConstructionScript`))