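; Stage 1 of Harper's static Tarot 2 equipment, which swaps itself for stage 2 when the archer runs out of MP.
; Tick polls the archer unit's MP through the player controller and, once at zero, removes the equipped item and equips the Stage 2 Blueprint.
; BeginPlay applies MaxHP and Defense penalties to a struct from the priest's class defaults, not the archer's, with no visible write-back.
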(event `self.ReceiveTick`
  (params (DeltaSeconds :type "Float (single-precision)"))
  (bind _asbp_jrpgplayer_controller (cast `/Game/TurnBasedJRPGTemplate/Blueprints/Controllers/BP_JRPGPlayerController` (`GameplayStatics.GetPlayerController` 0)))
  (if (== (`.curentMP_6_79399572456CC89F79B2DA9F0A8BB445` (break `/Game/TurnBasedJRPGTemplate/Blueprints/Structs/S_PlayerUnitData` (`BlueprintMapLibrary.Map_Find` (`/Game/TurnBasedJRPGTemplate/Blueprints/Controllers/BP_JRPGPlayerController.playerUnits` _asbp_jrpgplayer_controller) "/Game/TurnBasedJRPGTemplate/Blueprints/Units/PlayerUnits/BP_ArcherPlayerUnit.BP_ArcherPlayerUnit_C"))) 0)
    (`/Engine/EditorBlueprintResources/StandardMacros.DoOnce` false
      (:`Completed`
        (`KismetSystemLibrary.PrintString` "Tarot 2 stage 1 has been deactivated")
        (`/Game/TurnBasedJRPGTemplate/Blueprints/Controllers/BP_JRPGPlayerController.RemoveEquipmentOnUnit` _asbp_jrpgplayer_controller null "NewEnumerator9")
        (`/Game/TurnBasedJRPGTemplate/Blueprints/Controllers/BP_JRPGPlayerController.WearEquipmentOnUnit` _asbp_jrpgplayer_controller "/Game/TurnBasedJRPGTemplate/Blueprints/Units/PlayerUnits/BP_ArcherPlayerUnit.BP_ArcherPlayerUnit_C" "/Game/TurnBasedJRPGTemplate/Blueprints/Items/Equipment/StaticTarot2/Harper/BP_StaticTarot2Stage2Harperr.BP_StaticTarot2Stage2Harperr_C")))))

(event `self.ReceiveBeginPlay`
  (bind _firstlevelstats (defaults `/Game/TurnBasedJRPGTemplate/Blueprints/Units/PlayerUnits/BP_PriestPlayerUnit` "/Game/TurnBasedJRPGTemplate/Blueprints/Units/PlayerUnits/BP_PriestPlayerUnit.BP_PriestPlayerUnit_C"))
  (bind ((`maxHP_2_41B41BC24C39ED8CDC0C58B3398B651D` _maxhp) (`defense_16_FEA01B2E4A985F64F6B9359A13E3F651` _defense)) (break `/Game/TurnBasedJRPGTemplate/Blueprints/Structs/S_UnitStats` _firstlevelstats))
  (`parent.ReceiveBeginPlay`)
  (setmembers `/Game/TurnBasedJRPGTemplate/Blueprints/Structs/S_UnitStats` :`StructRef` _firstlevelstats :`maxHP` (- _maxhp 5) :`defense` (- _defense 2)))

(fn `UserConstructionScript`
  (`parent.UserConstructionScript`))