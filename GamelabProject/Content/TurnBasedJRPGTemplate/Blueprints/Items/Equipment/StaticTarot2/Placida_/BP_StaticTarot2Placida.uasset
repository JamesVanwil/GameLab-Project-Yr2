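; BP_StaticTarot2Placida is a tarot equipment item that changes to its second-stage version when the Priest runs out of MP.
; Each Tick looks up the Priest in the JRPG player controller's PlayerUnits and checks whether current MP is zero.
; A DoOnce then removes equipment of one slot type through the controller and equips BP_StaticTarot2Stage2Placida on the Priest.
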(event `self.ReceiveTick`
  (params (DeltaSeconds :type "Float (single-precision)"))
  (bind _asbp_jrpgplayer_controller (cast `/Game/TurnBasedJRPGTemplate/Blueprints/Controllers/BP_JRPGPlayerController` (`GameplayStatics.GetPlayerController` 0)))
  (if (== (`.curentMP_6_79399572456CC89F79B2DA9F0A8BB445` (break `/Game/TurnBasedJRPGTemplate/Blueprints/Structs/S_PlayerUnitData` (`BlueprintMapLibrary.Map_Find` (`/Game/TurnBasedJRPGTemplate/Blueprints/Controllers/BP_JRPGPlayerController.playerUnits` _asbp_jrpgplayer_controller) "/Game/TurnBasedJRPGTemplate/Blueprints/Units/PlayerUnits/BP_PriestPlayerUnit.BP_PriestPlayerUnit_C"))) 0)
    (`/Engine/EditorBlueprintResources/StandardMacros.DoOnce` false
      (:`Completed`
        (`/Game/TurnBasedJRPGTemplate/Blueprints/Controllers/BP_JRPGPlayerController.RemoveEquipmentOnUnit` _asbp_jrpgplayer_controller null "NewEnumerator9")
        (`/Game/TurnBasedJRPGTemplate/Blueprints/Controllers/BP_JRPGPlayerController.WearEquipmentOnUnit` _asbp_jrpgplayer_controller "/Game/TurnBasedJRPGTemplate/Blueprints/Units/PlayerUnits/BP_PriestPlayerUnit.BP_PriestPlayerUnit_C" "/Game/TurnBasedJRPGTemplate/Blueprints/Items/Equipment/StaticTarot2/Placida_/BP_StaticTarot2Stage2Placida.BP_StaticTarot2Stage2Placida_C")))))

(fn `UserConstructionScript`
  (`parent.UserConstructionScript`))