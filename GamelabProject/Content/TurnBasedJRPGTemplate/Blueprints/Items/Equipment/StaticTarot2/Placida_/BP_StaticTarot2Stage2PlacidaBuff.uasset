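; Buff for the stage 2 Placida static tarot that, despite its name, lowers attack and defense stats while active.
; ApplyBuff loops over the player controller's unit classes, checking each pass whether the Priest's second static tarot socket holds this tarot.
; If so, it subtracts fixed amounts from min/max attack, defense and magic defense on structs read from class defaults, with no explicit write-back.
; OnBuffEnded mirrors this, adding the same amounts.
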(event `self.ApplyBuff`
  ;[1 1 1] Apply Tarot 1 Buff
  (bind _asbp_jrpgplayer_controller (cast `/Game/TurnBasedJRPGTemplate/Blueprints/Controllers/BP_JRPGPlayerController` (`GameplayStatics.GetPlayerController` 0)))
  (bind _playerunits (`/Game/TurnBasedJRPGTemplate/Blueprints/Controllers/BP_JRPGPlayerController.playerUnits` _asbp_jrpgplayer_controller))
  (bind _keys (`BlueprintMapLibrary.Map_Keys` _playerunits))
  (for _array_element _keys
    (if (== (`.StaticTarotSocket2_52_C805DEBE4D5F6DCAF20172BE33318FDF` (break `/Game/TurnBasedJRPGTemplate/Blueprints/Structs/S_PlayerUnitData` (`BlueprintMapLibrary.Map_Find` _playerunits "/Game/TurnBasedJRPGTemplate/Blueprints/Units/PlayerUnits/BP_PriestPlayerUnit.BP_PriestPlayerUnit_C"))) "/Game/TurnBasedJRPGTemplate/Blueprints/Items/Equipment/StaticTarot2/Placida_/BP_StaticTarot2Stage2Placida.BP_StaticTarot2Stage2Placida_C")
      (bind _firstlevelstats (defaults `Object` _array_element))
      (bind ((`minAttack_14_0D64A0224152A597434ECDAF6DFC9964` _minattack) (`maxAttack_15_24D8527844E2DFB657716C9F16A4AE21` _maxattack) (`defense_16_FEA01B2E4A985F64F6B9359A13E3F651` _defense) (`magicDefense_25_FE826AEB41C90F001AB72DA466AF2D63` _magicdefense)) (break `/Game/TurnBasedJRPGTemplate/Blueprints/Structs/S_UnitStats` _firstlevelstats))
      (setmembers `/Game/TurnBasedJRPGTemplate/Blueprints/Structs/S_UnitStats` :`StructRef` _firstlevelstats :`minAttack` (- _minattack 5) :`maxAttack` (- _maxattack 5) :`defense` (- _defense 3) :`magicDefense` (- _magicdefense 3)))))

(event `self.OnBuffEnded`
  ;[1 1 1] Remove Tarot 1 buff
  (bind _asbp_jrpgplayer_controller (cast `/Game/TurnBasedJRPGTemplate/Blueprints/Controllers/BP_JRPGPlayerController` (`GameplayStatics.GetPlayerController` 0)))
  (bind _playerunits (`/Game/TurnBasedJRPGTemplate/Blueprints/Controllers/BP_JRPGPlayerController.playerUnits` _asbp_jrpgplayer_controller))
  (bind _keys (`BlueprintMapLibrary.Map_Keys` _playerunits))
  (for _array_element _keys
    (if (== (`.StaticTarotSocket2_52_C805DEBE4D5F6DCAF20172BE33318FDF` (break `/Game/TurnBasedJRPGTemplate/Blueprints/Structs/S_PlayerUnitData` (`BlueprintMapLibrary.Map_Find` _playerunits "/Game/TurnBasedJRPGTemplate/Blueprints/Units/PlayerUnits/BP_PriestPlayerUnit.BP_PriestPlayerUnit_C"))) "/Game/TurnBasedJRPGTemplate/Blueprints/Items/Equipment/StaticTarot2/Placida_/BP_StaticTarot2Stage2Placida.BP_StaticTarot2Stage2Placida_C")
      (bind _firstlevelstats (defaults `Object` _array_element))
      (bind ((`minAttack_14_0D64A0224152A597434ECDAF6DFC9964` _minattack) (`maxAttack_15_24D8527844E2DFB657716C9F16A4AE21` _maxattack) (`defense_16_FEA01B2E4A985F64F6B9359A13E3F651` _defense) (`magicDefense_25_FE826AEB41C90F001AB72DA466AF2D63` _magicdefense)) (break `/Game/TurnBasedJRPGTemplate/Blueprints/Structs/S_UnitStats` _firstlevelstats))
      (setmembers `/Game/TurnBasedJRPGTemplate/Blueprints/Structs/S_UnitStats` :`StructRef` _firstlevelstats :`minAttack` (+ _minattack 5) :`maxAttack` (+ _maxattack 5) :`defense` (+ _defense 3) :`magicDefense` (+ _magicdefense 3)))))

(fn `UserConstructionScript`
  (`parent.UserConstructionScript`))