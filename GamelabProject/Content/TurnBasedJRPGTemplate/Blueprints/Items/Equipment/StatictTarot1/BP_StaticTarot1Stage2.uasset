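; Stage 2 of the StaticTarot1 equipment item, which makes the battle a loss once the Mage runs out of MP.
; Tick reads the Mage unit's current MP from the JRPG player controller and, at zero, calls EnemyWon once on the battle controller and destroys the player character.
; Separate add and remove stat events both apply the same MaxAttack increase to BP_StaticTarot1Mage class-default values, so removal does not subtract it.
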(event `self.ReceiveTick`
  (params (DeltaSeconds :type "Float (single-precision)"))
  (bind _asbp_jrpgplayer_controller (cast `/Game/TurnBasedJRPGTemplate/Blueprints/Controllers/BP_JRPGPlayerController` (`GameplayStatics.GetPlayerController` 0)))
  (if (== (`.curentMP_6_79399572456CC89F79B2DA9F0A8BB445` (break `/Game/TurnBasedJRPGTemplate/Blueprints/Structs/S_PlayerUnitData` (`BlueprintMapLibrary.Map_Find` (`/Game/TurnBasedJRPGTemplate/Blueprints/Controllers/BP_JRPGPlayerController.playerUnits` _asbp_jrpgplayer_controller) "/Game/TurnBasedJRPGTemplate/Blueprints/Units/PlayerUnits/BP_MagePlayerUnit.BP_MagePlayerUnit_C"))) 0)
    (`/Engine/EditorBlueprintResources/StandardMacros.DoOnce` false
      (:`Completed`
        (bind _returnvalue (`GameplayStatics.GetActorOfClass` "/Game/TurnBasedJRPGTemplate/Blueprints/Battle/BP_BattleController.BP_BattleController_C"))
        (`/Game/TurnBasedJRPGTemplate/Blueprints/Battle/BP_BattleController.EnemyWon` _returnvalue)
        (`self.K2_DestroyActor` (`GameplayStatics.GetPlayerCharacter` 0))))))

(event `RemoveStaticTarot2Stats`
  (bind _stats (defaults `/Game/TurnBasedJRPGTemplate/Blueprints/Items/Equipment/StatictTarot1/BP_StaticTarot1Mage` "/Game/TurnBasedJRPGTemplate/Blueprints/Items/Equipment/StatictTarot1/BP_StaticTarot1Mage.BP_StaticTarot1Mage_C"))
  (setmembers `/Game/TurnBasedJRPGTemplate/Blueprints/Structs/S_UnitStats` :`StructRef` _stats :`maxAttack` (+ (`.maxAttack_15_24D8527844E2DFB657716C9F16A4AE21` (break `/Game/TurnBasedJRPGTemplate/Blueprints/Structs/S_UnitStats` _stats)) 15)))

(event `AddStatucTarot2Stats`
  (bind _stats (defaults `/Game/TurnBasedJRPGTemplate/Blueprints/Items/Equipment/StatictTarot1/BP_StaticTarot1Mage` "/Game/TurnBasedJRPGTemplate/Blueprints/Items/Equipment/StatictTarot1/BP_StaticTarot1Mage.BP_StaticTarot1Mage_C"))
  (setmembers `/Game/TurnBasedJRPGTemplate/Blueprints/Structs/S_UnitStats` :`StructRef` _stats :`maxAttack` (+ (`.maxAttack_15_24D8527844E2DFB657716C9F16A4AE21` (break `/Game/TurnBasedJRPGTemplate/Blueprints/Structs/S_UnitStats` _stats)) 15)))

(fn `UserConstructionScript`
  (`parent.UserConstructionScript`))