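; Roland's first static tarot buff for the turn-based JRPG, which adjusts player units' minimum and maximum attack by a flat amount.
; ApplyBuff loops the controller's PlayerUnits keys and raises attack on each class-default stats struct if BP_MagePlayerUnit is present.
; OnBuffEnded lowers it only if that mage entry has this tarot in socket one and a Winchester or Revolver as weapon or armor.
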(event `self.ApplyBuff`
  ;[1 1 1] Apply Tarot 1 Buff
  (bind _asbp_jrpgplayer_controller (cast `/Game/TurnBasedJRPGTemplate/Blueprints/Controllers/BP_JRPGPlayerController` (`GameplayStatics.GetPlayerController` 0)))
  (bind _playerunits (`/Game/TurnBasedJRPGTemplate/Blueprints/Controllers/BP_JRPGPlayerController.playerUnits` _asbp_jrpgplayer_controller))
  (bind _keys (`BlueprintMapLibrary.Map_Keys` _playerunits))
  (for _array_element _keys
    (if (`.ReturnValue` (`BlueprintMapLibrary.Map_Find` _playerunits "/Game/TurnBasedJRPGTemplate/Blueprints/Units/PlayerUnits/BP_MagePlayerUnit.BP_MagePlayerUnit_C"))
      (bind _firstlevelstats (defaults `Object` _array_element))
      (bind ((`minAttack_14_0D64A0224152A597434ECDAF6DFC9964` _minattack) (`maxAttack_15_24D8527844E2DFB657716C9F16A4AE21` _maxattack)) (break `/Game/TurnBasedJRPGTemplate/Blueprints/Structs/S_UnitStats` _firstlevelstats))
      (setmembers `/Game/TurnBasedJRPGTemplate/Blueprints/Structs/S_UnitStats` :`StructRef` _firstlevelstats :`minAttack` (+ _minattack 3) :`maxAttack` (+ _maxattack 3)))))

(event `self.OnBuffEnded`
  ;[1 1 1] Remove Tarot 1 buff
  (bind _asbp_jrpgplayer_controller (cast `/Game/TurnBasedJRPGTemplate/Blueprints/Controllers/BP_JRPGPlayerController` (`GameplayStatics.GetPlayerController` 0)))
  (bind _playerunits (`/Game/TurnBasedJRPGTemplate/Blueprints/Controllers/BP_JRPGPlayerController.playerUnits` _asbp_jrpgplayer_controller))
  (bind _keys (`BlueprintMapLibrary.Map_Keys` _playerunits))
  (for _array_element _keys
    (bind ((`Weapon_19_25C66CFA4AEC9B2EB46636BA5392040B` _weapon) (`Armor_20_3FACB90A4F7AB732B976FDBD9DF85285` _armor) (`StaticTarotSocket1_49_386CDF41496C8A1A94652D804435853A` _statictarotsocket1)) (break `/Game/TurnBasedJRPGTemplate/Blueprints/Structs/S_PlayerUnitData` (`BlueprintMapLibrary.Map_Find` _playerunits "/Game/TurnBasedJRPGTemplate/Blueprints/Units/PlayerUnits/BP_MagePlayerUnit.BP_MagePlayerUnit_C")))
    (if (== _statictarotsocket1 "/Game/TurnBasedJRPGTemplate/Blueprints/Items/Equipment/StatictTarot1/Roland/BP_StaticTarot1Roland.BP_StaticTarot1Roland_C")
      (if (or (or (== _weapon "/Game/TurnBasedJRPGTemplate/Blueprints/Items/Equipment/Weapons/BP_WinchesterWeapon.BP_WinchesterWeapon_C") (== _weapon "/Game/TurnBasedJRPGTemplate/Blueprints/Items/Equipment/Weapons/BP_Revolver.BP_Revolver_C")) (or (== _armor "/Game/TurnBasedJRPGTemplate/Blueprints/Items/Equipment/Weapons/BP_WinchesterWeapon.BP_WinchesterWeapon_C") (== _armor "/Game/TurnBasedJRPGTemplate/Blueprints/Items/Equipment/Weapons/BP_Revolver.BP_Revolver_C")))
        (bind _firstlevelstats (defaults `Object` _array_element))
        (bind ((`minAttack_14_0D64A0224152A597434ECDAF6DFC9964` _minattack) (`maxAttack_15_24D8527844E2DFB657716C9F16A4AE21` _maxattack)) (break `/Game/TurnBasedJRPGTemplate/Blueprints/Structs/S_UnitStats` _firstlevelstats))
        (setmembers `/Game/TurnBasedJRPGTemplate/Blueprints/Structs/S_UnitStats` :`StructRef` _firstlevelstats :`minAttack` (- _minattack 3) :`maxAttack` (- _maxattack 3))))))

(fn `UserConstructionScript`
  (`parent.UserConstructionScript`))