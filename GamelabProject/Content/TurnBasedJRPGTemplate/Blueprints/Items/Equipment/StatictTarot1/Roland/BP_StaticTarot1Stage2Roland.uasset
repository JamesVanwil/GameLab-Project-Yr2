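; Stage 2 Blueprint of Roland's first static tarot equipment item in the turn-based JRPG template, meant to adjust his unit stats.
; Add and remove events read the BP_StaticTarot1Roland class defaults and set MaxAttack to that value plus a flat bonus.
; Both events add the bonus, so removal does not subtract it, and neither stores the modified struct.
; The construction script only calls its parent.
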(event `RemoveStaticTarot2Stats`
  (bind _stats (defaults `/Game/TurnBasedJRPGTemplate/Blueprints/Items/Equipment/StatictTarot1/Roland/BP_StaticTarot1Roland` "/Game/TurnBasedJRPGTemplate/Blueprints/Items/Equipment/StatictTarot1/Roland/BP_StaticTarot1Roland.BP_StaticTarot1Roland_C"))
  (setmembers `/Game/TurnBasedJRPGTemplate/Blueprints/Structs/S_UnitStats` :`StructRef` _stats :`maxAttack` (+ (`.maxAttack_15_24D8527844E2DFB657716C9F16A4AE21` (break `/Game/TurnBasedJRPGTemplate/Blueprints/Structs/S_UnitStats` _stats)) 15)))

(event `AddStatucTarot2Stats`
  (bind _stats (defaults `/Game/TurnBasedJRPGTemplate/Blueprints/Items/Equipment/StatictTarot1/Roland/BP_StaticTarot1Roland` "/Game/TurnBasedJRPGTemplate/Blueprints/Items/Equipment/StatictTarot1/Roland/BP_StaticTarot1Roland.BP_StaticTarot1Roland_C"))
  (setmembers `/Game/TurnBasedJRPGTemplate/Blueprints/Structs/S_UnitStats` :`StructRef` _stats :`maxAttack` (+ (`.maxAttack_15_24D8527844E2DFB657716C9F16A4AE21` (break `/Game/TurnBasedJRPGTemplate/Blueprints/Structs/S_UnitStats` _stats)) 15)))

(fn `UserConstructionScript`
  (`parent.UserConstructionScript`))