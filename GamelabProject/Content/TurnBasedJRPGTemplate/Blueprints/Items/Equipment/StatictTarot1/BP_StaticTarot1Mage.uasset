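; BP_StaticTarot1Mage is an unfinished tarot equipment item for the Mage in the JRPG template.
; BeginPlay sets a fixed MaxHP on stats read from BP_MagePlayerUnit's class defaults, not a live unit.
; An unconnected MP check would toggle activation and deactivation events, both empty.
; A name-switch event picks "The Sun" or "The Moon", but its only call is unreachable, as are older percentage-based HP changes.
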(event `self.ReceiveBeginPlay`
  (`parent.ReceiveBeginPlay`)
  (setmembers `/Game/TurnBasedJRPGTemplate/Blueprints/Structs/S_UnitStats` :`StructRef` (defaults `/Game/TurnBasedJRPGTemplate/Blueprints/Units/PlayerUnits/BP_MagePlayerUnit` "/Game/TurnBasedJRPGTemplate/Blueprints/Units/PlayerUnits/BP_MagePlayerUnit.BP_MagePlayerUnit_C") :`maxHP` 130))

(event `self.ReceiveTick`
  (params (DeltaSeconds :type "Float (single-precision)")))

(event `StaticTarot1Mage`
  ;[1 1 1] Static Tarot 1
)

(event `DeactivationStaticTarot`
  ;[1 1 1] Deactivation of Static Tarot 1
)

(event `ChangeStaticTarot1NameBasedOnMP`
  (if (== (defaults `/Game/TurnBasedJRPGTemplate/Blueprints/Units/PlayerUnits/BP_MagePlayerUnit` "/Game/TurnBasedJRPGTemplate/Blueprints/Units/PlayerUnits/BP_MagePlayerUnit.BP_MagePlayerUnit_C") 0)
    (bind _output_get (set `self.name` "The Moon"))
    (else
      (bind _output_get_2 (set `self.name` "The Sun")))))

(fn `UserConstructionScript`
  (`parent.UserConstructionScript`))