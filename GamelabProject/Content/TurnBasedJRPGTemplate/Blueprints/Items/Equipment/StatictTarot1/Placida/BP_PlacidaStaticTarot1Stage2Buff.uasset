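; Stage 2 buff for Placida's first static tarot, granting a flat MaxAttack bonus tied to the Priest's equipment.
; ApplyBuff loops the controller's PlayerUnits, adding the bonus to each unit class's default stats struct.
; Every iteration checks only the Priest's entry: Placida tarot in socket 1, plus Axe or KitchenKnife as Weapon or Armor.
; OnBuffEnded repeats that check before subtracting the same amount.
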(event `self.ApplyBuff`
  ;[1 1 1] Apply Tarot 1 Buff
  (bind _asbp_jrpgplayer_controller (cast `/Game/TurnBasedJRPGTemplate/Blueprints/Controllers/BP_JRPGPlayerController` (`GameplayStatics.GetPlayerController` 0)))
  (bind _playerunits (`/Game/TurnBasedJRPGTemplate/Blueprints/Controllers/BP_JRPGPlayerController.playerUnits` _asbp_jrpgplayer_controller))
  (bind _keys (`BlueprintMapLibrary.Map_Keys` _playerunits))
  (for _array_element _keys
    (bind ((`Weapon_19_25C66CFA4AEC9B2EB46636BA5392040B` _weapon) (`Armor_20_3FACB90A4F7AB732B976FDBD9DF85285` _armor) (`StaticTarotSocket1_49_386CDF41496C8A1A94652D804435853A` _statictarotsocket1)) (break `/Game/TurnBasedJRPGTemplate/Blueprints/Structs/S_PlayerUnitData` (`BlueprintMapLibrary.Map_Find` _playerunits "/Game/TurnBasedJRPGTemplate/Blueprints/Units/PlayerUnits/BP_PriestPlayerUnit.BP_PriestPlayerUnit_C")))
    (if (== _statictarotsocket1 "/Game/TurnBasedJRPGTemplate/Blueprints/Items/Equipment/StatictTarot1/Placida/BP_StaticTarot1Placida.BP_StaticTarot1Placida_C")
      (if (or (or (== _weapon "/Game/TurnBasedJRPGTemplate/Blueprints/Items/Equipment/Weapons/BP_Axe.BP_Axe_C") (== _weapon "/Game/TurnBasedJRPGTemplate/Blueprints/Items/Equipment/Weapons/BP_KitchenKnife.BP_KitchenKnife_C")) (or (== _armor "/Game/TurnBasedJRPGTemplate/Blueprints/Items/Equipment/Weapons/BP_Axe.BP_Axe_C") (== _armor "/Game/TurnBasedJRPGTemplate/Blueprints/Items/Equipment/Weapons/BP_KitchenKnife.BP_KitchenKnife_C")))
        (bind _firstlevelstats (defaults `Object` _array_element))
        (setmembers `/Game/TurnBasedJRPGTemplate/Blueprints/Structs/S_UnitStats` :`StructRef` _firstlevelstats :`maxAttack` (+ (`.maxAttack_15_24D8527844E2DFB657716C9F16A4AE21` (break `/Game/TurnBasedJRPGTemplate/Blueprints/Structs/S_UnitStats` _firstlevelstats)) 5))))))

(event `self.OnBuffEnded`
  ;[1 1 1] Remove Tarot 1 buff
  (bind _asbp_jrpgplayer_controller (cast `/Game/TurnBasedJRPGTemplate/Blueprints/Controllers/BP_JRPGPlayerController` (`GameplayStatics.GetPlayerController` 0)))
  (bind _playerunits (`/Game/TurnBasedJRPGTemplate/Blueprints/Controllers/BP_JRPGPlayerController.playerUnits` _asbp_jrpgplayer_controller))
  (bind _keys (`BlueprintMapLibrary.Map_Keys` _playerunits))
  (for _array_element _keys
    (bind ((`Weapon_19_25C66CFA4AEC9B2EB46636BA5392040B` _weapon) (`Armor_20_3FACB90A4F7AB732B976FDBD9DF85285` _armor) (`StaticTarotSocket1_49_386CDF41496C8A1A94652D804435853A` _statictarotsocket1)) (break `/Game/TurnBasedJRPGTemplate/Blueprints/Structs/S_PlayerUnitData` (`BlueprintMapLibrary.Map_Find` _playerunits "/Game/TurnBasedJRPGTemplate/Blueprints/Units/PlayerUnits/BP_PriestPlayerUnit.BP_PriestPlayerUnit_C")))
    (if (== _statictarotsocket1 "/Game/TurnBasedJRPGTemplate/Blueprints/Items/Equipment/StatictTarot1/Placida/BP_StaticTarot1Placida.BP_StaticTarot1Placida_C")
      (if (or (or (== _weapon "/Game/TurnBasedJRPGTemplate/Blueprints/Items/Equipment/Weapons/BP_Axe.BP_Axe_C") (== _weapon "/Game/TurnBasedJRPGTemplate/Blueprints/Items/Equipment/Weapons/BP_KitchenKnife.BP_KitchenKnife_C")) (or (== _armor "/Game/TurnBasedJRPGTemplate/Blueprints/Items/Equipment/Weapons/BP_Axe.BP_Axe_C") (== _armor "/Game/TurnBasedJRPGTemplate/Blueprints/Items/Equipment/Weapons/BP_KitchenKnife.BP_KitchenKnife_C")))
        (bind _firstlevelstats (defaults `Object` _array_element))
        (setmembers `/Game/TurnBasedJRPGTemplate/Blueprints/Structs/S_UnitStats` :`StructRef` _firstlevelstats :`maxAttack` (- (`.maxAttack_15_24D8527844E2DFB657716C9F16A4AE21` (break `/Game/TurnBasedJRPGTemplate/Blueprints/Structs/S_UnitStats` _firstlevelstats)) 5))))))

(fn `UserConstructionScript`
  (`parent.UserConstructionScript`))