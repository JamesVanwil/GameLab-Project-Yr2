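; Stage 2 Static Tarot 1 item for Placida that sets an attack bonus tied to owning certain weapons.
; Every Tick it searches the JRPG player controller's Equipment for the axe, book weapon or kitchen knife.
; On the first match, a DoOnce sets MaxAttack on the stats struct read from BP_StaticTarot1Placida's class defaults, rather than on this item's own stats.
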(event `self.ReceiveTick`
  (params (DeltaSeconds :type "Float (single-precision)"))
  (bind _asbp_jrpgplayer_controller (cast `/Game/TurnBasedJRPGTemplate/Blueprints/Controllers/BP_JRPGPlayerController` (`GameplayStatics.GetPlayerController` 0)))
  (bind _equipment (`/Game/TurnBasedJRPGTemplate/Blueprints/Controllers/BP_JRPGPlayerController.equipment` _asbp_jrpgplayer_controller))
  (if (or (`.ReturnValue` (`BlueprintMapLibrary.Map_Find` _equipment "/Game/TurnBasedJRPGTemplate/Blueprints/Items/Equipment/Weapons/BP_Axe.BP_Axe_C")) (`.ReturnValue` (`BlueprintMapLibrary.Map_Find` _equipment "/Game/TurnBasedJRPGTemplate/Blueprints/Items/Equipment/Weapons/BP_BookWeapon.BP_BookWeapon_C")) (`.ReturnValue` (`BlueprintMapLibrary.Map_Find` _equipment "/Game/TurnBasedJRPGTemplate/Blueprints/Items/Equipment/Weapons/BP_KitchenKnife.BP_KitchenKnife_C")))
    (`/Engine/EditorBlueprintResources/StandardMacros.DoOnce` false
      (:`Completed`
        (setmembers `/Game/TurnBasedJRPGTemplate/Blueprints/Structs/S_UnitStats` :`StructRef` (defaults `/Game/TurnBasedJRPGTemplate/Blueprints/Items/Equipment/StatictTarot1/Placida/BP_StaticTarot1Placida` "/Game/TurnBasedJRPGTemplate/Blueprints/Items/Equipment/StatictTarot1/Placida/BP_StaticTarot1Placida.BP_StaticTarot1Placida_C") :`maxAttack` 5)))))

(fn `UserConstructionScript`
  (`parent.UserConstructionScript`))