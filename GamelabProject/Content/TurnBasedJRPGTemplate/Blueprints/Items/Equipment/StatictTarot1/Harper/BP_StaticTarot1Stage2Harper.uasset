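; Stage 2 of Harper's first static tarot item, tying a magical attack buff to the archer unit's tarot points.
; BeginPlay adds three tarot points to that unit's data from the JRPG player controller.
; Tick checks for zero points to add or remove MaxMagicalAttack on BP_StaticTarot1Harper class defaults, setting IsBuffAppliedOnHarper.
; Both inner checks test constant true rather than that flag, so only the removal can run.
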(event `self.ReceiveBeginPlay`
  (bind _asbp_jrpgplayer_controller (cast `/Game/TurnBasedJRPGTemplate/Blueprints/Controllers/BP_JRPGPlayerController` (`GameplayStatics.GetPlayerController` 0)))
  (bind _value (`BlueprintMapLibrary.Map_Find` (`/Game/TurnBasedJRPGTemplate/Blueprints/Controllers/BP_JRPGPlayerController.playerUnits` _asbp_jrpgplayer_controller) "/Game/TurnBasedJRPGTemplate/Blueprints/Units/PlayerUnits/BP_ArcherPlayerUnit.BP_ArcherPlayerUnit_C"))
  (setmembers `/Game/TurnBasedJRPGTemplate/Blueprints/Structs/S_PlayerUnitData` :`StructRef` _value :`PlayerCurrentTarotPoints` (+ (`.PlayerCurrentTarotPoints_40_BD606433466E94380072AEBC073B173E` (break `/Game/TurnBasedJRPGTemplate/Blueprints/Structs/S_PlayerUnitData` _value)) 3)))

(event `self.ReceiveTick`
  (params (DeltaSeconds :type "Float (single-precision)"))
  (bind _stats (defaults `/Game/TurnBasedJRPGTemplate/Blueprints/Items/Equipment/StatictTarot1/Harper/BP_StaticTarot1Harper` "/Game/TurnBasedJRPGTemplate/Blueprints/Items/Equipment/StatictTarot1/Harper/BP_StaticTarot1Harper.BP_StaticTarot1Harper_C"))
  (bind _stats_2 (defaults `/Game/TurnBasedJRPGTemplate/Blueprints/Items/Equipment/StatictTarot1/Harper/BP_StaticTarot1Harper` "/Game/TurnBasedJRPGTemplate/Blueprints/Items/Equipment/StatictTarot1/Harper/BP_StaticTarot1Harper.BP_StaticTarot1Harper_C"))
  (bind _asbp_jrpgplayer_controller (cast `/Game/TurnBasedJRPGTemplate/Blueprints/Controllers/BP_JRPGPlayerController` (`GameplayStatics.GetPlayerController` 0)))
  (if (== (`.PlayerCurrentTarotPoints_40_BD606433466E94380072AEBC073B173E` (break `/Game/TurnBasedJRPGTemplate/Blueprints/Structs/S_PlayerUnitData` (`BlueprintMapLibrary.Map_Find` (`/Game/TurnBasedJRPGTemplate/Blueprints/Controllers/BP_JRPGPlayerController.playerUnits` _asbp_jrpgplayer_controller) "/Game/TurnBasedJRPGTemplate/Blueprints/Units/PlayerUnits/BP_ArcherPlayerUnit.BP_ArcherPlayerUnit_C"))) 0)
    (if (not true)
      (setmembers `/Game/TurnBasedJRPGTemplate/Blueprints/Structs/S_UnitStats` :`StructRef` _stats_2 :`maxMagicalAttack` (+ (`.maxMagicalAttack_24_C0C7731143A09315B418E7876A1F2F19` (break `/Game/TurnBasedJRPGTemplate/Blueprints/Structs/S_UnitStats` _stats_2)) 8))
      (set `self.IsBuffAppliedOnHarper?` true))
    (elif true
      (setmembers `/Game/TurnBasedJRPGTemplate/Blueprints/Structs/S_UnitStats` :`StructRef` _stats :`maxMagicalAttack` (- (`.maxMagicalAttack_24_C0C7731143A09315B418E7876A1F2F19` (break `/Game/TurnBasedJRPGTemplate/Blueprints/Structs/S_UnitStats` _stats)) 8))
      (set `self.IsBuffAppliedOnHarper?` false))))

(fn `UserConstructionScript`
  (`parent.UserConstructionScript`))