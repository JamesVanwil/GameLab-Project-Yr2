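; Buff for the Harper static tarot in socket 1, meant to adjust the Archer unit's max magical attack in the turn-based JRPG.
; ApplyBuff checks the Archer's StaticTarotSocket1 through the player controller, then adds a flat bonus to the stats struct read from Archer class defaults.
; OnBuffEnded repeats that Archer check while looping over all PlayerUnits keys, subtracting the bonus from each unit class's defaults, not just the Archer's.
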(event `self.ApplyBuff`
  (bind _firstlevelstats (defaults `/Game/TurnBasedJRPGTemplate/Blueprints/Units/PlayerUnits/BP_ArcherPlayerUnit` "/Game/TurnBasedJRPGTemplate/Blueprints/Units/PlayerUnits/BP_ArcherPlayerUnit.BP_ArcherPlayerUnit_C"))
  ;[1 1 1] Apply Tarot 1 Buff
  (bind _asbp_jrpgplayer_controller (cast `/Game/TurnBasedJRPGTemplate/Blueprints/Controllers/BP_JRPGPlayerController` (`GameplayStatics.GetPlayerController` 0)))
  (if (== (`.StaticTarotSocket1_49_386CDF41496C8A1A94652D804435853A` (break `/Game/TurnBasedJRPGTemplate/Blueprints/Structs/S_PlayerUnitData` (`BlueprintMapLibrary.Map_Find` (`/Game/TurnBasedJRPGTemplate/Blueprints/Controllers/BP_JRPGPlayerController.playerUnits` _asbp_jrpgplayer_controller) "/Game/TurnBasedJRPGTemplate/Blueprints/Units/PlayerUnits/BP_ArcherPlayerUnit.BP_ArcherPlayerUnit_C"))) "/Game/TurnBasedJRPGTemplate/Blueprints/Items/Equipment/StatictTarot1/Harper/BP_StaticTarot1Harper.BP_StaticTarot1Harper_C")
    (`KismetSystemLibrary.PrintString` "Stats changed")
    (setmembers `/Game/TurnBasedJRPGTemplate/Blueprints/Structs/S_UnitStats` :`StructRef` _firstlevelstats :`maxMagicalAttack` (+ (`.maxMagicalAttack_24_C0C7731143A09315B418E7876A1F2F19` (break `/Game/TurnBasedJRPGTemplate/Blueprints/Structs/S_UnitStats` _firstlevelstats)) 3))))

(event `self.OnBuffEnded`
  ;[1 1 1] Remove Tarot 1 buff
  (bind _asbp_jrpgplayer_controller (cast `/Game/TurnBasedJRPGTemplate/Blueprints/Controllers/BP_JRPGPlayerController` (`GameplayStatics.GetPlayerController` 0)))
  (bind _playerunits (`/Game/TurnBasedJRPGTemplate/Blueprints/Controllers/BP_JRPGPlayerController.playerUnits` _asbp_jrpgplayer_controller))
  (bind _keys (`BlueprintMapLibrary.Map_Keys` _playerunits))
  (for _array_element _keys
    (if (== (`.StaticTarotSocket1_49_386CDF41496C8A1A94652D804435853A` (break `/Game/TurnBasedJRPGTemplate/Blueprints/Structs/S_PlayerUnitData` (`BlueprintMapLibrary.Map_Find` _playerunits "/Game/TurnBasedJRPGTemplate/Blueprints/Units/PlayerUnits/BP_ArcherPlayerUnit.BP_ArcherPlayerUnit_C"))) "/Game/TurnBasedJRPGTemplate/Blueprints/Items/Equipment/StatictTarot1/Harper/BP_StaticTarot1Harper.BP_StaticTarot1Harper_C")
      (bind _firstlevelstats (defaults `Object` _array_element))
      (setmembers `/Game/TurnBasedJRPGTemplate/Blueprints/Structs/S_UnitStats` :`StructRef` _firstlevelstats :`maxMagicalAttack` (- (`.maxMagicalAttack_24_C0C7731143A09315B418E7876A1F2F19` (break `/Game/TurnBasedJRPGTemplate/Blueprints/Structs/S_UnitStats` _firstlevelstats)) 3)))))

(fn `UserConstructionScript`
  (`parent.UserConstructionScript`))