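; Tarot 7 boots equipment Blueprint whose logic actually governs the Tarot3 damage buff.
; On Tick, it checks the player controller for a Mage or Archer unit and Tarot3 in the equipment data.
; When the first BP_BuffDamageTarot3 actor found has DurationTurn above two, it calls OnBuffEnded once, latched by IsTarotBeenActivated.
; Unconnected Priest and Swordsman logic would toggle the Tarot 3 socket button by turn count.
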(event `self.ReceiveTick`
  (params (DeltaSeconds :type "Float (single-precision)"))
  ;[1 1 1] Activate/Deactivate Tarot on Tick for each character
  (`parent.ReceiveTick` DeltaSeconds)
  (bind _asbp_jrpgplayer_controller (cast `/Game/TurnBasedJRPGTemplate/Blueprints/Controllers/BP_JRPGPlayerController` (`GameplayStatics.GetPlayerController` 0)))
  ;;[1 0.9373 0.749] Mage
  (bind _allequipment (`/Game/TurnBasedJRPGTemplate/Blueprints/Controllers/BP_JRPGFunctionLibrary.GetAllEquipment` (`/Game/TurnBasedJRPGTemplate/Blueprints/Controllers/BP_JRPGPlayerController.Player Unit Data` _asbp_jrpgplayer_controller)))
  (bind _returnvalue (`GameplayStatics.GetActorOfClass` "/Game/TurnBasedJRPGTemplate/Blueprints/Skills/Buffs/BP_BuffDamageTarot3.BP_BuffDamageTarot3_C"))
  (bind _playerunits (`/Game/TurnBasedJRPGTemplate/Blueprints/Controllers/BP_JRPGPlayerController.playerUnits` _asbp_jrpgplayer_controller))
  (if (and (`.ReturnValue` (`BlueprintMapLibrary.Map_Find` _playerunits "/Game/TurnBasedJRPGTemplate/Blueprints/Units/PlayerUnits/BP_MagePlayerUnit.BP_MagePlayerUnit_C")) (`KismetArrayLibrary.Array_Contains` _allequipment "/Game/TurnBasedJRPGTemplate/Blueprints/Items/Equipment/TarotSocket3/Tarot3.Tarot3_C"))
    (if (> (`/Game/TurnBasedJRPGTemplate/Blueprints/Skills/Buffs/BP_BuffBase.durationTurn` _returnvalue) 2)
      (if (not (`self.IsTarotBeenActivated?`))
        (bind _returnvalue_2 (`GameplayStatics.GetActorOfClass` "/Game/TurnBasedJRPGTemplate/Blueprints/Skills/Buffs/BP_BuffDamageTarot3.BP_BuffDamageTarot3_C"))
        (`/Game/TurnBasedJRPGTemplate/Blueprints/Skills/Buffs/BP_BuffBase.OnBuffEnded` _returnvalue_2)
        (set `self.IsTarotBeenActivated?` true)))
    (else
      ;;[0.6157 0.8078 1] Archer
      (bind _allequipment_2 (`/Game/TurnBasedJRPGTemplate/Blueprints/Controllers/BP_JRPGFunctionLibrary.GetAllEquipment` (`/Game/TurnBasedJRPGTemplate/Blueprints/Controllers/BP_JRPGPlayerController.Player Unit Data` _asbp_jrpgplayer_controller)))
      (bind _returnvalue_3 (`GameplayStatics.GetActorOfClass` "/Game/TurnBasedJRPGTemplate/Blueprints/Skills/Buffs/BP_BuffDamageTarot3.BP_BuffDamageTarot3_C"))
      (if (and (`.ReturnValue` (`BlueprintMapLibrary.Map_Find` _playerunits "/Game/TurnBasedJRPGTemplate/Blueprints/Units/PlayerUnits/BP_ArcherPlayerUnit.BP_ArcherPlayerUnit_C")) (`KismetArrayLibrary.Array_Contains` _allequipment_2 "/Game/TurnBasedJRPGTemplate/Blueprints/Items/Equipment/TarotSocket3/Tarot3.Tarot3_C"))
        (if (> (`/Game/TurnBasedJRPGTemplate/Blueprints/Skills/Buffs/BP_BuffBase.durationTurn` _returnvalue_3) 2)
          (if (not (`self.IsTarotBeenActivated?`))
            (bind _returnvalue_4 (`GameplayStatics.GetActorOfClass` "/Game/TurnBasedJRPGTemplate/Blueprints/Skills/Buffs/BP_BuffDamageTarot3.BP_BuffDamageTarot3_C"))
            (`/Game/TurnBasedJRPGTemplate/Blueprints/Skills/Buffs/BP_BuffBase.OnBuffEnded` _returnvalue_4)
            (set `self.IsTarotBeenActivated?` true)))))))

(fn `UserConstructionScript`
  (`parent.UserConstructionScript`))