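; Boots tarot equipment that grants 25 bonus Max HP while the checked character's current HP is above 90.
; Tick checks Mage, Archer, Priest and Swordsman in an else chain, handling only the first match, and toggles the equipment UI's boots button alongside the bonus.
; Flag-guarded events edit the class-default stats, which BeginPlay resets to zero Max HP.
; Disconnected test graphs never run.
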(event `self.ReceiveTick`
  (params (DeltaSeconds :type "Float (single-precision)"))
  ;[1 1 1] Activate/Deactivate Tarot on Tick for each character
  (`parent.ReceiveTick` DeltaSeconds)
  (bind _asbp_jrpgplayer_controller (cast `/Game/TurnBasedJRPGTemplate/Blueprints/Controllers/BP_JRPGPlayerController` (`GameplayStatics.GetPlayerController` 0)))
  ;;[1 0.9373 0.749] Mage
  (bind _allequipment (`/Game/TurnBasedJRPGTemplate/Blueprints/Controllers/BP_JRPGFunctionLibrary.GetAllEquipment` (`/Game/TurnBasedJRPGTemplate/Blueprints/Controllers/BP_JRPGPlayerController.Player Unit Data` _asbp_jrpgplayer_controller)))
  (bind _playerunits (`/Game/TurnBasedJRPGTemplate/Blueprints/Controllers/BP_JRPGPlayerController.playerUnits` _asbp_jrpgplayer_controller))
  (bind (_value _returnvalue) (`BlueprintMapLibrary.Map_Find` _playerunits "/Game/TurnBasedJRPGTemplate/Blueprints/Units/PlayerUnits/BP_MagePlayerUnit.BP_MagePlayerUnit_C"))
  (if (and _returnvalue (`KismetArrayLibrary.Array_Contains` _allequipment "BP_AddHPTarotBoots_C"))
    (if (<= (`.currentHP_4_0B53A15447C685E66E26429EA6694AA4` (break `/Game/TurnBasedJRPGTemplate/Blueprints/Structs/S_PlayerUnitData` _value)) 90)
      (bind _foundwidgets (`WidgetBlueprintLibrary.GetAllWidgetsOfClass` "/Game/TurnBasedJRPGTemplate/Blueprints/UI/MainMenu/BP_WearEquipmentUI.BP_WearEquipmentUI_C"))
      (`Widget.SetIsEnabled` (`/Game/TurnBasedJRPGTemplate/Blueprints/UI/MainMenu/BP_WearEquipmentUI.BootsButton` (`|GetArrayItem` _foundwidgets)) false)
      (`self.RemoveHPTarotBoots`)
      (else
        (bind _foundwidgets_2 (`WidgetBlueprintLibrary.GetAllWidgetsOfClass` "/Game/TurnBasedJRPGTemplate/Blueprints/UI/MainMenu/BP_WearEquipmentUI.BP_WearEquipmentUI_C"))
        (`Widget.SetIsEnabled` (`/Game/TurnBasedJRPGTemplate/Blueprints/UI/MainMenu/BP_WearEquipmentUI.BootsButton` (`|GetArrayItem` _foundwidgets_2)) true)
        (`self.AddHPTarotBoots`)))
    (else
      ;;[0.6157 0.8078 1] Archer
      (bind _allequipment_2 (`/Game/TurnBasedJRPGTemplate/Blueprints/Controllers/BP_JRPGFunctionLibrary.GetAllEquipment` (`/Game/TurnBasedJRPGTemplate/Blueprints/Controllers/BP_JRPGPlayerController.Player Unit Data` _asbp_jrpgplayer_controller)))
      (bind (_value_2 _returnvalue_2) (`BlueprintMapLibrary.Map_Find` _playerunits "/Game/TurnBasedJRPGTemplate/Blueprints/Units/PlayerUnits/BP_ArcherPlayerUnit.BP_ArcherPlayerUnit_C"))
      (if (and (`KismetArrayLibrary.Array_Contains` _allequipment_2 "BP_AddHPTarotBoots_C") _returnvalue_2)
        (if (<= (`.currentHP_4_0B53A15447C685E66E26429EA6694AA4` (break `/Game/TurnBasedJRPGTemplate/Blueprints/Structs/S_PlayerUnitData` _value_2)) 90)
          (bind _foundwidgets_3 (`WidgetBlueprintLibrary.GetAllWidgetsOfClass` "/Game/TurnBasedJRPGTemplate/Blueprints/UI/MainMenu/BP_WearEquipmentUI.BP_WearEquipmentUI_C"))
          (`Widget.SetIsEnabled` (`/Game/TurnBasedJRPGTemplate/Blueprints/UI/MainMenu/BP_WearEquipmentUI.BootsButton` (`|GetArrayItem` _foundwidgets_3)) false)
          (`self.RemoveHPTarotBoots`)
          (else
            (bind _foundwidgets_4 (`WidgetBlueprintLibrary.GetAllWidgetsOfClass` "/Game/TurnBasedJRPGTemplate/Blueprints/UI/MainMenu/BP_WearEquipmentUI.BP_WearEquipmentUI_C"))
            (`Widget.SetIsEnabled` (`/Game/TurnBasedJRPGTemplate/Blueprints/UI/MainMenu/BP_WearEquipmentUI.BootsButton` (`|GetArrayItem` _foundwidgets_4)) true)
            (`self.AddHPTarotBoots`)))
        (else
          ;;[0.5529 1 0.5961] Priest
          (bind _allequipment_3 (`/Game/TurnBasedJRPGTemplate/Blueprints/Controllers/BP_JRPGFunctionLibrary.GetAllEquipment` (`/Game/TurnBasedJRPGTemplate/Blueprints/Controllers/BP_JRPGPlayerController.Player Unit Data` _asbp_jrpgplayer_controller)))
          (bind (_value_3 _returnvalue_3) (`BlueprintMapLibrary.Map_Find` _playerunits "/Game/TurnBasedJRPGTemplate/Blueprints/Units/PlayerUnits/BP_PriestPlayerUnit.BP_PriestPlayerUnit_C"))
          (if (and (`KismetArrayLibrary.Array_Contains` _allequipment_3 "BP_AddHPTarotBoots_C") _returnvalue_3)
            (if (<= (`.currentHP_4_0B53A15447C685E66E26429EA6694AA4` (break `/Game/TurnBasedJRPGTemplate/Blueprints/Structs/S_PlayerUnitData` _value_3)) 90)
              (bind _foundwidgets_5 (`WidgetBlueprintLibrary.GetAllWidgetsOfClass` "/Game/TurnBasedJRPGTemplate/Blueprints/UI/MainMenu/BP_WearEquipmentUI.BP_WearEquipmentUI_C"))
              (`Widget.SetIsEnabled` (`/Game/TurnBasedJRPGTemplate/Blueprints/UI/MainMenu/BP_WearEquipmentUI.BootsButton` (`|GetArrayItem` _foundwidgets_5)) false)
              (`self.RemoveHPTarotBoots`)
              (else
                (bind _foundwidgets_6 (`WidgetBlueprintLibrary.GetAllWidgetsOfClass` "/Game/TurnBasedJRPGTemplate/Blueprints/UI/MainMenu/BP_WearEquipmentUI.BP_WearEquipmentUI_C"))
                (`Widget.SetIsEnabled` (`/Game/TurnBasedJRPGTemplate/Blueprints/UI/MainMenu/BP_WearEquipmentUI.BootsButton` (`|GetArrayItem` _foundwidgets_6)) true)
                (`self.AddHPTarotBoots`)))
            (else
              ;;[1 0.4745 0.9333] Swordsman
              (bind _allequipment_4 (`/Game/TurnBasedJRPGTemplate/Blueprints/Controllers/BP_JRPGFunctionLibrary.GetAllEquipment` (`/Game/TurnBasedJRPGTemplate/Blueprints/Controllers/BP_JRPGPlayerController.Player Unit Data` _asbp_jrpgplayer_controller)))
              (bind (_value_4 _returnvalue_4) (`BlueprintMapLibrary.Map_Find` _playerunits "/Game/TurnBasedJRPGTemplate/Blueprints/Units/PlayerUnits/BP_SwordsmanPlayerUnit.BP_SwordsmanPlayerUnit_C"))
              (if (and (`KismetArrayLibrary.Array_Contains` _allequipment_4 "BP_AddHPTarotBoots_C") _returnvalue_4)
                (if (<= (`.currentHP_4_0B53A15447C685E66E26429EA6694AA4` (break `/Game/TurnBasedJRPGTemplate/Blueprints/Structs/S_PlayerUnitData` _value_4)) 90)
                  (bind _foundwidgets_7 (`WidgetBlueprintLibrary.GetAllWidgetsOfClass` "/Game/TurnBasedJRPGTemplate/Blueprints/UI/MainMenu/BP_WearEquipmentUI.BP_WearEquipmentUI_C"))
                  (`Widget.SetIsEnabled` (`/Game/TurnBasedJRPGTemplate/Blueprints/UI/MainMenu/BP_WearEquipmentUI.BootsButton` (`|GetArrayItem` _foundwidgets_7)) false)
                  (`self.RemoveHPTarotBoots`)
                  (else
                    (bind _foundwidgets_8 (`WidgetBlueprintLibrary.GetAllWidgetsOfClass` "/Game/TurnBasedJRPGTemplate/Blueprints/UI/MainMenu/BP_WearEquipmentUI.BP_WearEquipmentUI_C"))
                    (`Widget.SetIsEnabled` (`/Game/TurnBasedJRPGTemplate/Blueprints/UI/MainMenu/BP_WearEquipmentUI.BootsButton` (`|GetArrayItem` _foundwidgets_8)) true)
                    (`self.AddHPTarotBoots`)))))))))))

(event `self.ReceiveBeginPlay`
  ;[1 1 1] Set Class Defaults Max HP to zero on start
  (`parent.ReceiveBeginPlay`)
  (setmembers `/Game/TurnBasedJRPGTemplate/Blueprints/Structs/S_UnitStats` :`StructRef` (`.stats` (defaults `/Game/TurnBasedJRPGTemplate/Blueprints/Items/Equipment/Helms/BP_AddHPTarotBoots` "BP_AddHPTarotBoots_C")) :`maxHP` 0))

(event `AddHPTarotBoots`
  (bind (_playerunit _bp_condition _conditionfraction _player_units _istarotbeenactivated_ _stats) (defaults `/Game/TurnBasedJRPGTemplate/Blueprints/Items/Equipment/Helms/BP_AddHPTarotBoots` "BP_AddHPTarotBoots_C"))
  ;[1 1 1] Add Tarot HP
  (if (not (`self.IsTarotBeenActivated?`))
    (setmembers `/Game/TurnBasedJRPGTemplate/Blueprints/Structs/S_UnitStats` :`StructRef` _stats :`maxHP` (+ (`.maxHP_2_41B41BC24C39ED8CDC0C58B3398B651D` (break `/Game/TurnBasedJRPGTemplate/Blueprints/Structs/S_UnitStats` _stats)) 25))
    (set `self.IsTarotBeenActivated?` true)))

(event `RemoveHPTarotBoots`
  (bind (_playerunit _bp_condition _conditionfraction _player_units _istarotbeenactivated_ _stats) (defaults `/Game/TurnBasedJRPGTemplate/Blueprints/Items/Equipment/Helms/BP_AddHPTarotBoots` "BP_AddHPTarotBoots_C"))
  ;[1 1 1] Remove Tarot HP
  (if (`self.IsTarotBeenActivated?`)
    (setmembers `/Game/TurnBasedJRPGTemplate/Blueprints/Structs/S_UnitStats` :`StructRef` _stats :`maxHP` (- (`.maxHP_2_41B41BC24C39ED8CDC0C58B3398B651D` (break `/Game/TurnBasedJRPGTemplate/Blueprints/Structs/S_UnitStats` _stats)) 25))
    (set `self.IsTarotBeenActivated?` false)))

(fn `StatGet`
  (params (StatType :type "/Game/TurnBasedJRPGTemplate/Blueprints/Conditions/E_StatType Enum" :default "NewEnumerator0") (Stats :type "/Game/TurnBasedJRPGTemplate/Blueprints/Structs/S_PlayerUnitData Structure"))
  (returns (Stat :type Integer))
  (switch `/Game/TurnBasedJRPGTemplate/Blueprints/Conditions/E_StatType` StatType
    (:`NewEnumerator0`
      (return Stats_currentHP_4_0B53A15447C685E66E26429EA6694AA4))))

(fn `UserConstructionScript`
  (`parent.UserConstructionScript`))