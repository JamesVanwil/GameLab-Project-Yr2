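; Helm-slot tarot equipment meant to add damage, switched on or off by its wearer's condition.
; Tick checks Mage, Archer, Priest and Swordsman in order, acting on the first match.
; For the Mage, low HP ends the BP_BuffAddDamage buff and recovery reapplies it.
; For the others, low MP disables the helm button, but the Add/Remove events are empty and the MinAttack edits are disconnected.
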(event `self.ReceiveBeginPlay`
  ;[1 1 1] Set Min Attack to 25 at start
  (`parent.ReceiveBeginPlay`))

(event `AddDamageTarot`
  ;[1 1 1] Add Damage Tarot
)

(event `RemoveDamageTarot`
  ;[1 1 1] Remove Damage Tarot
)

(event `self.ReceiveTick`
  (params (DeltaSeconds :type "Float (single-precision)"))
  ;[1 1 1] Activate/Deactivate Tarot on Tick for each character
  (`parent.ReceiveTick` DeltaSeconds)
  (bind _asbp_jrpgplayer_controller (cast `/Game/TurnBasedJRPGTemplate/Blueprints/Controllers/BP_JRPGPlayerController` (`GameplayStatics.GetPlayerController` 0)))
  ;;[1 0.9373 0.749] Mage
  (bind _allequipment (`/Game/TurnBasedJRPGTemplate/Blueprints/Controllers/BP_JRPGFunctionLibrary.GetAllEquipment` (`/Game/TurnBasedJRPGTemplate/Blueprints/Controllers/BP_JRPGPlayerController.Player Unit Data` _asbp_jrpgplayer_controller)))
  (bind _playerunits (`/Game/TurnBasedJRPGTemplate/Blueprints/Controllers/BP_JRPGPlayerController.playerUnits` _asbp_jrpgplayer_controller))
  (bind (_value _returnvalue) (`BlueprintMapLibrary.Map_Find` _playerunits "/Game/TurnBasedJRPGTemplate/Blueprints/Units/PlayerUnits/BP_MagePlayerUnit.BP_MagePlayerUnit_C"))
  (if (and _returnvalue (`KismetArrayLibrary.Array_Contains` _allequipment "BP_AddDamageTarot_C"))
    (if (< (`.currentHP_4_0B53A15447C685E66E26429EA6694AA4` (break `/Game/TurnBasedJRPGTemplate/Blueprints/Structs/S_PlayerUnitData` _value)) 125)
      (if (not (`self.IsTarotBeenActivated?`))
        (bind _returnvalue_2 (`GameplayStatics.GetActorOfClass` "/Game/TurnBasedJRPGTemplate/Blueprints/Skills/Buffs/BP_BuffAddDamage.BP_BuffAddDamage_C"))
        (`/Game/TurnBasedJRPGTemplate/Blueprints/Skills/Buffs/BP_BuffBase.OnBuffEnded` _returnvalue_2)
        (set `self.IsTarotBeenActivated?` true)
        (set `self.HasBuffEnded` true))
      (elif (`self.HasBuffEnded`)
        (bind _returnvalue_3 (`GameplayStatics.GetActorOfClass` "/Game/TurnBasedJRPGTemplate/Blueprints/Skills/Buffs/BP_BuffAddDamage.BP_BuffAddDamage_C"))
        (`/Game/TurnBasedJRPGTemplate/Blueprints/Skills/Buffs/BP_BuffBase.ApplyBuff` _returnvalue_3)
        (set `self.IsTarotBeenActivated?` false)
        (set `self.HasBuffEnded` false)))
    (else
      ;;[0.6157 0.8078 1] Archer
      (bind _allequipment_2 (`/Game/TurnBasedJRPGTemplate/Blueprints/Controllers/BP_JRPGFunctionLibrary.GetAllEquipment` (`/Game/TurnBasedJRPGTemplate/Blueprints/Controllers/BP_JRPGPlayerController.Player Unit Data` _asbp_jrpgplayer_controller)))
      (bind (_value_2 _returnvalue_4) (`BlueprintMapLibrary.Map_Find` _playerunits "/Game/TurnBasedJRPGTemplate/Blueprints/Units/PlayerUnits/BP_ArcherPlayerUnit.BP_ArcherPlayerUnit_C"))
      (if (and _returnvalue_4 (`KismetArrayLibrary.Array_Contains` _allequipment_2 "BP_AddDamageTarot_C"))
        (if (<= (`.curentMP_6_79399572456CC89F79B2DA9F0A8BB445` (break `/Game/TurnBasedJRPGTemplate/Blueprints/Structs/S_PlayerUnitData` _value_2)) 24)
          (bind _foundwidgets (`WidgetBlueprintLibrary.GetAllWidgetsOfClass` "/Game/TurnBasedJRPGTemplate/Blueprints/UI/MainMenu/BP_WearEquipmentUI.BP_WearEquipmentUI_C"))
          (`Widget.SetIsEnabled` (`/Game/TurnBasedJRPGTemplate/Blueprints/UI/MainMenu/BP_WearEquipmentUI.HelmButton` (`|GetArrayItem` _foundwidgets)) false)
          (`self.RemoveDamageTarot`)
          (else
            (bind _foundwidgets_2 (`WidgetBlueprintLibrary.GetAllWidgetsOfClass` "/Game/TurnBasedJRPGTemplate/Blueprints/UI/MainMenu/BP_WearEquipmentUI.BP_WearEquipmentUI_C"))
            (`Widget.SetIsEnabled` (`/Game/TurnBasedJRPGTemplate/Blueprints/UI/MainMenu/BP_WearEquipmentUI.HelmButton` (`|GetArrayItem` _foundwidgets_2)) true)
            (`self.AddDamageTarot`)))
        (else
          ;;[0.5529 1 0.5961] Priest
          (bind _allequipment_3 (`/Game/TurnBasedJRPGTemplate/Blueprints/Controllers/BP_JRPGFunctionLibrary.GetAllEquipment` (`/Game/TurnBasedJRPGTemplate/Blueprints/Controllers/BP_JRPGPlayerController.Player Unit Data` _asbp_jrpgplayer_controller)))
          (bind (_value_3 _returnvalue_5) (`BlueprintMapLibrary.Map_Find` _playerunits "/Game/TurnBasedJRPGTemplate/Blueprints/Units/PlayerUnits/BP_PriestPlayerUnit.BP_PriestPlayerUnit_C"))
          (if (and _returnvalue_5 (`KismetArrayLibrary.Array_Contains` _allequipment_3 "BP_AddDamageTarot_C"))
            (if (<= (`.curentMP_6_79399572456CC89F79B2DA9F0A8BB445` (break `/Game/TurnBasedJRPGTemplate/Blueprints/Structs/S_PlayerUnitData` _value_3)) 24)
              (bind _foundwidgets_3 (`WidgetBlueprintLibrary.GetAllWidgetsOfClass` "/Game/TurnBasedJRPGTemplate/Blueprints/UI/MainMenu/BP_WearEquipmentUI.BP_WearEquipmentUI_C"))
              (`Widget.SetIsEnabled` (`/Game/TurnBasedJRPGTemplate/Blueprints/UI/MainMenu/BP_WearEquipmentUI.HelmButton` (`|GetArrayItem` _foundwidgets_3)) false)
              (`self.RemoveDamageTarot`)
              (else
                (bind _foundwidgets_4 (`WidgetBlueprintLibrary.GetAllWidgetsOfClass` "/Game/TurnBasedJRPGTemplate/Blueprints/UI/MainMenu/BP_WearEquipmentUI.BP_WearEquipmentUI_C"))
                (`Widget.SetIsEnabled` (`/Game/TurnBasedJRPGTemplate/Blueprints/UI/MainMenu/BP_WearEquipmentUI.HelmButton` (`|GetArrayItem` _foundwidgets_4)) true)
                (`self.AddDamageTarot`)))
            (else
              ;;[1 0.4745 0.9333] Swordsman
              (bind _allequipment_4 (`/Game/TurnBasedJRPGTemplate/Blueprints/Controllers/BP_JRPGFunctionLibrary.GetAllEquipment` (`/Game/TurnBasedJRPGTemplate/Blueprints/Controllers/BP_JRPGPlayerController.Player Unit Data` _asbp_jrpgplayer_controller)))
              (bind (_value_4 _returnvalue_6) (`BlueprintMapLibrary.Map_Find` _playerunits "/Game/TurnBasedJRPGTemplate/Blueprints/Units/PlayerUnits/BP_SwordsmanPlayerUnit.BP_SwordsmanPlayerUnit_C"))
              (if (and _returnvalue_6 (`KismetArrayLibrary.Array_Contains` _allequipment_4 "BP_AddDamageTarot_C"))
                (if (<= (`.curentMP_6_79399572456CC89F79B2DA9F0A8BB445` (break `/Game/TurnBasedJRPGTemplate/Blueprints/Structs/S_PlayerUnitData` _value_4)) 24)
                  (bind _foundwidgets_5 (`WidgetBlueprintLibrary.GetAllWidgetsOfClass` "/Game/TurnBasedJRPGTemplate/Blueprints/UI/MainMenu/BP_WearEquipmentUI.BP_WearEquipmentUI_C"))
                  (`Widget.SetIsEnabled` (`/Game/TurnBasedJRPGTemplate/Blueprints/UI/MainMenu/BP_WearEquipmentUI.HelmButton` (`|GetArrayItem` _foundwidgets_5)) false)
                  (`self.RemoveDamageTarot`)
                  (else
                    (bind _foundwidgets_6 (`WidgetBlueprintLibrary.GetAllWidgetsOfClass` "/Game/TurnBasedJRPGTemplate/Blueprints/UI/MainMenu/BP_WearEquipmentUI.BP_WearEquipmentUI_C"))
                    (`Widget.SetIsEnabled` (`/Game/TurnBasedJRPGTemplate/Blueprints/UI/MainMenu/BP_WearEquipmentUI.HelmButton` (`|GetArrayItem` _foundwidgets_6)) true)
                    (`self.AddDamageTarot`)))))))))))

(fn `UserConstructionScript`
  (`parent.UserConstructionScript`))