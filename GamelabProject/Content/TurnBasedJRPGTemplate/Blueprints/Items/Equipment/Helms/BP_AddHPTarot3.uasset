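; BP_AddHPTarot3 is a tarot equipment item under Helms, named for adding HP, but currently inert.
; Tick and BeginPlay only call their parents, and the AddHPTarot3 and RemoveHPTarot3 events are empty.
; Disconnected experiments remain: Max HP edits on class defaults, per-character BP_BuffAddSpeed toggling on projectile hits, and Swordsman HP-based socket locking.
; A StatGet helper returns current HP, used only by an unwired condition-threshold test.
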(event `self.ReceiveTick`
  (params (DeltaSeconds :type "Float (single-precision)"))
  ;[1 1 1] Activate/Deactivate Tarot on Tick for each character
  (`parent.ReceiveTick` DeltaSeconds))

(event `self.ReceiveBeginPlay`
  ;[1 1 1] Set Class Defaults Max HP to zero on start
  (`parent.ReceiveBeginPlay`))

(event `AddHPTarot3`
  ;[1 1 1] Add Tarot HP
)

(event `RemoveHPTarot3`
  ;[1 1 1] Remove Tarot HP
)

(fn `StatGet`
  (params (StatType :type "/Game/TurnBasedJRPGTemplate/Blueprints/Conditions/E_StatType Enum" :default "NewEnumerator0") (Stats :type "/Game/TurnBasedJRPGTemplate/Blueprints/Structs/S_PlayerUnitData Structure"))
  (returns (Stat :type Integer))
  (switch `/Game/TurnBasedJRPGTemplate/Blueprints/Conditions/E_StatType` StatType
    (:`NewEnumerator0`
      (return Stats_currentHP_4_0B53A15447C685E66E26429EA6694AA4))))

(fn `UserConstructionScript`
  (`parent.UserConstructionScript`))