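; Damage tarot helm item that toggles a damage buff according to the wearer's state.
; Tick checks the player's units and equipment, taking the Mage branch (ActionTime threshold) first, otherwise the Archer's (HP threshold).
; At low values it ends the BP_BuffAddDamage actor's buff and reapplies it on recovery, using flags to fire once per change.
; Priest, Swordsman and MinAttack logic is disconnected, and the Add/Remove events are empty.
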(event `self.ReceiveBeginPlay`
  ;[1 1 1] Set Min Attack to 25 at start
  (`parent.ReceiveBeginPlay`))

(event `AddDamageTarot4`
  ;[1 1 1] Add Damage Tarot
)

(event `RemoveDamageTarot4`
  ;[1 1 1] Remove Damage Tarot
)

(event `self.ReceiveTick`
  (params (DeltaSeconds :type "Float (single-precision)"))
  ;[1 1 1] Activate/Deactivate Tarot on Tick for each character
  (`parent.ReceiveTick` DeltaSeconds)
  (bind _asbp_jrpgplayer_controller (cast `/Game/TurnBasedJRPGTemplate/Blueprints/Controllers/BP_JRPGPlayerController` (`GameplayStatics.GetPlayerController` 0)))
  (bind _playerunitstats (`/Game/TurnBasedJRPGTemplate/Blueprints/Controllers/BP_JRPGFunctionLibrary.GetPlayerUnitStatsFromData` "/Game/TurnBasedJRPGTemplate/Blueprints/Units/PlayerUnits/BP_MagePlayerUnit.BP_MagePlayerUnit_C"))
  ;;[1 0.9373 0.749] Mage
  (bind _allequipment (`/Game/TurnBasedJRPGTemplate/Blueprints/Controllers/BP_JRPGFunctionLibrary.GetAllEquipment` (`/Game/TurnBasedJRPGTemplate/Blueprints/Controllers/BP_JRPGPlayerController.Player Unit Data` _asbp_jrpgplayer_controller)))
  (bind _playerunits (`/Game/TurnBasedJRPGTemplate/Blueprints/Controllers/BP_JRPGPlayerController.playerUnits` _asbp_jrpgplayer_controller))
  (if (and (`.ReturnValue` (`BlueprintMapLibrary.Map_Find` _playerunits "/Game/TurnBasedJRPGTemplate/Blueprints/Units/PlayerUnits/BP_MagePlayerUnit.BP_MagePlayerUnit_C")) (`KismetArrayLibrary.Array_Contains` _allequipment "BP_AddDamageTarot4_C"))
    (if (<= (`.actionTime_31_CD6B6FA04FF3CB1C1BA72A93110B7A28` (break `/Game/TurnBasedJRPGTemplate/Blueprints/Structs/S_UnitStats` _playerunitstats)) 2.0)
      (if (not (`self.IsTarotBeenActivated?`))
        (bind _returnvalue (`GameplayStatics.GetActorOfClass` "/Game/TurnBasedJRPGTemplate/Blueprints/Skills/Buffs/BP_BuffAddDamage.BP_BuffAddDamage_C"))
        (`/Game/TurnBasedJRPGTemplate/Blueprints/Skills/Buffs/BP_BuffBase.OnBuffEnded` _returnvalue)
        (set `self.IsTarotBeenActivated?` true)
        (set `self.HasBuffEnded` true))
      (elif (`self.HasBuffEnded`)
        (bind _returnvalue_2 (`GameplayStatics.GetActorOfClass` "/Game/TurnBasedJRPGTemplate/Blueprints/Skills/Buffs/BP_BuffAddDamage.BP_BuffAddDamage_C"))
        (`/Game/TurnBasedJRPGTemplate/Blueprints/Skills/Buffs/BP_BuffBase.ApplyBuff` _returnvalue_2)
        (set `self.IsTarotBeenActivated?` false)
        (set `self.HasBuffEnded` false)))
    (else
      ;;[0.6157 0.8078 1] Archer
      (bind _allequipment_2 (`/Game/TurnBasedJRPGTemplate/Blueprints/Controllers/BP_JRPGFunctionLibrary.GetAllEquipment` (`/Game/TurnBasedJRPGTemplate/Blueprints/Controllers/BP_JRPGPlayerController.Player Unit Data` _asbp_jrpgplayer_controller)))
      (bind (_value _returnvalue_3) (`BlueprintMapLibrary.Map_Find` _playerunits "/Game/TurnBasedJRPGTemplate/Blueprints/Units/PlayerUnits/BP_ArcherPlayerUnit.BP_ArcherPlayerUnit_C"))
      (if (and _returnvalue_3 (`KismetArrayLibrary.Array_Contains` _allequipment_2 "BP_AddDamageTarot4_C"))
        (if (< (`.currentHP_4_0B53A15447C685E66E26429EA6694AA4` (break `/Game/TurnBasedJRPGTemplate/Blueprints/Structs/S_PlayerUnitData` _value)) 125)
          (if (not (`self.IsTarotBeenActivated?`))
            (bind _returnvalue_4 (`GameplayStatics.GetActorOfClass` "/Game/TurnBasedJRPGTemplate/Blueprints/Skills/Buffs/BP_BuffAddDamage.BP_BuffAddDamage_C"))
            (`/Game/TurnBasedJRPGTemplate/Blueprints/Skills/Buffs/BP_BuffBase.OnBuffEnded` _returnvalue_4)
            (set `self.IsTarotBeenActivated?` true)
            (set `self.HasBuffEnded` true))
          (elif (`self.HasBuffEnded`)
            (bind _returnvalue_5 (`GameplayStatics.GetActorOfClass` "/Game/TurnBasedJRPGTemplate/Blueprints/Skills/Buffs/BP_BuffAddDamage.BP_BuffAddDamage_C"))
            (`/Game/TurnBasedJRPGTemplate/Blueprints/Skills/Buffs/BP_BuffBase.ApplyBuff` _returnvalue_5)
            (set `self.IsTarotBeenActivated?` false)
            (set `self.HasBuffEnded` false)))))))

(fn `UserConstructionScript`
  (`parent.UserConstructionScript`))