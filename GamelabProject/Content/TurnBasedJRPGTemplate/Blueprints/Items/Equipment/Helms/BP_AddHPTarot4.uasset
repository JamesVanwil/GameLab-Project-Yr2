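; Tarot equipment item that, despite its AddHP name, toggles a speed buff based on the wearer's HP.
; Each Tick checks the Mage, otherwise the Archer, for the equipped item and compares current HP to a fixed threshold.
; Flags make the level's BP_BuffAddSpeed actor end once below the threshold and reapply on recovery.
; Max HP edits and Priest/Swordsman socket-button checks are disconnected, leaving the Add/Remove HP events empty.
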(event `self.ReceiveTick`
  (params (DeltaSeconds :type "Float (single-precision)"))
  ;[1 1 1] Activate/Deactivate Tarot on Tick for each character
  (`parent.ReceiveTick` DeltaSeconds)
  (bind _asbp_jrpgplayer_controller (cast `/Game/TurnBasedJRPGTemplate/Blueprints/Controllers/BP_JRPGPlayerController` (`GameplayStatics.GetPlayerController` 0)))
  ;;[1 0.9373 0.749] Mage
  (bind _allequipment (`/Game/TurnBasedJRPGTemplate/Blueprints/Controllers/BP_JRPGFunctionLibrary.GetAllEquipment` (`/Game/TurnBasedJRPGTemplate/Blueprints/Controllers/BP_JRPGPlayerController.Player Unit Data` _asbp_jrpgplayer_controller)))
  (bind _playerunits (`/Game/TurnBasedJRPGTemplate/Blueprints/Controllers/BP_JRPGPlayerController.playerUnits` _asbp_jrpgplayer_controller))
  (bind (_value _returnvalue) (`BlueprintMapLibrary.Map_Find` _playerunits "/Game/TurnBasedJRPGTemplate/Blueprints/Units/PlayerUnits/BP_MagePlayerUnit.BP_MagePlayerUnit_C"))
  (if (and _returnvalue (`KismetArrayLibrary.Array_Contains` _allequipment "BP_AddHPTarot4_C"))
    (if (< (`.currentHP_4_0B53A15447C685E66E26429EA6694AA4` (break `/Game/TurnBasedJRPGTemplate/Blueprints/Structs/S_PlayerUnitData` _value)) 125)
      (if (not (`self.IsTarotBeenActivated?`))
        (bind _returnvalue_2 (`GameplayStatics.GetActorOfClass` "/Game/TurnBasedJRPGTemplate/Blueprints/Skills/Buffs/BP_BuffAddSpeed.BP_BuffAddSpeed_C"))
        (`/Game/TurnBasedJRPGTemplate/Blueprints/Skills/Buffs/BP_BuffBase.OnBuffEnded` _returnvalue_2)
        (set `self.IsTarotBeenActivated?` true)
        (set `self.HasBuffEnded` true)
        (set `self.IsTarot8WandsActive?` false))
      (elif (`self.HasBuffEnded`)
        (bind _returnvalue_3 (`GameplayStatics.GetActorOfClass` "/Game/TurnBasedJRPGTemplate/Blueprints/Skills/Buffs/BP_BuffAddSpeed.BP_BuffAddSpeed_C"))
        (`/Game/TurnBasedJRPGTemplate/Blueprints/Skills/Buffs/BP_BuffBase.ApplyBuff` _returnvalue_3)
        (set `self.IsTarotBeenActivated?` false)
        (set `self.HasBuffEnded` false)
        (set `self.IsTarot8WandsActive?` true)))
    (else
      ;;[0.6157 0.8078 1] Archer
      (bind _allequipment_2 (`/Game/TurnBasedJRPGTemplate/Blueprints/Controllers/BP_JRPGFunctionLibrary.GetAllEquipment` (`/Game/TurnBasedJRPGTemplate/Blueprints/Controllers/BP_JRPGPlayerController.Player Unit Data` _asbp_jrpgplayer_controller)))
      (bind (_value_2 _returnvalue_4) (`BlueprintMapLibrary.Map_Find` _playerunits "/Game/TurnBasedJRPGTemplate/Blueprints/Units/PlayerUnits/BP_ArcherPlayerUnit.BP_ArcherPlayerUnit_C"))
      (if (and (`KismetArrayLibrary.Array_Contains` _allequipment_2 "BP_AddHPTarot4_C") _returnvalue_4)
        (if (< (`.currentHP_4_0B53A15447C685E66E26429EA6694AA4` (break `/Game/TurnBasedJRPGTemplate/Blueprints/Structs/S_PlayerUnitData` _value_2)) 125)
          (if (not (`self.IsTarotBeenActivated?`))
            (bind _returnvalue_5 (`GameplayStatics.GetActorOfClass` "/Game/TurnBasedJRPGTemplate/Blueprints/Skills/Buffs/BP_BuffAddSpeed.BP_BuffAddSpeed_C"))
            (`/Game/TurnBasedJRPGTemplate/Blueprints/Skills/Buffs/BP_BuffBase.OnBuffEnded` _returnvalue_5)
            (set `self.IsTarotBeenActivated?` true)
            (set `self.HasBuffEnded` true)
            (set `self.IsTarot8WandsActive?` false))
          (elif (`self.HasBuffEnded`)
            (bind _returnvalue_6 (`GameplayStatics.GetActorOfClass` "/Game/TurnBasedJRPGTemplate/Blueprints/Skills/Buffs/BP_BuffAddSpeed.BP_BuffAddSpeed_C"))
            (`/Game/TurnBasedJRPGTemplate/Blueprints/Skills/Buffs/BP_BuffBase.ApplyBuff` _returnvalue_6)
            (set `self.IsTarotBeenActivated?` false)
            (set `self.HasBuffEnded` false)
            (set `self.IsTarot8WandsActive?` true)))))))

(event `self.ReceiveBeginPlay`
  ;[1 1 1] Set Class Defaults Max HP to zero on start
  (`parent.ReceiveBeginPlay`))

(event `AddHPTarot4`
  ;[1 1 1] Add Tarot HP
)

(event `RemoveHPTarot4`
  ;[1 1 1] Remove Tarot HP
)

(fn `StatGet`
  (params (StatType :type "/Game/TurnBasedJRPGTemplate/Blueprints/Conditions/E_StatType Enum" :default "NewEnumerator0") (Stats :type "/Game/TurnBasedJRPGTemplate/Blueprints/Structs/S_PlayerUnitData Structure"))
  (returns (Stat :type Integer))
  (switch `/Game/TurnBasedJRPGTemplate/Blueprints/Conditions/E_StatType` StatType
    (:`NewEnumerator0`
      (return Stats_currentHP_4_0B53A15447C685E66E26429EA6694AA4))))

(fn `UserConstructionScript`
  (`parent.UserConstructionScript`))