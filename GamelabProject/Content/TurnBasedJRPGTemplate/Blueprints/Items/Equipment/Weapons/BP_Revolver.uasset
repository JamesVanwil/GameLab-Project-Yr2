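; BP_Revolver is a revolver weapon in the turn-based JRPG template that draws on bullets from the player's miscellaneous items.
; On every Tick, after the parent logic, it checks the player controller's MiscItems and removes one BP_Bullet if any remain.
; With no bullets, it sets min and max attack to half the class-default values on the stats struct read from its class defaults.
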(event `self.ReceiveTick`
  (params (DeltaSeconds :type "Float (single-precision)"))
  (bind _stats (defaults `/Game/TurnBasedJRPGTemplate/Blueprints/Items/Equipment/Weapons/BP_Revolver` "BP_Revolver_C"))
  (bind ((`minAttack_14_0D64A0224152A597434ECDAF6DFC9964` _minattack) (`maxAttack_15_24D8527844E2DFB657716C9F16A4AE21` _maxattack)) (break `/Game/TurnBasedJRPGTemplate/Blueprints/Structs/S_UnitStats` _stats))
  (`parent.ReceiveTick` DeltaSeconds)
  (bind _asbp_jrpgplayer_controller (cast `/Game/TurnBasedJRPGTemplate/Blueprints/Controllers/BP_JRPGPlayerController` (`GameplayStatics.GetPlayerController` 0)))
  (if (> (`BlueprintMapLibrary.Map_Find` (`/Game/TurnBasedJRPGTemplate/Blueprints/Controllers/BP_JRPGPlayerController.miscItems` _asbp_jrpgplayer_controller) "/Game/TurnBasedJRPGTemplate/Blueprints/Items/MiscItems/BP_Bullet.BP_Bullet_C") 0)
    (bind _asbp_jrpgplayer_controller_2 (cast `/Game/TurnBasedJRPGTemplate/Blueprints/Controllers/BP_JRPGPlayerController` (`GameplayStatics.GetPlayerController` 0)))
    (`/Game/TurnBasedJRPGTemplate/Blueprints/Controllers/BP_JRPGPlayerController.RemoveMiscItem` _asbp_jrpgplayer_controller_2 "/Game/TurnBasedJRPGTemplate/Blueprints/Items/MiscItems/BP_Bullet.BP_Bullet_C" 1)
    (else
      (setmembers `/Game/TurnBasedJRPGTemplate/Blueprints/Structs/S_UnitStats` :`StructRef` _stats :`minAttack` (/ _minattack 2) :`maxAttack` (/ _maxattack 2)))))

(fn `UserConstructionScript`
  (`parent.UserConstructionScript`))