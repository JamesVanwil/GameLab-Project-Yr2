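; BP_WinchesterWeapon is a JRPG weapon that toggles the Winchester buff based on equip state and bullet supply.
; On Tick, after a short Delay, it applies the existing BP_WinchesterBuff actor once if the player controller reports it equipped with bullets.
; An applied buff ends only when bullets run out.
; Unequipping with bullets left loops back through the delayed check instead of removing the buff.
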(event `self.ReceiveTick`
  (params (DeltaSeconds :type "Float (single-precision)"))
  (`parent.ReceiveTick` DeltaSeconds)
  (bind _asbp_jrpgplayer_controller (cast `/Game/TurnBasedJRPGTemplate/Blueprints/Controllers/BP_JRPGPlayerController` (`GameplayStatics.GetPlayerController` 0) :!label _label))
  (`KismetSystemLibrary.Delay` 0.2)
  (if (and (`/Game/TurnBasedJRPGTemplate/Blueprints/Controllers/BP_JRPGPlayerController.WinchesterEquiped` _asbp_jrpgplayer_controller) (> (`BlueprintMapLibrary.Map_Find` (`/Game/TurnBasedJRPGTemplate/Blueprints/Controllers/BP_JRPGPlayerController.miscItems` _asbp_jrpgplayer_controller) "/Game/TurnBasedJRPGTemplate/Blueprints/Items/MiscItems/BP_Bullet.BP_Bullet_C") 0))
    (if (not (`self.HasBuffBeenApplied`))
      (bind _returnvalue (`GameplayStatics.GetActorOfClass` "/Game/TurnBasedJRPGTemplate/Blueprints/Skills/Buffs/BP_WinchesterBuff.BP_WinchesterBuff_C"))
      (`/Game/TurnBasedJRPGTemplate/Blueprints/Skills/Buffs/BP_BuffBase.ApplyBuff` _returnvalue)
      (set `self.HasBuffBeenApplied` true))
    (elif (`self.HasBuffBeenApplied`)
      (bind _asbp_jrpgplayer_controller_2 (cast `/Game/TurnBasedJRPGTemplate/Blueprints/Controllers/BP_JRPGPlayerController` (`GameplayStatics.GetPlayerController` 0)))
      (if (> (`BlueprintMapLibrary.Map_Find` (`/Game/TurnBasedJRPGTemplate/Blueprints/Controllers/BP_JRPGPlayerController.miscItems` _asbp_jrpgplayer_controller_2) "/Game/TurnBasedJRPGTemplate/Blueprints/Items/MiscItems/BP_Bullet.BP_Bullet_C") 0)
        (goto _label)
        (else
          (bind _returnvalue_2 (`GameplayStatics.GetActorOfClass` "/Game/TurnBasedJRPGTemplate/Blueprints/Skills/Buffs/BP_WinchesterBuff.BP_WinchesterBuff_C"))
          (`/Game/TurnBasedJRPGTemplate/Blueprints/Skills/Buffs/BP_BuffBase.OnBuffEnded` _returnvalue_2)
          (set `self.HasBuffBeenApplied` false))))))

(fn `UserConstructionScript`
  (`parent.UserConstructionScript`))