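; BP_Condition is a condition Blueprint in the turn-based JRPG template that tests a value against a threshold.
; ConditionalCheck switches on its Condition setting, compares the passed Value with Threshold and returns HasMetCondition.
; The two Smaller cases negate the Greater comparisons, so their boundaries are swapped: Smaller Than passes on equality, while Smaller or Equal to fails on it.
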(fn `ConditionalCheck`
  (params (Value :type Integer))
  (returns (Check :type Boolean))
  (locals (HasMetCondition :type Boolean))
  (bind _threshold (`self.Threshold`))
  (bind _returnvalue (> Value _threshold))
  (bind _returnvalue_2 (>= Value _threshold))
  (switch `/Game/TurnBasedJRPGTemplate/Blueprints/Conditions/E_Conditions` (`self.Condition`)
    (:`NewEnumerator0`
      (set `local.HasMetCondition` (== _threshold Value)))
    (:`NewEnumerator1`
      (set `local.HasMetCondition` _returnvalue))
    (:`NewEnumerator2`
      (set `local.HasMetCondition` _returnvalue_2))
    (:`NewEnumerator3`
      (set `local.HasMetCondition` (not _returnvalue)))
    (:`NewEnumerator4`
      (set `local.HasMetCondition` (not _returnvalue_2))))
  (return (`local.HasMetCondition`)))