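; BP_RadioSavePoint is a radio interactable that sends the player's mage character to a fixed location, apparently the Void.
; On BeginPlay it binds to its child-actor interaction detector, enables interaction and refreshes the controller's interactions.
; Interacting sets a used flag, stops the audio manager's environment sound, teleports the mage and shows void text for a few seconds.
; Despite the name, no save logic appears here.
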(event `self.ReceiveBeginPlay`
  (bind _as_bp_interaction_detector (`self.As BP Interaction Detector`))
  (bind _asbp_interaction_detector (cast `/Game/TurnBasedJRPGTemplate/Blueprints/Interactables/BP_InteractionDetector` (`ChildActorComponent.ChildActor` (`self.InteractionActor`))))
  (bind _output_get (set `self.As BP Interaction Detector` _asbp_interaction_detector))
  (add `/Game/TurnBasedJRPGTemplate/Blueprints/Interactables/BP_InteractionDetector.OnInteracted` _output_get (delegate `TP Player`))
  (`/Game/TurnBasedJRPGTemplate/Blueprints/Interactables/BP_InteractionDetector.EnableInteraction` _as_bp_interaction_detector)
  (`/Game/TurnBasedJRPGTemplate/Blueprints/Controllers/BP_JRPGPlayerController.RefreshInteractions` (`/Game/TurnBasedJRPGTemplate/Blueprints/Interactables/BP_InteractionDetector.jRPGPlayerController` _as_bp_interaction_detector)))

(event `TP Player`
  (bind _asbp_mage_character (cast `/Game/TurnBasedJRPGTemplate/Blueprints/PlayerPawns/BP_MageCharacter` (`GameplayStatics.GetPlayerCharacter` 0)))
  (set `self.RadioSavePoint1Used` true)
  (bind _returnvalue (`GameplayStatics.GetActorOfClass` "/Game/BP_AudioManager.BP_AudioManager_C"))
  (`AudioComponent.Stop` (`/Game/BP_AudioManager.EnvriomentSoundRef` _returnvalue))
  (`self.K2_TeleportTo` _asbp_mage_character (-110.0 11100.0 480.0) (struct :`Yaw` -130.0))
  (bind _returnvalue_2 (`|CreateWidget` "/Game/TheVoid/WBP_VoidText.WBP_VoidText_C"))
  (`UserWidget.AddToViewport` _returnvalue_2 0)
  (bind _thevoidtxt (`/Game/TheVoid/WBP_VoidText.TheVoidTxt` _returnvalue_2))
  (`Widget.SetVisibility` _thevoidtxt "Visible")
  (`KismetSystemLibrary.Delay` 3.0)
  (`Widget.SetVisibility` _thevoidtxt "Hidden"))

(fn `UserConstructionScript`
  (`parent.UserConstructionScript`))