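; BP_RadioSavePoint2 is a radio interactable that sends the mage player to a fixed location presented as "the Void".
; It binds TPPlayer to its child interaction detector, which plays an animated transition widget before marking the radio used, stopping environment sound and teleporting the player.
; It then applies a shield overlay material and briefly shows the Void text.
; A DoOnce blocks re-triggering until interaction is re-enabled at the end.
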(event `self.ReceiveBeginPlay`
  (bind _asbp_interaction_detector (cast `/Game/TurnBasedJRPGTemplate/Blueprints/Interactables/BP_InteractionDetector` (`ChildActorComponent.ChildActor` (`self.InteractionActor`))))
  (bind _output_get (set `self.As BP Interaction Detector` _asbp_interaction_detector))
  (add `/Game/TurnBasedJRPGTemplate/Blueprints/Interactables/BP_InteractionDetector.OnInteracted` _output_get (delegate `TP Player`)))

(event `TP Player`
  (bind _as_bp_interaction_detector (`self.As BP Interaction Detector`))
  (`/Engine/EditorBlueprintResources/StandardMacros.DoOnce` false :!label _label
    (:`Completed`
      (bind _returnvalue (`|CreateWidget` "/Game/WBP_VoidAnimsText.WBP_VoidAnimsText_C"))
      (`UserWidget.AddToViewport` _returnvalue 0)
      (`UserWidget.PlayAnimation` _returnvalue (`/Game/WBP_VoidAnimsText.TextAnim` _returnvalue) 0.0 1 "Forward" 1.0 false)
      (`UserWidget.PlayAnimation` _returnvalue (`/Game/WBP_VoidAnimsText.BackgroundAnim` _returnvalue) 0.0 1 "Forward" 1.0 false)
      (`KismetSystemLibrary.Delay` 2.0)
      (`Widget.RemoveFromParent` _returnvalue)
      (bind _asbp_mage_character (cast `/Game/TurnBasedJRPGTemplate/Blueprints/PlayerPawns/BP_MageCharacter` (`GameplayStatics.GetPlayerCharacter` 0)))
      (set `self.RadioSavePoint2Used` true)
      (bind _returnvalue_2 (`GameplayStatics.GetActorOfClass` "/Game/BP_AudioManager.BP_AudioManager_C"))
      (`AudioComponent.Stop` (`/Game/BP_AudioManager.EnvriomentSoundRef` _returnvalue_2))
      (`self.K2_TeleportTo` _asbp_mage_character (-7115.0 12320.0 625.0) (struct :`Yaw` -130.0))
      (bind _returnvalue_3 (`GameplayStatics.GetActorOfClass` "/Game/TurnBasedJRPGTemplate/Blueprints/PlayerPawns/BP_MageCharacter.BP_MageCharacter_C"))
      (`MeshComponent.SetOverlayMaterial` (`Character.Mesh` _returnvalue_3) "/Game/Effects/Materials/Shield_Material2.Shield_Material2")
      (bind _returnvalue_4 (`|CreateWidget` "/Game/TheVoid/WBP_VoidText.WBP_VoidText_C"))
      (`UserWidget.AddToViewport` _returnvalue_4 0)
      (bind _thevoidtxt (`/Game/TheVoid/WBP_VoidText.TheVoidTxt` _returnvalue_4))
      (`Widget.SetVisibility` _thevoidtxt "Visible")
      (`KismetSystemLibrary.Delay` 3.0)
      (`Widget.SetVisibility` _thevoidtxt "Hidden")
      (`Widget.RemoveFromParent` _returnvalue_4)
      (`/Game/TurnBasedJRPGTemplate/Blueprints/Interactables/BP_InteractionDetector.EnableInteraction` _as_bp_interaction_detector)
      (`/Game/TurnBasedJRPGTemplate/Blueprints/Controllers/BP_JRPGPlayerController.RefreshInteractions` (`/Game/TurnBasedJRPGTemplate/Blueprints/Interactables/BP_InteractionDetector.jRPGPlayerController` _as_bp_interaction_detector))
      (goto _label :!via `Reset`))))

(fn `UserConstructionScript`
  (`parent.UserConstructionScript`))