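; BP_Bullets is an interactable ammo pickup that adds bullets to the player's inventory.
; On BeginPlay it binds to the OnInteracted event of a child-actor BP_InteractionDetector.
; On interaction, the handler, named PickUpBattery, adds six BP_Bullet misc items through BP_JRPGPlayerController, plays an equip sound and destroys the pickup.
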(event `self.ReceiveBeginPlay`
  ;[1 1 1] Interact Setup
  (bind _asbp_interaction_detector (cast `/Game/TurnBasedJRPGTemplate/Blueprints/Interactables/BP_InteractionDetector` (`ChildActorComponent.ChildActor` (`self.InteractionActor`))))
  (bind _output_get (set `self.As BP Interaction Detector` _asbp_interaction_detector))
  (add `/Game/TurnBasedJRPGTemplate/Blueprints/Interactables/BP_InteractionDetector.OnInteracted` _output_get (delegate `PickUpBattery`)))

(event `PickUpBattery`
  ;[1 1 1] Interact Setup
  (bind _asbp_jrpgplayer_controller (cast `/Game/TurnBasedJRPGTemplate/Blueprints/Controllers/BP_JRPGPlayerController` (`GameplayStatics.GetPlayerController` 0)))
  (`/Game/TurnBasedJRPGTemplate/Blueprints/Controllers/BP_JRPGPlayerController.AddMiscItemToInventory` _asbp_jrpgplayer_controller "/Game/TurnBasedJRPGTemplate/Blueprints/Items/MiscItems/BP_Bullet.BP_Bullet_C" 6)
  (`GameplayStatics.PlaySound2D` "/Game/Audio/equipmaxingShort.equipmaxingShort" 1.0 1.0 0.0 null null)
  (`self.K2_DestroyActor`))

(fn `UserConstructionScript`)