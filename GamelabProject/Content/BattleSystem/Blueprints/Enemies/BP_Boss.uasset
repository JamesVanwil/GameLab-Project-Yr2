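; Boss enemy actor for the battle system that sends play to the 3EnemyMap level when anything begins overlapping its HitBox.
; Ending the overlap hides the FightUI on the top-down character's HUD, and EnemyDeath destroys the actor.
; PlayerEnemyCombat is an empty event, and the in-place battle setup that shows FightUI, sets enemy health and enables the cursor is disconnected, so it never runs.
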(event `PlayerEnemyCombat`)

(event `self.HitBox.OnComponentBeginOverlap`
  (params (OverlappedComponent :type "PrimitiveComponent Object Reference") (OtherActor :type "Actor Object Reference") (OtherComp :type "PrimitiveComponent Object Reference") (OtherBodyIndex :type Integer) (bFromSweep :type Boolean) (SweepResult :type "HitResult Structure (by ref)"))
  (`GameplayStatics.OpenLevel` "3EnemyMap"))

(event `self.HitBox.OnComponentEndOverlap`
  (params (OverlappedComponent :type "PrimitiveComponent Object Reference") (OtherActor :type "Actor Object Reference") (OtherComp :type "PrimitiveComponent Object Reference") (OtherBodyIndex :type Integer))
  (bind _asbp_top_down_character (cast `/Game/TopDown/Blueprints/BP_TopDownCharacter` OtherActor))
  (`Widget.SetVisibility` (`/Game/BattleSystem/Blueprints/BP_HUDEnemy1_Battery.FightUI` (`/Game/TopDown/Blueprints/BP_TopDownCharacter.HUD_Var` _asbp_top_down_character)) "Hidden"))

(event `EnemyDeath`
  (`self.K2_DestroyActor`))

(fn `UserConstructionScript`)