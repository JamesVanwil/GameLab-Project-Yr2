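; BP_Enemy2 is an enemy actor that sends the game into a separate level when its HitBox is overlapped.
; The overlap opens the 1EnemyMap level without filtering the overlapping actor, and EnemyDeath destroys the actor.
; PlayerEnemyCombat is empty, and a disconnected chain that would teleport the player and start the HUD battle UI with a mouse cursor never runs.
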(event `self.HitBox.OnComponentBeginOverlap`
  (params (OverlappedComponent :type "PrimitiveComponent Object Reference") (OtherActor :type "Actor Object Reference") (OtherComp :type "PrimitiveComponent Object Reference") (OtherBodyIndex :type Integer) (bFromSweep :type Boolean) (SweepResult :type "HitResult Structure (by ref)"))
  (`GameplayStatics.OpenLevel` "1EnemyMap"))

(event `PlayerEnemyCombat`)

(event `EnemyDeath`
  (`self.K2_DestroyActor`))

(fn `UserConstructionScript`)