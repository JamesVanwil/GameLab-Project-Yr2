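; BP_Enemy is a battle-system enemy that starts a fight when BP_TopDownCharacter overlaps its HitBox.
; On overlap it teleports the player to its actor-relative TpPosition, shows the HUD's FightUI, calls BattleBegin and enables the mouse cursor.
; End overlap hides FightUI but leaves the cursor enabled, reusing the begin-overlap cast for that controller lookup.
; EnemyDeath destroys the actor, while PlayerEnemyCombat is an empty event.
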(event `PlayerEnemyCombat`)

(event `self.HitBox.OnComponentBeginOverlap`
  (params (OverlappedComponent :type "PrimitiveComponent Object Reference") (OtherActor :type "Actor Object Reference") (OtherComp :type "PrimitiveComponent Object Reference") (OtherBodyIndex :type Integer) (bFromSweep :type Boolean) (SweepResult :type "HitResult Structure (by ref)"))
  (bind (_tpposition_location _tpposition_rotation) (`KismetMathLibrary.BreakTransform` (`self.TpPosition`)))
  (bind _asbp_top_down_character (cast `/Game/TopDown/Blueprints/BP_TopDownCharacter` OtherActor))
  (`self.K2_SetActorLocationAndRotation` _asbp_top_down_character (`KismetMathLibrary.TransformLocation` (`self.GetTransform`) _tpposition_location) _tpposition_rotation false false)
  (bind _hud (`/Game/TopDown/Blueprints/BP_TopDownCharacter.HUD` _asbp_top_down_character))
  (`Widget.SetVisibility` (`/Game/BattleSystem/Blueprints/BP_HUD.FightUI` _hud) "Visible")
  (`/Game/BattleSystem/Blueprints/BP_HUD.BattleBegin` _hud null)
  (set `PlayerController.bShowMouseCursor` true (`PlayerState.GetPlayerController` (`Pawn.PlayerState` _asbp_top_down_character))))

(event `self.HitBox.OnComponentEndOverlap`
  (params (OverlappedComponent :type "PrimitiveComponent Object Reference") (OtherActor :type "Actor Object Reference") (OtherComp :type "PrimitiveComponent Object Reference") (OtherBodyIndex :type Integer))
  (bind _asbp_top_down_character (cast `/Game/TopDown/Blueprints/BP_TopDownCharacter` OtherActor))
  (`Widget.SetVisibility` (`/Game/BattleSystem/Blueprints/BP_HUD.FightUI` (`/Game/TopDown/Blueprints/BP_TopDownCharacter.HUD` _asbp_top_down_character)) "Hidden")
  (set `PlayerController.bShowMouseCursor` true (`PlayerState.GetPlayerController` (`Pawn.PlayerState` (stale `self.HitBox.OnComponentBeginOverlap` _asbp_top_down_character)))))

(event `EnemyDeath`
  (`self.K2_DestroyActor`))

(fn `UserConstructionScript`)