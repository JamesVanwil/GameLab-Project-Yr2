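; BP_VoidTPBack is a trigger that teleports the mage character back from the void to the last radio save point used.
; On box overlap it checks used flags on BP_RadioSavePoint, then BP_RadioSavePoint2, teleporting to that point's hardcoded transform and clearing the flag.
; It then creates a WBP_VoidText widget and shows its Preston's Mansion text briefly before hiding it, without removing the widget.
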(event `self.Box.OnComponentBeginOverlap`
  (params (OverlappedComponent :type "PrimitiveComponent Object Reference") (OtherActor :type "Actor Object Reference") (OtherComp :type "PrimitiveComponent Object Reference") (OtherBodyIndex :type Integer) (bFromSweep :type Boolean) (SweepResult :type "HitResult Structure (by ref)"))
  ;[1 1 1] TP spawn based on radio interacted with
  (bind _asbp_mage_character (cast `/Game/TurnBasedJRPGTemplate/Blueprints/PlayerPawns/BP_MageCharacter` OtherActor))
  (bind _returnvalue (`GameplayStatics.GetActorOfClass` "/Game/TurnBasedJRPGTemplate/Blueprints/Interactables/BP_RadioSavePoint.BP_RadioSavePoint_C"))
  (if (`/Game/TurnBasedJRPGTemplate/Blueprints/Interactables/BP_RadioSavePoint.RadioSavePoint1Used` _returnvalue)
    (`self.K2_TeleportTo` _asbp_mage_character (1110.0 6970.0 200.0) (struct :`Yaw` 90.0))
    (set `/Game/TurnBasedJRPGTemplate/Blueprints/Interactables/BP_RadioSavePoint.RadioSavePoint1Used` false _returnvalue)
    (bind _returnvalue_2 (`|CreateWidget` "/Game/WBP_VoidText.WBP_VoidText_C"))
    (`UserWidget.AddToViewport` _returnvalue_2 0)
    (bind _prestonsmansiontxt (`/Game/WBP_VoidText.PrestonsMansionTxt` _returnvalue_2))
    (`Widget.SetVisibility` _prestonsmansiontxt "Visible")
    (`KismetSystemLibrary.Delay` 3.0)
    (`Widget.SetVisibility` _prestonsmansiontxt "Hidden")
    (else
      (bind _returnvalue_3 (`GameplayStatics.GetActorOfClass` "/Game/TurnBasedJRPGTemplate/Blueprints/Interactables/BP_RadioSavePoint2.BP_RadioSavePoint2_C"))
      (if (`/Game/TurnBasedJRPGTemplate/Blueprints/Interactables/BP_RadioSavePoint2.RadioSavePoint2Used` _returnvalue_3)
        (`self.K2_TeleportTo` _asbp_mage_character (2455.711504 2330.641778 230.0) (struct :`Yaw` -40.0))
        (set `/Game/TurnBasedJRPGTemplate/Blueprints/Interactables/BP_RadioSavePoint2.RadioSavePoint2Used` false _returnvalue_3)
        (bind _returnvalue_4 (`|CreateWidget` "/Game/WBP_VoidText.WBP_VoidText_C"))
        (`UserWidget.AddToViewport` _returnvalue_4 0)
        (bind _prestonsmansiontxt_2 (`/Game/WBP_VoidText.PrestonsMansionTxt` _returnvalue_4))
        (`Widget.SetVisibility` _prestonsmansiontxt_2 "Visible")
        (`KismetSystemLibrary.Delay` 3.0)
        (`Widget.SetVisibility` _prestonsmansiontxt_2 "Hidden")))))

(fn `UserConstructionScript`)