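; BP_AudioGodISHere is a one-shot trigger that announces the god's arrival when BP_MageCharacter overlaps its Box.
; A DoOnce gate plays the Screem_God_Of_Destruction sound in 2D and adds a WBP_FarGodText widget with its GodisHereText shown.
; Delays hide the text after a few seconds, then destroy the trigger actor later, without removing the widget from the viewport.
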(event `self.Box.OnComponentBeginOverlap`
  (params (OverlappedComponent :type "PrimitiveComponent Object Reference") (OtherActor :type "Actor Object Reference") (OtherComp :type "PrimitiveComponent Object Reference") (OtherBodyIndex :type Integer) (bFromSweep :type Boolean) (SweepResult :type "HitResult Structure (by ref)"))
  (cast `/Game/TurnBasedJRPGTemplate/Blueprints/PlayerPawns/BP_MageCharacter` OtherActor)
  (`/Engine/EditorBlueprintResources/StandardMacros.DoOnce` false
    (:`Completed`
      (`GameplayStatics.PlaySound2D` "/Game/Audio/Screem_God_Of_Destruction.Screem_God_Of_Destruction" 1.0 1.0 0.0 null null)
      (bind _returnvalue (`|CreateWidget` "/Game/Audio/AudioUI/WBP_FarGodText.WBP_FarGodText_C"))
      (`UserWidget.AddToViewport` _returnvalue 0)
      (bind _godisheretext (`/Game/Audio/AudioUI/WBP_FarGodText.GodisHereText` _returnvalue))
      (`Widget.SetVisibility` _godisheretext "Visible")
      (`KismetSystemLibrary.Delay` 5.0)
      (`Widget.SetVisibility` _godisheretext "Hidden")
      (`KismetSystemLibrary.Delay` 15.0)
      (`self.K2_DestroyActor`))))

(fn `UserConstructionScript`)