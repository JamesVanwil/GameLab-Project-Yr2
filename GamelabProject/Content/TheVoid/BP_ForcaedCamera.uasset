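; BP_ForcaedCamera is a trigger box that plays a short forced camera view when the mage character enters it.
; On overlap it stops movement and input, saves the camera transform, moves the camera to a hardcoded world location and rotation, and turns the capsule to match.
; After a two-second delay it restores the camera, input and walking mode.
; Nothing disables the trigger, so it can fire again on later overlaps.
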(event `self.Box.OnComponentBeginOverlap`
  (params (OverlappedComponent :type "PrimitiveComponent Object Reference") (OtherActor :type "Actor Object Reference") (OtherComp :type "PrimitiveComponent Object Reference") (OtherBodyIndex :type Integer) (bFromSweep :type Boolean) (SweepResult :type "HitResult Structure (by ref)"))
  (bind _asbp_mage_character (cast `/Game/TurnBasedJRPGTemplate/Blueprints/PlayerPawns/BP_MageCharacter` OtherActor))
  (`CharacterMovementComponent.SetMovementMode` (`Character.CharacterMovement` _asbp_mage_character) "MOVE_None" 0)
  (bind _camera (`/Game/TurnBasedJRPGTemplate/Blueprints/PlayerPawns/BP_JRPGCharacterBase.Camera` _asbp_mage_character))
  (set `self.Camera World Rotation` (`SceneComponent.K2_GetComponentRotation` _camera))
  (set `self.Camera World Location` (`SceneComponent.K2_GetComponentLocation` _camera))
  (`SceneComponent.K2_SetWorldLocationAndRotation` _camera (-1472.214346 10436.945892 670.0) (struct :`Pitch` -15.0 :`Yaw` 140.0) false false)
  (`self.DisableInput` _asbp_mage_character (`GameplayStatics.GetPlayerController` 0))
  (`SceneComponent.K2_SetWorldRotation` (`Character.CapsuleComponent` _asbp_mage_character) (struct :`Yaw` 140.0) false false)
  (`KismetSystemLibrary.Delay` 2.0)
  (`SceneComponent.K2_SetWorldLocationAndRotation` _camera (`self.Camera World Location`) (`self.Camera World Rotation`) false false)
  (`self.EnableInput` _asbp_mage_character (`GameplayStatics.GetPlayerController` 0))
  (`CharacterMovementComponent.SetMovementMode` (`Character.CharacterMovement` _asbp_mage_character) "MOVE_Walking" 0))

(fn `UserConstructionScript`)