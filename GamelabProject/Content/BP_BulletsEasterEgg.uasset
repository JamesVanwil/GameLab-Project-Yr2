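; BP_BulletsEasterEgg is a hidden pickup that rewards the mage character with bullets when touched.
; On sphere overlap with BP_MageCharacter, it calls AddBulletsToInventory on the mage and adds a large BP_Bullet stack through the JRPG player controller.
; It then plays a farewell 2D sound and destroys itself.
; The pickup-prompt widget logic and its delay are disconnected, and end overlap does nothing beyond a cast.
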(event `self.Sphere.OnComponentBeginOverlap`
  (params (OverlappedComponent :type "PrimitiveComponent Object Reference") (OtherActor :type "Actor Object Reference") (OtherComp :type "PrimitiveComponent Object Reference") (OtherBodyIndex :type Integer) (bFromSweep :type Boolean) (SweepResult :type "HitResult Structure (by ref)"))
  (cast `/Game/TurnBasedJRPGTemplate/Blueprints/PlayerPawns/BP_MageCharacter` OtherActor)
  (bind _asbp_mage_character (cast `/Game/TurnBasedJRPGTemplate/Blueprints/PlayerPawns/BP_MageCharacter` OtherActor))
  (`/Game/TurnBasedJRPGTemplate/Blueprints/PlayerPawns/BP_MageCharacter.AddBulletsToInventory` _asbp_mage_character)
  (bind _asbp_jrpgplayer_controller (cast `/Game/TurnBasedJRPGTemplate/Blueprints/Controllers/BP_JRPGPlayerController` (`GameplayStatics.GetPlayerController` 0)))
  (`/Game/TurnBasedJRPGTemplate/Blueprints/Controllers/BP_JRPGPlayerController.AddMiscItemToInventory` _asbp_jrpgplayer_controller "/Game/TurnBasedJRPGTemplate/Blueprints/Items/MiscItems/BP_Bullet.BP_Bullet_C" 69)
  (`GameplayStatics.PlaySound2D` "/Game/Audio/bye-bye-lumi-athena-sfx__mp3cut_net_.bye-bye-lumi-athena-sfx__mp3cut_net_" 1.0 1.0 0.0 null null)
  (`self.K2_DestroyActor`))

(event `self.Sphere.OnComponentEndOverlap`
  (params (OverlappedComponent :type "PrimitiveComponent Object Reference") (OtherActor :type "Actor Object Reference") (OtherComp :type "PrimitiveComponent Object Reference") (OtherBodyIndex :type Integer))
  (cast `/Game/TurnBasedJRPGTemplate/Blueprints/PlayerPawns/BP_MageCharacter` OtherActor))

(fn `UserConstructionScript`)