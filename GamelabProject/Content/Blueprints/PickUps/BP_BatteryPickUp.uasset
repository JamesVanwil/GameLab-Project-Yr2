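; BP_BatteryPickUp is a battery pickup that the mage character collects through interaction.
; On BeginPlay it casts its InteractionActor child actor to BP_InteractionDetector and binds PickUpBattery to that detector's OnInteracted event.
; PickUpBattery finds the BP_MageCharacter, calls its BatteryPickUp and destroys the pickup.
; The Box overlap events are empty; older overlap-driven prompt and pickup logic remains disconnected.
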(event `self.ReceiveBeginPlay`
  ;[1 1 1] Setup Interaction
  (bind _asbp_interaction_detector (cast `/Game/TurnBasedJRPGTemplate/Blueprints/Interactables/BP_InteractionDetector` (`ChildActorComponent.ChildActor` (`self.InteractionActor`))))
  (bind _output_get (set `self.As BP Interaction Detector` _asbp_interaction_detector))
  (add `/Game/TurnBasedJRPGTemplate/Blueprints/Interactables/BP_InteractionDetector.OnInteracted` _output_get (delegate `PickUpBattery`)))

(event `PickUpBattery`
  ;[1 1 1] Setup Interaction
  (bind _returnvalue (`GameplayStatics.GetActorOfClass` "/Game/TurnBasedJRPGTemplate/Blueprints/PlayerPawns/BP_MageCharacter.BP_MageCharacter_C"))
  (`/Game/TurnBasedJRPGTemplate/Blueprints/PlayerPawns/BP_MageCharacter.BatteryPickUp` _returnvalue)
  (`self.K2_DestroyActor`))

(event `self.Box.OnComponentBeginOverlap`
  (params (OverlappedComponent :type "PrimitiveComponent Object Reference") (OtherActor :type "Actor Object Reference") (OtherComp :type "PrimitiveComponent Object Reference") (OtherBodyIndex :type Integer) (bFromSweep :type Boolean) (SweepResult :type "HitResult Structure (by ref)"))
  ;[1 1 1] Detect Collision and call Function
)

(event `self.Box.OnComponentEndOverlap`
  (params (OverlappedComponent :type "PrimitiveComponent Object Reference") (OtherActor :type "Actor Object Reference") (OtherComp :type "PrimitiveComponent Object Reference") (OtherBodyIndex :type Integer)))

(fn `UserConstructionScript`)