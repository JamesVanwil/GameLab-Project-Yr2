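; Interactive door that the mage character opens and closes with the Interact input while inside its Box trigger.
; Box overlap enables and disables input, and a FlipFlop plays or reverses a timeline that drives the door's yaw.
; Each press also destroys an NPC_Base_HumanDoorLockedOneSide actor and clears DoorOpening just before testing it, so that guard never blocks.
; The interaction prompt show/hide nodes are disconnected and never run.
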(event `self.Box.OnComponentBeginOverlap`
  (params (OverlappedComponent :type "PrimitiveComponent Object Reference") (OtherActor :type "Actor Object Reference") (OtherComp :type "PrimitiveComponent Object Reference") (OtherBodyIndex :type Integer) (bFromSweep :type Boolean) (SweepResult :type "HitResult Structure (by ref)"))
  ;[1 1 1] Door Logic
  (cast `/Game/TurnBasedJRPGTemplate/Blueprints/PlayerPawns/BP_MageCharacter` OtherActor)
  (`self.EnableInput` (`GameplayStatics.GetPlayerController` 0)))

(event `self.Box.OnComponentEndOverlap`
  (params (OverlappedComponent :type "PrimitiveComponent Object Reference") (OtherActor :type "Actor Object Reference") (OtherComp :type "PrimitiveComponent Object Reference") (OtherBodyIndex :type Integer))
  ;[1 1 1] Door Logic
  (cast `/Game/TurnBasedJRPGTemplate/Blueprints/PlayerPawns/BP_MageCharacter` OtherActor)
  (`self.DisableInput` (`GameplayStatics.GetPlayerController` 0)))

(event `InputAction|Interact`
  (params (Key :type "Key Structure"))
  (:`Pressed`
    (bind _returnvalue (`GameplayStatics.GetActorOfClass` "/Game/DialogueSystem/Blueprints/NPC_Base_HumanDoorLockedOneSide.NPC_Base_HumanDoorLockedOneSide_C"))
    (`self.K2_DestroyActor` _returnvalue)
    ;[1 1 1] Door Logic
    (set `self.bDoorOpening?` false)
    (if (not (`self.bDoorOpening?`))
      (`/Engine/EditorBlueprintResources/StandardMacros.FlipFlop`
        (:`A`
          (bind (_direction _newtrack_0) (`Timeline|DoorRotateTimeline` :!via `PlayFromStart` :!label _label)
            (:`Update`
              (set `self.bDoorOpening?` true)
              (`SceneComponent.K2_SetRelativeRotation` (`self.Door`) (`KismetMathLibrary.MakeRotator` 0.0 0.0 _newtrack_0) false false))))
        (:`B`
          (goto _label :!via `ReverseFromEnd`))))))

(fn `UserConstructionScript`)