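; Combat component that runs a battle unit's timed turns, actions and damage math.
; Level-based table stats load at BeginPlay, and a haste-scaled timer requests turns from the battle game mode.
; On its turn, a party unit opens an action HUD, while others attack a random party member.
; Actions chain AI moves and montages, spawn spells on notifies, then return the unit to its battle position and restart the timer.
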(event `self.ReceiveBeginPlay`
  (bind _asunitbase (cast `/Game/ImportStuff/Unitbase` (`self.GetOwner`)))
  (bind _output_get (set `self.UnitCharacter` _asunitbase))
  (set `self.BattlePosition` (`Actor.GetTransform` _output_get))
  (bind _returnvalue (`|GetDataTableRow` "/Game/ImportStuff/BaseStat_Table.BaseStat_Table" (`KismetStringLibrary.Conv_StringToName` (`KismetStringLibrary.Conv_IntToString` (`self.UnitLevel`))))
    (:`then`
      (set `self.BaseUnitStats` _returnvalue)
      (`self.BeginBattle`))))

(event `MeleeAttack`
  (`|AIMoveTo` (`self.UnitCharacter`) (0.0 0.0 0.0) (`self.UnitTarget`) 100.0
    (:`then`
      (bind _actionswindow (`self.ActionsWindow`)
        (:`then`
          (`Widget.RemoveFromParent` _actionswindow))
        (:`else`)))
    (:`OnSuccess`
      (`|PlayMontage` (`Character.Mesh` (`self.UnitCharacter`)) (`self.AttackMontage`)
        (:`OnCompleted`
          (`|AIMoveTo` (`self.UnitCharacter`) (.location (`self.BattlePosition`)) null
            (:`OnSuccess`
              (`AIController.K2_SetFocus` (`AIBlueprintHelperLibrary.GetAIController` (`self.UnitCharacter`)) (`self.UnitTarget`))
              (`KismetSystemLibrary.Delay` 2.0)
              (`self.EndUnitTurn`))))))))

(event `CastBlackMagic`
  (params (BlackMagicSpell :type "/Game/ImportStuff/Abilities/Magic/MagicBase Class Reference"))
  (bind _unittarget (`self.UnitTarget`))
  (`|AIMoveTo` (`self.UnitCharacter`) (`self.GetRangePosition` true) null 100.0
    (:`then`
      (bind _actionswindow (`self.ActionsWindow`)
        (:`then`
          (`Widget.RemoveFromParent` _actionswindow))
        (:`else`)))
    (:`OnSuccess`
      (`|PlayMontage` (`Character.Mesh` (`self.UnitCharacter`)) (`self.MagicCastMontage`)
        (:`OnCompleted`
          (`|AIMoveTo` (`self.UnitCharacter`) (.location (`self.BattlePosition`)) null
            (:`OnSuccess`
              (`AIController.K2_SetFocus` (`AIBlueprintHelperLibrary.GetAIController` (`self.UnitCharacter`)) (`self.UnitTarget`))
              (`KismetSystemLibrary.Delay` 2.0)
              (`self.EndUnitTurn`))))
        (:`OnNotifyBegin`
          (`|SpawnActorFromClass` BlackMagicSpell (`Actor.GetTransform` _unittarget) "Undefined" "MultiplyWithRoot" null _unittarget (`self.UnitCharacter`)))))))

(event `AttackCommand`
  (message `/Game/ImportStuff/DynamicCameraInterface.SetOrbit` (`Controller.GetViewTarget` (`GameplayStatics.GetPlayerController` 0)) false)
  (if (`self.IsRangedCharacter`)
    (`self.RangedAttack`)
    (else
      (`self.MeleeAttack`))))

(event `MagicCommand`
  (params (MagicClass :type "/Game/ImportStuff/Abilities/Magic/MagicBase Class Reference"))
  (message `/Game/ImportStuff/DynamicCameraInterface.SetOrbit` (`Controller.GetViewTarget` (`GameplayStatics.GetPlayerController` 0)) false)
  (if (`KismetMathLibrary.ClassIsChildOf` MagicClass "/Game/ImportStuff/Abilities/Magic/BlackMagic/BlackMagicBase.BlackMagicBase_C")
    (`self.CastBlackMagic` MagicClass)
    (else
      (`self.CastWhiteMagic` MagicClass))))

(event `RangedAttack`
  (`|AIMoveTo` (`self.UnitCharacter`) (`self.GetRangePosition` true) null 100.0
    (:`then`
      (bind _actionswindow (`self.ActionsWindow`)
        (:`then`
          (`Widget.RemoveFromParent` _actionswindow))
        (:`else`)))
    (:`OnSuccess`
      (`KismetSystemLibrary.Delay` 2.0)
      (`|AIMoveTo` (`self.UnitCharacter`) (.location (`self.BattlePosition`)) null
        (:`OnSuccess`
          (`AIController.K2_SetFocus` (`AIBlueprintHelperLibrary.GetAIController` (`self.UnitCharacter`)) (`self.UnitTarget`))
          (`KismetSystemLibrary.Delay` 2.0)
          (`self.EndUnitTurn`))))))

(event `CastWhiteMagic`
  (params (Ability :type "/Game/ImportStuff/Abilities/Magic/MagicBase Class Reference"))
  (bind _unittarget (`self.UnitTarget`))
  (bind _location (.location (`self.BattlePosition`)))
  (`|AIMoveTo` (`self.UnitCharacter`) (`self.GetRangePosition` false) null 100.0
    (:`then`
      (bind _actionswindow (`self.ActionsWindow`)
        (:`then`
          (`Widget.RemoveFromParent` _actionswindow))
        (:`else`)))
    (:`OnSuccess`
      (`|PlayMontage` (`Character.Mesh` (`self.UnitCharacter`)) (`self.MagicCastMontage`)
        (:`OnCompleted`
          (`|AIMoveTo` (`self.UnitCharacter`) _location null
            (:`OnSuccess`
              (`AIController.K2_SetFocalPoint` (`AIBlueprintHelperLibrary.GetAIController` (`self.UnitCharacter`)) (+ _location (* (`KismetMathLibrary.GetForwardVector` (.rotation (`self.BattlePosition`))) 100.0)))
              (`KismetSystemLibrary.Delay` 2.0)
              (`self.EndUnitTurn`))))
        (:`OnNotifyBegin`
          (`|SpawnActorFromClass` Ability (`Actor.GetTransform` _unittarget) "Undefined" "MultiplyWithRoot" null _unittarget (`self.UnitCharacter`)))))))

(fn `BeginBattle`
  (bind _returnvalue (`KismetSystemLibrary.K2_SetTimer` self "RequestTurn" (+ (* (- 1.0 (`KismetMathLibrary.NormalizeToRange` (* (`.HST_14_F49810064D771D7E30D186B469A02B39` (break `/Game/ImportStuff/StatTable_ST` (`self.BaseUnitStats`))) (`.HST_23_F49810064D771D7E30D186B469A02B39` (break `/Game/ImportStuff/StatModifier` (`self.UnitStatModifier`)))) 0.0 255.0)) (- (`self.MaxActionTime`) (`self.MinActionTime`))) (`self.MinActionTime`))))
  (set `self.ActionTimer` _returnvalue))

(fn `CalculateBaseDamage`
  (returns (CalculatedDamage :type "Float (double-precision)"))
  (return (* (* (* (`.STR_9_1709A2724AD13E282AAAF78BB91BC5D0` (break `/Game/ImportStuff/StatTable_ST` (`self.BaseUnitStats`))) (`.STR_20_1709A2724AD13E282AAAF78BB91BC5D0` (break `/Game/ImportStuff/StatModifier` (`self.UnitStatModifier`)))) 2.0) (`KismetMathLibrary.RandomFloatInRange` 1.0 3.0))))

(fn `CalculateDamage`
  (returns (BaseDamage :type "Float (double-precision)"))
  (bind _calculateddamage (`self.CalculateBaseDamage`))
  (return _calculateddamage))

(fn `CalculateDamageResistance`
  (params (BaseDamage :type "Float (double-precision)"))
  (returns (NewDamage :type "Float (double-precision)"))
  (return (/ (`KismetMathLibrary.MultiplyMultiply_FloatFloat` BaseDamage 2.0) (+ BaseDamage (* (`.RES_18_0E5D1E3E4DCD2AD256DFF19A2F2F738F` (break `/Game/ImportStuff/StatTable_ST` (`self.BaseUnitStats`))) (`.RES_25_0E5D1E3E4DCD2AD256DFF19A2F2F738F` (break `/Game/ImportStuff/StatModifier` (`self.UnitStatModifier`))))))))

(fn `CalculateMagicBaseDamage`
  (params (SpellClass :type "/Game/ImportStuff/Abilities/Magic/MagicBase Class Reference"))
  (returns (ReturnValue :type "Float (double-precision)"))
  (bind (_abilityname _rank _spelltarget _spellpower) (defaults `Object` (`local.SpellClass`)))
  (return (* (* (`.WIS_17_F37BED824D2DB82ED06DA587CF4C54E3` (break `/Game/ImportStuff/StatTable_ST` (`self.BaseUnitStats`))) (`.WIS_24_F37BED824D2DB82ED06DA587CF4C54E3` (break `/Game/ImportStuff/StatModifier` (`self.UnitStatModifier`)))) (* (`KismetMathLibrary.Sqrt` (`BlueprintMapLibrary.Map_Find` _spellpower _rank)) 2.0))))

(fn `EndUnitTurn`
  (`self.TurnEnded`)
  (`/Engine/EditorBlueprintResources/StandardMacros.IsValid` (`AIBlueprintHelperLibrary.GetAIController` (`self.UnitCharacter`))
    (:`Is Valid`
      (`self.BeginBattle`)
      (`AIController.K2_ClearFocus` (`AIBlueprintHelperLibrary.GetAIController` (`self.UnitTarget`))))))

(fn `GetRangePosition`
  (params (TargetingEnemy :type Boolean :default true))
  (returns (ReturnValue :type "Vector Structure"))
  (bind _unittarget (`self.UnitTarget`))
  (bind _returnvalue (`Actor.K2_GetActorLocation` (`self.UnitCharacter`)))
  (return (`KismetMathLibrary.SelectVector` (+ _returnvalue (* (`KismetMathLibrary.GetDirectionUnitVector` _returnvalue (`Actor.K2_GetActorLocation` (`self.UnitTarget`))) 500.0)) (+ (`Actor.K2_GetActorLocation` _unittarget) (* (`Actor.GetActorForwardVector` _unittarget) 500.0)) TargetingEnemy)))

(fn `RequestTurn`
  (`/Engine/EditorBlueprintResources/StandardMacros.IsValid` (`AIBlueprintHelperLibrary.GetAIController` (`self.UnitCharacter`))
    (:`Is Valid`
      (bind _asbp_battle_game_mode (cast `/Game/ImportStuff/BP_BattleGameMode` (`GameplayStatics.GetGameMode`)))
      (`/Game/ImportStuff/BP_BattleGameMode.TurnRequest` _asbp_battle_game_mode (`self.UnitCharacter`)))))

(fn `SetCamera`
  (bind _returnvalue (`GameplayStatics.GetActorOfClass` "/Game/ImportStuff/DynamicCamera.DynamicCamera_C"))
  (`PlayerController.SetViewTargetWithBlend` (`GameplayStatics.GetPlayerController` 0) _returnvalue 0.0 "VTBlend_Linear" 0.0 false)
  (message `/Game/ImportStuff/DynamicCameraInterface.SetDynamicLoaction` _returnvalue (`self.UnitCharacter`) (0.0 0.0 0.0))
  (message `/Game/ImportStuff/DynamicCameraInterface.SetOrbit` (`Controller.GetViewTarget` (`GameplayStatics.GetPlayerController` 0)) true))

(fn `StartUnitTurn`
  (`/Engine/EditorBlueprintResources/StandardMacros.IsValid` (`AIBlueprintHelperLibrary.GetAIController` (`self.UnitCharacter`))
    (:`Is Valid`
      (if (`KismetMathLibrary.ClassIsChildOf` (`GameplayStatics.GetObjectClass` (`self.UnitCharacter`)) "/Game/ImportStuff/PartyUnitBase.PartyUnitBase_C")
        (bind _returnvalue (`|CreateWidget` "/Game/ImportStuff/UI/WIdgets/W_UnitBattleHUD.W_UnitBattleHUD_C" null (`self.UnitCharacter`)))
        (bind _output_get (set `self.ActionsWindow` _returnvalue))
        (`UserWidget.AddToViewport` _output_get 0)
        (`self.SetCamera`)
        (else
          (bind _outactors (`GameplayStatics.GetAllActorsOfClass` "/Game/ImportStuff/PartyUnitBase.PartyUnitBase_C"))
          (set `self.UnitTarget` (`KismetArrayLibrary.Array_Random` _outactors))
          (switch `int` 0
            (:`0`
              (`self.AttackCommand`)
              (`self.SetCamera`))))))
    (:`Is Not Valid`
      (`self.EndUnitTurn`))))