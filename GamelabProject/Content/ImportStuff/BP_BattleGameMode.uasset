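; Battle game mode that runs queued turn-based combat between party and enemy units.
; On BeginPlay it sets the top-down camera, gathers both sides and adds party members to the battle HUD.
; Turn requests join a unique queue; a DoOnce gate starts one unit's turn at a time through its combat component.
; Removing the last enemy triggers victory: camera switch, party montages and loading TopDownMap, with no defeat check.
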(event `self.ReceiveBeginPlay`
  (bind _returnvalue (`GameplayStatics.GetActorOfClass` "/Game/ImportStuff/BP_CameraTopDown.BP_CameraTopDown_C"))
  (bind _output_get (set `self.MainBattleCamera` _returnvalue))
  (`PlayerController.SetViewTargetWithBlend` (`GameplayStatics.GetPlayerController` 0) _output_get 0.0 "VTBlend_Linear" 0.0 false)
  (bind _outactors (`GameplayStatics.GetAllActorsOfClass` "/Game/ImportStuff/PartyUnitBase.PartyUnitBase_C"))
  (set `self.PartyUnits` _outactors)
  (bind _outactors_2 (`GameplayStatics.GetAllActorsOfClass` "/Game/ImportStuff/EnemyUnitBase.EnemyUnitBase_C"))
  (set `self.EnemyUnits` _outactors_2)
  (`KismetSystemLibrary.Delay` 0.2)
  (bind _asbp_battle_player_controller (cast `/Game/ImportStuff/BP_BattlePlayerController` (`GameplayStatics.GetPlayerController` 0)))
  (set `self.Battle HUD` (`/Game/ImportStuff/BP_BattlePlayerController.BattleHUD` _asbp_battle_player_controller))
  (for _array_element (`self.PartyUnits`)
    (`/Game/ImportStuff/UI/WIdgets/W_HUDDisplay.AddPartyUnitToHUD` (`self.Battle HUD`) _array_element)))

(event `TurnRequest`
  (params (Unit :type "/Game/ImportStuff/Unitbase Object Reference"))
  (`KismetArrayLibrary.Array_AddUnique` (`self.TurnOrder`) Unit)
  (`self.StartTurn`))

(event `StartTurn`
  (bind _output (`|GetArrayItem` (`self.TurnOrder`)))
  (bind _bp_combatcomponent (`/Game/ImportStuff/Unitbase.BP_CombatComponent` _output))
  (if (not (`self.IsBattleComplete`))
    (`/Engine/EditorBlueprintResources/StandardMacros.DoOnce` false :!label _label
      (:`Completed`
        (if (`KismetArrayLibrary.Array_IsValidIndex` (`self.TurnOrder`))
          (`/Engine/EditorBlueprintResources/StandardMacros.IsValid` (`AIBlueprintHelperLibrary.GetAIController` _output)
            (:`Is Valid`
              (`/Game/ImportStuff/BP_CombatComponent.StartUnitTurn` _bp_combatcomponent)
              (set `self.CurrentUnit` _output)
              (add `/Game/ImportStuff/BP_CombatComponent.TurnEnded` _bp_combatcomponent (`|CreateDelegate` :!event `ReadyNextTurn`))
              (`KismetArrayLibrary.Array_Remove` (`self.TurnOrder`)))
            (:`Is Not Valid`
              (`self.ReadyNextTurn`)
              (`KismetArrayLibrary.Array_Remove` (`self.TurnOrder`))))
          (else
            (`self.ReadyNextTurn`)))))))

(event `ReadyNextTurn`
  (`|ExecutionSequence`
    (:`then_0`
      (goto _label :!via `Reset`))
    (:`then_1`
      (`KismetSystemLibrary.Delay` 0.5)
      (if (`KismetArrayLibrary.Array_IsValidIndex` (`self.TurnOrder`))
        (`self.StartTurn`)))))

(fn `InitiateVictory`
  (bind _returnvalue (`GameplayStatics.GetActorOfClass` "/Game/ImportStuff/VictoryCamera.VictoryCamera_C"))
  (`PlayerController.SetViewTargetWithBlend` (`GameplayStatics.GetPlayerController` 0) _returnvalue 0.0 "VTBlend_Linear" 0.0 false)
  (for _array_element (`self.PartyUnits`)
    (`Character.PlayAnimMontage` _array_element (`/Game/ImportStuff/Unitbase.VictoryAnim` _array_element) 1.0 "None")
    (`GameplayStatics.OpenLevel` "TopDownMap"))
  (set `self.IsBattleComplete` true))

(fn `RemoveUnitFromBattle`
  (params (Unit :type "/Game/ImportStuff/Unitbase Object Reference"))
  (bind _asenemy_unit_base (cast `/Game/ImportStuff/EnemyUnitBase` Unit)
    (:`then`
      (`KismetArrayLibrary.Array_RemoveItem` (`self.EnemyUnits`) _asenemy_unit_base)
      (if (not (`KismetArrayLibrary.Array_IsValidIndex` (`self.EnemyUnits`)))
        (`KismetSystemLibrary.K2_SetTimer` null "InitiateVictory" 5.0)
        (`self.InitiateVictory`)))
    (:`CastFailed`
      (bind _asparty_unit_base (cast `/Game/ImportStuff/PartyUnitBase` Unit))
      (`KismetArrayLibrary.Array_RemoveItem` (`self.PartyUnits`) _asparty_unit_base))))

(fn `UserConstructionScript`)